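; BP_DungeonGameState tracks the dungeon game's phase and triggers the matching start, game over or clear logic.
; BeginPlay enters GameReady and sets Game-and-UI input with a visible cursor.
; ChangeGameState ignores repeated states; GameReady calls StartGame, then advances immediately to GameIng.
; Game Over and Game Clear call their respective functions, then both show the same WBP_GameResult widget.
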(event EventBeginPlay
  (bind _returnvalue (Game|GetPlayerController 0))
  (Class|DungeonGameStateBase|ChangeGameState "GameReady")
  (Input|SetInputModeGameandUI _returnvalue 0 "DoNotLock" false false)
  (Variables|/Script/Engine.PlayerController|SetbShowMouseCursor _returnvalue true))

(event EventTick
  (params (DeltaSeconds :type Float%20%28single-precision%29)))

(event EventChangeGameState
  (params (NewGameState :type EPOEGameState%20Enum :default "NONE"))
  (if (not (Utilities|Enum|Equal(Enum) (Variables|Default|GetCurGameState) NewGameState))
    (bind _output_get (Variables|Default|SetCurGameState NewGameState))
    (switch Utilities|FlowControl|Switch|SwitchonEPOEGameState _output_get
      (:GameReady
        ;[0.15 0.15 0.15 0.5] Set GameStart / Show Character UI
        (Class|DungeonGameStateBase|StartGame)
        (Class|DungeonGameStateBase|ChangeGameState "GameIng"))
      (:GameOver
        ;[0.15 0.15 0.15 0.5] Set GameState/ Show Result UI
        (Class|DungeonGameStateBase|GameOver)
        (bind _returnvalue (UserInterface|CreateWidget "/Game/KJW/Blueprint/UI/WBP_GameResult.WBP_GameResult_C" (Game|GetPlayerController 0) :!label _label))
        (UserInterface|Viewport|AddtoViewport _returnvalue 0))
      (:GameClear
        (Class|DungeonGameStateBase|GameClear)
        (goto _label)))))

(fn ConstructionScript)