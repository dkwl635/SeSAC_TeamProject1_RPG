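; Boss enemy Blueprint that deals melee damage and runs a forward-moving special attack, Pattern 1.
; A toggleable weapon box passes overlapped Characters to AttackTarget, while AttackEvent applies the same damage for normal and Pattern 1 states.
; Pattern 1 is eligible when its cooldown has expired and the target is within range.
; Its tick sweeps the boss forward, scaling speed by a curve sampled at normalized montage position.
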(event OnComponentBeginOverlap(WeaponBox)
  (params (OverlappedComponent :type Primitive%20Component%20Object%20Reference) (OtherActor :type Actor%20Object%20Reference) (OtherComp :type Primitive%20Component%20Object%20Reference) (OtherBodyIndex :type Integer) (bFromSweep :type Boolean) (SweepResult :type Hit%20Result%20Structure%20%28by%20ref%29))
  (bind _ascharacter (Utilities|Casting|CastToCharacter OtherActor))
  (Class|Boss|AttackTarget _ascharacter))

(event EventAttackEvent
  (params (Charactertarget :type Character%20Object%20Reference))
  (switch Utilities|FlowControl|Switch|SwitchonEBossState (Variables|Default|GetBossState)
    (:NormalAttack
      (Game|Damage|ApplyDamage Charactertarget 1e+01 0 0))
    (:Pattern1
      (Game|Damage|ApplyDamage Charactertarget 1e+01 0 0))))

(event EventTickPattern
  (switch Utilities|FlowControl|Switch|SwitchonEBossState (Variables|Default|GetBossState)
    (:Pattern1
      (Pattern|Pattern1Tick))))

(event EventSetAttackCollision
  (params (OnOff :type Boolean))
  (if OnOff
    (Collision|SetCollisionEnabled (Variables|Default|GetWeaponBox) "QueryOnly")
    (else
      (Collision|SetCollisionEnabled (Variables|Default|GetWeaponBox) "NoCollision"))))

(fn ConstructionScript)

(fn IsStartPattern1
  (if (<= (Variables|Default|GetPattern1CoolTimer) 0.0)
    (if (< (Variables|Default|GetTargetDistance) (Variables|Default|GetPattern1Distance))
      (return true)
      (else
        _)))
  (return false))

(fn Pattern1Tick
  (bind _skeletalmeshcomponent (Variables|Default|GetSkeletalMeshComponent))
  (bind _returnvalue (Components|SkeletalMesh|GetAnimInstance _skeletalmeshcomponent))
  (Transformation|SetActorLocation (+ (Transformation|GetActorLocation) (* (Transformation|GetActorForwardVector) (* (Math|Curves|GetFloatValue (Variables|Pattern1|GetPattern1MoveSpeed) (/ (Animation|Montage|MontageGetPosition _returnvalue (Animation|Montage|GetCurrentActiveMontage _returnvalue)) (Variables|Default|GetPlayMontageLength))) (Variables|Pattern1|GetPattern1Speed) (Utilities|Time|GetWorldDeltaSeconds)))) true false))