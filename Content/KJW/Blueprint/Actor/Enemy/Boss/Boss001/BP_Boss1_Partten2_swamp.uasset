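; Boss 1 pattern 2 swamp hazard: a telegraphed area that slows the player character while inside.
; On spawn a timeline scales a warning circle, then hides it, shows the swamp effect, enables overlap queries, and destroys the actor 15 seconds later.
; Sphere overlap subtracts a slow amount from the player's jog and max speeds; any end overlap adds it back without checking which actor left.
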(event OnComponentBeginOverlap(SphereCollision)
  (params (OverlappedComponent :type Primitive%20Component%20Object%20Reference) (OtherActor :type Actor%20Object%20Reference) (OtherComp :type Primitive%20Component%20Object%20Reference) (OtherBodyIndex :type Integer) (bFromSweep :type Boolean) (SweepResult :type Hit%20Result%20Structure%20%28by%20ref%29))
  (bind _asbp_main_c01_kjw (Utilities|Casting|CastToBP_Main_C01_KJW OtherActor))
  (Variables|Default|SetTarget _asbp_main_c01_kjw)
  (Variables|Default|SetIsTarget true)
  (CallFunction|SetTargetSlow))

(event OnComponentEndOverlap(SphereCollision)
  (params (OverlappedComponent :type Primitive%20Component%20Object%20Reference) (OtherActor :type Actor%20Object%20Reference) (OtherComp :type Primitive%20Component%20Object%20Reference) (OtherBodyIndex :type Integer))
  (Variables|Default|SetIsTarget false)
  (CallFunction|SetTargetSlow))

(event Custom|SetTargetSlow
  (bind _target (Variables|Default|GetTarget))
  (bind _target_2 (Variables|Default|GetTarget))
  (bind _target_3 (Variables|Default|GetTarget))
  (bind _target_4 (Variables|Default|GetTarget))
  (Utilities|IsValid (Variables|Default|GetTarget)
    (:Is%20Valid
      (if (Variables|Default|GetIsTarget)
        (Variables|/Game/KJW/BP_Main_C01_KJW.BP_Main_C01_KJW_C|SetJog%20Speed _target_3 (- (Variables|/Game/KJW/BP_Main_C01_KJW.BP_Main_C01_KJW_C|GetJog%20Speed _target_3) (Variables|Default|GetSlowWalkSpeed)))
        (Variables|/Game/KJW/BP_Main_C01_KJW.BP_Main_C01_KJW_C|SetMax%20Speed _target_4 (- (Variables|/Game/KJW/BP_Main_C01_KJW.BP_Main_C01_KJW_C|GetMax%20Speed _target_4) (Variables|Default|GetSlowWalkSpeed)))
        (else
          (Variables|/Game/KJW/BP_Main_C01_KJW.BP_Main_C01_KJW_C|SetJog%20Speed _target_2 (+ (Variables|/Game/KJW/BP_Main_C01_KJW.BP_Main_C01_KJW_C|GetJog%20Speed _target_2) (Variables|Default|GetSlowWalkSpeed)))
          (Variables|/Game/KJW/BP_Main_C01_KJW.BP_Main_C01_KJW_C|SetMax%20Speed _target (+ (Variables|/Game/KJW/BP_Main_C01_KJW.BP_Main_C01_KJW_C|GetMax%20Speed _target) (Variables|Default|GetSlowWalkSpeed))))))))

(event EventBeginPlay
  (Collision|SetCollisionEnabled (Variables|Default|GetSphereCollision) "NoCollision")
  (Rendering|SetVisibility (Variables|Default|GetBP_ky_Boss_SwampEffect) false false)
  (bind _scale (Timeline|ShowCircle Play)
    (:Update
      (Transformation|SetRelativeScale3D (Variables|Default|GetCicle) (* (Class|KismetMathLibrary|VectorOne) _scale)))
    (:Finished
      (Rendering|SetVisibility (Variables|Default|GetCicle) false false)
      (Rendering|SetVisibility (Variables|Default|GetBP_ky_Boss_SwampEffect) true false)
      (Collision|SetCollisionEnabled (Variables|Default|GetSphereCollision) "QueryOnly")
      (Utilities|FlowControl|Delay 15.0)
      (Actor|DestroyActor))))

(fn ConstructionScript)