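; BP_Enemy_Griffon is a ranged enemy that shoots projectiles at its target character.
; AttackStart plays the attack montage, whose notify spawns BP_Enemy_Projectile at AttackPoint, aimed at the target with the enemy's attack power.
; On death it stops its AI, disables body collision, ragdolls with a backward impulse, requests an item drop from the item subsystem, then destroys itself after a short delay.
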(event EventBeginPlay)

(event Collision|EventActorBeginOverlap
  (params (OtherActor :type Actor%20Object%20Reference)))

(event EventTick
  (params (DeltaSeconds :type Float%20%28single-precision%29)))

(event EventAttackStart
  (bind _attackmontage (Variables|Default|GetAttackMontage))
  (Development|PrintString "Barghest_AttackStart")
  (Utilities|IsValid _attackmontage
    (:Is%20Valid
      (bind _notifyname (Animation|Montage|PlayMontage (Variables|Default|GetSkeletalMeshComponent) _attackmontage)
        (:OnCompleted
          (Class|Enemy|AttackEnd))
        (:OnNotifyBegin
          (Development|PrintString (Utilities|String|ToString(Name) _notifyname))
          (Class|Enemy|AttackEvent))))))

(event EventAttackEvent
  (Development|PrintString "Attack Event")
  (bind _returnvalue (Game|SpawnActorfromClass "/Game/KJW/Blueprint/Actor/Enemy/Normal/Projectile/BP_Enemy_Projectile.BP_Enemy_Projectile_C" (Math|Transform|MakeTransform (Transformation|GetWorldLocation (Variables|Default|GetAttackPoint)) "0, 0, 0" "1.000000,1.000000,1.000000") "Undefined" "MultiplyWithRoot" 0 0))
  (Default|SetProjectile _returnvalue (Math|Vector|Normalize (- (Transformation|GetActorLocation (Variables|Default|GetTargetCharacter)) (Transformation|GetWorldLocation (Variables|Default|GetAttackPoint)))) (Variables|Default|GetAtkPower) 3.0 3e+02 (Variables|Default|GetTargetCharacter)))

(event EventAttackEnd
  (Development|PrintString "Attack End"))

(event EventDieStart
  (bind _skeletalmeshcomponent (Variables|Default|GetSkeletalMeshComponent))
  (bind _asbp_aicontroller (Utilities|Casting|CastToBP_AIController (Pawn|GetController)))
  (Default|StopAI _asbp_aicontroller)
  (Collision|SetCollisionEnabled (Variables|Default|GetBodyCollision) "NoCollision")
  (Collision|SetCollisionEnabled _skeletalmeshcomponent "PhysicsOnly")
  (Physics|SetSimulatePhysics _skeletalmeshcomponent true)
  (Physics|SetPhysicsLinearVelocity _skeletalmeshcomponent "0, 0, 0" false "None")
  (Class|SkeletalMeshComponent|AddImpulsetoAllBodiesBelow _skeletalmeshcomponent (* (* (Transformation|GetActorForwardVector) -1.0) 5e+03) "None" false true)
  (Class|ItemGameInstanceSubsystem|GetNewDropItem (Subsystems|GetItemGameInstanceSubsystem) (Variables|Default|GetDropItemID) 1 self)
  (Utilities|FlowControl|Delay 2.0)
  (Class|Enemy|DieEnd))

(event EventDieEnd
  (Actor|DestroyActor))

(fn ConstructionScript)