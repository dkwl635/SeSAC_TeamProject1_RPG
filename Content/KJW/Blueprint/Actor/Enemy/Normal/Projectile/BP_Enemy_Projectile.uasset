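; Enemy projectile actor that flies in a straight line and damages one designated target character.
; SetProjectile receives direction, damage, lifetime, speed and target from outside.
; Tick moves it by direction times speed and delta time with a swept SetActorLocation, and ProjectileBody overlap applies damage only when the other actor is that target.
; The graph stores LifeTime without using it and never destroys the projectile on hit.
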(event OnComponentBeginOverlap(ProjectileBody)
  (params (OverlappedComponent :type Primitive%20Component%20Object%20Reference) (OtherActor :type Actor%20Object%20Reference) (OtherComp :type Primitive%20Component%20Object%20Reference) (OtherBodyIndex :type Integer) (bFromSweep :type Boolean) (SweepResult :type Hit%20Result%20Structure%20%28by%20ref%29))
  (bind _charactertarget (Variables|Default|GetCharacterTarget))
  (if (== OtherActor _charactertarget)
    (Game|Damage|ApplyDamage _charactertarget (Variables|Default|GetDamage) 0 0)))

(event Custom|SetProjectile
  (params (NewDir :type Vector) (NewDamage :type Float%20%28double-precision%29) (NewLifeTime :type Float%20%28double-precision%29) (NewSpeed :type Float%20%28double-precision%29) (NewTarget :type Actor%20Object%20Reference))
  (Variables|Default|SetDirection NewDir)
  (Variables|Default|SetDamage NewDamage)
  (Variables|Default|SetLifeTime NewLifeTime)
  (Variables|Default|SetSpeed NewSpeed)
  (Variables|Default|SetCharacterTarget NewTarget))

(event EventTick
  (params (DeltaSeconds :type Float%20%28single-precision%29))
  (Transformation|SetActorLocation (+ (Transformation|GetActorLocation) (* (Variables|Default|GetDirection) (* (Variables|Default|GetSpeed) (Utilities|Time|GetWorldDeltaSeconds)))) true false))

(fn ConstructionScript)