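; Barghest enemy Blueprint that handles its melee attack and death, with tail and mane meshes following the body's pose.
; An attack montage's notify fires a short forward line trace from AttackPoint, damaging any Character it hits by AtkPower.
; Death stops the AI controller, ragdolls the body with a backward impulse, spawns an item drop from the item subsystem, then destroys the actor after a delay.
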(event EventBeginPlay
  (Components|SkinnedMesh|SetLeaderPoseComponent (Variables|Default|GetSK_BARGHEST_TAIL) (Variables|Default|GetSkeletalMeshComponent) false false))

(event Collision|EventActorBeginOverlap
  (params (OtherActor :type Actor%20Object%20Reference)))

(event EventTick
  (params (DeltaSeconds :type Float%20%28single-precision%29)))

(event EventAttackStart
  (bind _attackmontage (Variables|Default|GetAttackMontage))
  (Development|PrintString "Barghest_AttackStart")
  (Utilities|IsValid _attackmontage
    (:Is%20Valid
      (bind _notifyname (Animation|Montage|PlayMontage (Variables|Default|GetSkeletalMeshComponent) _attackmontage)
        (:OnCompleted
          (Class|Enemy|AttackEnd))
        (:OnNotifyBegin
          (Development|PrintString (Utilities|String|ToString(Name) _notifyname))
          (Class|Enemy|AttackEvent))))))

(event EventAttackEvent
  (bind _attackpoint (Variables|Default|GetAttackPoint))
  (bind _returnvalue (Transformation|GetWorldLocation _attackpoint))
  (Development|PrintString "Attack Event")
  (bind (_outhit _returnvalue_2) (Collision|LineTraceByChannel _returnvalue (+ _returnvalue (* (Transformation|GetActorForwardVector) 1e+02)) "TraceTypeQuery4" false 0 "ForDuration" true "(R=1.000000,G=0.000000,B=0.000000,A=1.000000)" "(R=0.000000,G=1.000000,B=0.000000,A=1.000000)" 2.0))
  (if _returnvalue_2
    (bind _ascharacter (Utilities|Casting|CastToCharacter (.HitActor (Collision|BreakHitResult _outhit))))
    (Game|Damage|ApplyDamage _ascharacter (Variables|Default|GetAtkPower) 0 0)))

(event EventAttackEnd
  (Development|PrintString "Attack End"))

(event EventDieStart
  (bind _skeletalmeshcomponent (Variables|Default|GetSkeletalMeshComponent))
  (bind _asbp_aicontroller (Utilities|Casting|CastToBP_AIController (Pawn|GetController)))
  (Default|StopAI _asbp_aicontroller)
  (Collision|SetCollisionEnabled (Variables|Default|GetBodyCollision) "NoCollision")
  (Collision|SetCollisionEnabled _skeletalmeshcomponent "PhysicsOnly")
  (Physics|SetSimulatePhysics _skeletalmeshcomponent true)
  (Physics|SetPhysicsLinearVelocity _skeletalmeshcomponent "0, 0, 0" false "None")
  (Class|SkeletalMeshComponent|AddImpulsetoAllBodiesBelow _skeletalmeshcomponent (* (* (Transformation|GetActorForwardVector) -1.0) 5e+03) "None" false true)
  (bind _returnvalue (Game|SpawnActorfromClass "/Game/KJW/Blueprint/Actor/Item/BP_DropItem.BP_DropItem_C" (Math|Transform|MakeTransform (Transformation|GetActorLocation) "0, 0, 0" "1.000000,1.000000,1.000000") "Undefined" "MultiplyWithRoot" 0 0))
  (bind _returnvalue_2 (Class|ItemGameInstanceSubsystem|GetNewItem (Subsystems|GetItemGameInstanceSubsystem) (Variables|Default|GetDropItemID) 1))
  (Variables|/Script/TeamProject_POEKor.DropItem|SetItem _returnvalue _returnvalue_2)
  (Utilities|FlowControl|Delay 2.0)
  (Class|Enemy|DieEnd))

(event EventDieEnd
  (Actor|DestroyActor))

(fn ConstructionScript)