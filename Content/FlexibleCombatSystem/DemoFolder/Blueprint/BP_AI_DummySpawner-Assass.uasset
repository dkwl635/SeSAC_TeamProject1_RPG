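; Demo spawner actor that populates five spawn-point components with assassin AI dummies (BP_AI_AssassDummy).
; On BeginPlay the server spawns one per point, raised in Z and yawed 90 degrees from the actor, passing in a faction and AI setup data.
; Spawned dummies are tracked in AISpawned, so Interact can destroy them all and respawn a fresh set on the authority.
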(event EventInteract
  (params (Character :type Character%20Object%20Reference))
  (bind _returnvalue (Transformation|GetActorRotation))
  (bind _aispawned (Variables|Default|GetAISpawned))
  (Networking|SwitchHasAuthority
    (:Authority
      (for _array_element _aispawned
        (Actor|DestroyActor _array_element))
      (Utilities|Array|Clear _aispawned)
      (Networking|SwitchHasAuthority
        (:Authority
          (Utilities|Array|Clear (Variables|Default|GetAISpawned))
          (for _array_element_2 (Utilities|Array|MakeArray (Variables|Default|GetSpawn_1) (Variables|Default|GetSpawn_2) (Variables|Default|GetSpawn_0) (Variables|Default|GetSpawn_3) (Variables|Default|GetSpawn_4))
            (bind _returnvalue_2 (Game|SpawnActorfromClass "/Game/FlexibleCombatSystem/Blueprints/AI/Dummy/BP_AI_AssassDummy.BP_AI_AssassDummy_C" (Math|Transform|MakeTransform (Math|Vector|MakeVector (.x (Transformation|GetWorldLocation _array_element_2)) (.y (Transformation|GetWorldLocation _array_element_2)) (+ (.z (Transformation|GetWorldLocation _array_element_2)) 9e+01)) (Math|Rotator|MakeRotator (.roll _returnvalue) (.pitch _returnvalue) (+ (.yaw _returnvalue) 9e+01)) "1,1,1") "Undefined" 0 "NewEnumerator2" (Variables|Default|GetAI%20Setup%20Data) false 0 0 0 0 false 0))
            (Utilities|Array|Add (Variables|Default|GetAISpawned) _returnvalue_2)))))))

(event EventBeginPlay
  (bind _returnvalue (Transformation|GetActorRotation))
  (Networking|SwitchHasAuthority
    (:Authority
      (Utilities|Array|Clear (Variables|Default|GetAISpawned))
      (for _array_element (Utilities|Array|MakeArray (Variables|Default|GetSpawn_1) (Variables|Default|GetSpawn_2) (Variables|Default|GetSpawn_0) (Variables|Default|GetSpawn_3) (Variables|Default|GetSpawn_4))
        (bind _returnvalue_2 (Game|SpawnActorfromClass "/Game/FlexibleCombatSystem/Blueprints/AI/Dummy/BP_AI_AssassDummy.BP_AI_AssassDummy_C" (Math|Transform|MakeTransform (Math|Vector|MakeVector (.x (Transformation|GetWorldLocation _array_element)) (.y (Transformation|GetWorldLocation _array_element)) (+ (.z (Transformation|GetWorldLocation _array_element)) 9e+01)) (Math|Rotator|MakeRotator (.roll _returnvalue) (.pitch _returnvalue) (+ (.yaw _returnvalue) 9e+01)) "1,1,1") "Undefined" 0 "NewEnumerator2" (Variables|Default|GetAI%20Setup%20Data) false 0 0 0 0 false 0))
        (Utilities|Array|Add (Variables|Default|GetAISpawned) _returnvalue_2)))))

(fn ConstructionScript)