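; War room teleporter for the demo that moves an overlapping Player-tagged Character, then after a short delay the companions it reports, to a destination.
; Each teleport picks random navigable coordinates around the destination Sphere and spawns a Niagara effect just below that location.
; The construction script sets the label and color-based material, and places the Sphere at Destination.
; "Return To Start" labels instead use hardcoded world positions chosen by the Systems flag.
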(event OnComponentBeginOverlap(Box)
  (params (OverlappedComponent :type Primitive%20Component%20Object%20Reference) (OtherActor :type Actor%20Object%20Reference) (OtherComp :type Primitive%20Component%20Object%20Reference) (OtherBodyIndex :type Integer) (bFromSweep :type Boolean) (SweepResult :type Hit%20Result%20Structure%20%28by%20ref%29))
  (if (Actor|ActorHasTag OtherActor "Player")
    (bind _ascharacter (Utilities|Casting|CastToCharacter OtherActor))
    (CallFunction|Teleport _ascharacter)
    (Utilities|FlowControl|Delay 0.1)
    (bind _companionref (Class|ICharacter|PassCompanions(Message) _ascharacter))
    (for _array_element _companionref
      (CallFunction|Teleport _array_element))))

(fn ConstructionScript
  (bind _sphere (Variables|Default|GetSphere))
  (if (Utilities|Enum|Equal(Enum) (Variables|Default|GetTextValue) (Utilities|Text|MakeLiteralText "Return To Start"))
    (Transformation|SetWorldLocation _sphere (select (Variables|Default|GetSystems) "0, 0, 0" "0,-23122.000000,113.000000") false false)
    (Variables|Default|SetDestination (Variables|/Script/Engine.SceneComponent|GetRelativeLocation _sphere))
    (else
      (Transformation|SetRelativeLocation (Variables|Default|GetSphere) (Variables|Default|GetDestination) false false)))
  (Rendering|Components|TextRender|SetText (Variables|Default|GetTextRender) (Variables|Default|GetTextValue))
  (Rendering|Material|SetMaterial (Variables|Default|GetStaticMesh) 0 (Utilities|Select :Index (Variables|Default|GetColor) :NewEnumerator0 "/Game/FlexibleCombatSystem/DemoFolder/Materials/MI_MagicTraining.MI_MagicTraining" :NewEnumerator1 "/Game/FlexibleCombatSystem/DemoFolder/Materials/MI_SystemsTraining.MI_SystemsTraining" :NewEnumerator2 "/Game/FlexibleCombatSystem/DemoFolder/Materials/MI_MagicTraining.MI_MagicTraining")))

(fn Teleport
  (params (Target :type Actor%20Object%20Reference))
  (bind _sphere (Variables|Default|GetSphere))
  (bind _returnvalue (Transformation|GetWorldLocation _sphere))
  (bind _randomlocation (Class|NavigationSystemV1|GetRandomPointinNavigableRadius _returnvalue 2e+02 0 0))
  (bind _output_get (LocalVariables|SetLocation (Math|Vector|MakeVector (.x _randomlocation) (.y _randomlocation) (.z _randomlocation))))
  (Transformation|SetActorLocation Target _output_get false false)
  (Niagara|SpawnSystematLocation "/Game/FlexibleCombatSystem/VFX/MeleeVFX/Teleport/NS_Skill_TeleportationOut.NS_Skill_TeleportationOut" (- (LocalVariables|GetLocation) "0, 0,70.000000")))