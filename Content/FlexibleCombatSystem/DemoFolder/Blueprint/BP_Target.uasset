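; Shooting-range target for the ranged practice demo, switched on and off by a RangedPractise manager.
; Five ring hit components map arrow or projectile hits to different scores; the first hit while active shows combat text, adds score and tips the target over, gated by a DoOnce until Deactivate.
; Moving targets slide sideways on a looping timeline until stopped.
; The construction script sets a training-type material and lays out the moving-target frame and start side.
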(event OnComponentHit(Outer1)
  (params (HitComponent :type Primitive%20Component%20Object%20Reference) (OtherActor :type Actor%20Object%20Reference) (OtherComp :type Primitive%20Component%20Object%20Reference) (NormalImpulse :type Vector :default "0, 0, 0") (Hit :type Hit%20Result%20Structure%20%28by%20ref%29))
  (Utilities|Casting|CastToBP_ArrowParent OtherActor
    (:then
      _)
    (:CastFailed
      (Utilities|Casting|CastToBP_ProjectileParent OtherActor)))
  (Variables|Default|SetDamageValue 40)
  (if (Variables|Default|GetActive)
    (Utilities|FlowControl|DoOnce false
      (:Completed
        (Networking|SwitchHasAuthority
          (:Authority
            (if (Pawn|IsLocalController (Game|GetPlayerController 0))
              (bind _returnvalue (UserInterface|CreateWidget "/Game/FlexibleCombatSystem/Widgets/Combat/WB_CombatText.WB_CombatText_C" 0 (Transformation|GetActorLocation) (Variables|Default|GetDamageValue) :!label _label))
              (UserInterface|Viewport|AddtoViewport _returnvalue 0)))
          (:Remote
            (goto _label)))
        (Default|AddScore (Variables|Default|GetRangedPractise) (Variables|Default|GetDamageValue))
        (bind _newtrack_0 (Timeline|Movebaby PlayFromStart)
          (:Update
            (Transformation|SetRelativeRotation (Variables|Default|GetScene) (Math|Rotator|Lerp(Rotator) "0, 0, 0" "0, 0,90.000000" _newtrack_0 true) false false))
          (:Finished
            (CallFunction|Stop)))))))

(event OnComponentHit(Outer2)
  (params (HitComponent :type Primitive%20Component%20Object%20Reference) (OtherActor :type Actor%20Object%20Reference) (OtherComp :type Primitive%20Component%20Object%20Reference) (NormalImpulse :type Vector :default "0, 0, 0") (Hit :type Hit%20Result%20Structure%20%28by%20ref%29))
  (Utilities|Casting|CastToBP_ArrowParent OtherActor
    (:then
      _)
    (:CastFailed
      (Utilities|Casting|CastToBP_ProjectileParent OtherActor)))
  (Variables|Default|SetDamageValue 60)
  (if (Variables|Default|GetActive)
    (Utilities|FlowControl|DoOnce false
      (:Completed
        (Networking|SwitchHasAuthority
          (:Authority
            (if (Pawn|IsLocalController (Game|GetPlayerController 0))
              (bind _returnvalue (UserInterface|CreateWidget "/Game/FlexibleCombatSystem/Widgets/Combat/WB_CombatText.WB_CombatText_C" 0 (Transformation|GetActorLocation) (Variables|Default|GetDamageValue) :!label _label))
              (UserInterface|Viewport|AddtoViewport _returnvalue 0)))
          (:Remote
            (goto _label)))
        (Default|AddScore (Variables|Default|GetRangedPractise) (Variables|Default|GetDamageValue))
        (bind _newtrack_0 (Timeline|Movebaby PlayFromStart)
          (:Update
            (Transformation|SetRelativeRotation (Variables|Default|GetScene) (Math|Rotator|Lerp(Rotator) "0, 0, 0" "0, 0,90.000000" _newtrack_0 true) false false))
          (:Finished
            (CallFunction|Stop)))))))

(event OnComponentHit(Outer3)
  (params (HitComponent :type Primitive%20Component%20Object%20Reference) (OtherActor :type Actor%20Object%20Reference) (OtherComp :type Primitive%20Component%20Object%20Reference) (NormalImpulse :type Vector :default "0, 0, 0") (Hit :type Hit%20Result%20Structure%20%28by%20ref%29))
  (Utilities|Casting|CastToBP_ArrowParent OtherActor
    (:then
      _)
    (:CastFailed
      (Utilities|Casting|CastToBP_ProjectileParent OtherActor)))
  (Variables|Default|SetDamageValue 80)
  (if (Variables|Default|GetActive)
    (Utilities|FlowControl|DoOnce false
      (:Completed
        (Networking|SwitchHasAuthority
          (:Authority
            (if (Pawn|IsLocalController (Game|GetPlayerController 0))
              (bind _returnvalue (UserInterface|CreateWidget "/Game/FlexibleCombatSystem/Widgets/Combat/WB_CombatText.WB_CombatText_C" 0 (Transformation|GetActorLocation) (Variables|Default|GetDamageValue) :!label _label))
              (UserInterface|Viewport|AddtoViewport _returnvalue 0)))
          (:Remote
            (goto _label)))
        (Default|AddScore (Variables|Default|GetRangedPractise) (Variables|Default|GetDamageValue))
        (bind _newtrack_0 (Timeline|Movebaby PlayFromStart)
          (:Update
            (Transformation|SetRelativeRotation (Variables|Default|GetScene) (Math|Rotator|Lerp(Rotator) "0, 0, 0" "0, 0,90.000000" _newtrack_0 true) false false))
          (:Finished
            (CallFunction|Stop)))))))

(event OnComponentHit(Outer4)
  (params (HitComponent :type Primitive%20Component%20Object%20Reference) (OtherActor :type Actor%20Object%20Reference) (OtherComp :type Primitive%20Component%20Object%20Reference) (NormalImpulse :type Vector :default "0, 0, 0") (Hit :type Hit%20Result%20Structure%20%28by%20ref%29))
  (Utilities|Casting|CastToBP_ArrowParent OtherActor
    (:then
      _)
    (:CastFailed
      (Utilities|Casting|CastToBP_ProjectileParent OtherActor)))
  (Variables|Default|SetDamageValue 100)
  (if (Variables|Default|GetActive)
    (Utilities|FlowControl|DoOnce false
      (:Completed
        (Networking|SwitchHasAuthority
          (:Authority
            (if (Pawn|IsLocalController (Game|GetPlayerController 0))
              (bind _returnvalue (UserInterface|CreateWidget "/Game/FlexibleCombatSystem/Widgets/Combat/WB_CombatText.WB_CombatText_C" 0 (Transformation|GetActorLocation) (Variables|Default|GetDamageValue) :!label _label))
              (UserInterface|Viewport|AddtoViewport _returnvalue 0)))
          (:Remote
            (goto _label)))
        (Default|AddScore (Variables|Default|GetRangedPractise) (Variables|Default|GetDamageValue))
        (bind _newtrack_0 (Timeline|Movebaby PlayFromStart)
          (:Update
            (Transformation|SetRelativeRotation (Variables|Default|GetScene) (Math|Rotator|Lerp(Rotator) "0, 0, 0" "0, 0,90.000000" _newtrack_0 true) false false))
          (:Finished
            (CallFunction|Stop)))))))

(event OnComponentHit(Outer0)
  (params (HitComponent :type Primitive%20Component%20Object%20Reference) (OtherActor :type Actor%20Object%20Reference) (OtherComp :type Primitive%20Component%20Object%20Reference) (NormalImpulse :type Vector :default "0, 0, 0") (Hit :type Hit%20Result%20Structure%20%28by%20ref%29))
  (Utilities|Casting|CastToBP_ArrowParent OtherActor
    (:then
      _)
    (:CastFailed
      (Utilities|Casting|CastToBP_ProjectileParent OtherActor)))
  (Variables|Default|SetDamageValue 20)
  (if (Variables|Default|GetActive)
    (Utilities|FlowControl|DoOnce false
      (:Completed
        (Networking|SwitchHasAuthority
          (:Authority
            (if (Pawn|IsLocalController (Game|GetPlayerController 0))
              (bind _returnvalue (UserInterface|CreateWidget "/Game/FlexibleCombatSystem/Widgets/Combat/WB_CombatText.WB_CombatText_C" 0 (Transformation|GetActorLocation) (Variables|Default|GetDamageValue) :!label _label))
              (UserInterface|Viewport|AddtoViewport _returnvalue 0)))
          (:Remote
            (goto _label)))
        (Default|AddScore (Variables|Default|GetRangedPractise) (Variables|Default|GetDamageValue))
        (bind _newtrack_0 (Timeline|Movebaby PlayFromStart)
          (:Update
            (Transformation|SetRelativeRotation (Variables|Default|GetScene) (Math|Rotator|Lerp(Rotator) "0, 0, 0" "0, 0,90.000000" _newtrack_0 true) false false))
          (:Finished
            (CallFunction|Stop)))))))

(event Custom|Activate
  (params (RangedPractise :type BP%20Ranged%20Practise%20Object%20Reference))
  (bind _rightstart (Variables|Default|GetRightStart))
  (bind _staticmesh (Variables|Default|GetStaticMesh))
  (bind _relativelocation (Variables|/Script/Engine.SceneComponent|GetRelativeLocation _staticmesh))
  (Variables|Default|SetRangedPractise RangedPractise)
  (Variables|Default|SetActive true)
  (if (Variables|Default|GetMoving)
    (bind _newtrack_0 (Timeline|Move PlayFromStart)
      (:Update
        (Transformation|SetRelativeLocation _staticmesh (Math|Vector|Lerp(Vector) (Math|Vector|MakeVector (select _rightstart 2.3e+02 -2.3e+02) (.y _relativelocation) (.z _relativelocation)) (Math|Vector|MakeVector (select _rightstart -2.3e+02 2.3e+02) (.y _relativelocation) (.z _relativelocation)) _newtrack_0) false false))
      (:Finished
        (CallFunction|MoveAgain)))))

(event Custom|Deactivate
  (CallFunction|Stop)
  (Variables|Default|SetActive false)
  (Utilities|FlowControl|DoOnce false) ; enters at Reset
)

(event Custom|MoveAgain
  (bind _rightstart (Variables|Default|GetRightStart))
  (bind _staticmesh (Variables|Default|GetStaticMesh))
  (bind _relativelocation (Variables|/Script/Engine.SceneComponent|GetRelativeLocation _staticmesh))
  (bind _newtrack_0 (Timeline|Move PlayFromStart)
    (:Update
      (Transformation|SetRelativeLocation _staticmesh (Math|Vector|Lerp(Vector) (Math|Vector|MakeVector (select _rightstart 2.3e+02 -2.3e+02) (.y _relativelocation) (.z _relativelocation)) (Math|Vector|MakeVector (select _rightstart -2.3e+02 2.3e+02) (.y _relativelocation) (.z _relativelocation)) _newtrack_0) false false))
    (:Finished
      (CallFunction|MoveAgain))))

(event Custom|Stop
  (bind _rightstart (Variables|Default|GetRightStart))
  (bind _staticmesh (Variables|Default|GetStaticMesh))
  (bind _relativelocation (Variables|/Script/Engine.SceneComponent|GetRelativeLocation _staticmesh))
  (bind _newtrack_0 (Timeline|Move Stop)
    (:Update
      (Transformation|SetRelativeLocation _staticmesh (Math|Vector|Lerp(Vector) (Math|Vector|MakeVector (select _rightstart 2.3e+02 -2.3e+02) (.y _relativelocation) (.z _relativelocation)) (Math|Vector|MakeVector (select _rightstart -2.3e+02 2.3e+02) (.y _relativelocation) (.z _relativelocation)) _newtrack_0) false false))
    (:Finished
      (CallFunction|MoveAgain))))

(event Custom|Reset
  (Transformation|SetRelativeLocation (Variables|Default|GetStaticMesh) (Variables|Default|GetResetLocation) false false)
  (Transformation|SetRelativeRotation (Variables|Default|GetScene) "0, 0, 0" false false))

(event EventBeginPlay
  (Variables|Default|SetResetLocation (Variables|/Script/Engine.SceneComponent|GetRelativeLocation (Variables|Default|GetStaticMesh))))

(fn ConstructionScript
  (Rendering|Material|SetMaterial (Variables|Default|GetStaticMesh1) 0 (Utilities|Select :Index (Variables|Default|GetColour) :NewEnumerator0 "/Game/FlexibleCombatSystem/DemoFolder/Materials/MI_MeleeTraining.MI_MeleeTraining" :NewEnumerator1 "/Game/FlexibleCombatSystem/DemoFolder/Materials/MI_RangedTraining.MI_RangedTraining" :NewEnumerator2 "/Game/FlexibleCombatSystem/DemoFolder/Materials/MI_MagicTraining.MI_MagicTraining"))
  (if (Variables|Default|GetMoving)
    (Transformation|SetRelativeLocation (Variables|Default|GetStaticMesh2) "-300.000000, 0,-560.000000" false false)
    (Transformation|SetRelativeLocation (Variables|Default|GetStaticMesh3) "300.000000, 0,-560.000000" false false)
    (Transformation|SetRelativeScale3D (Variables|Default|GetStaticMesh1) "6.000000,0.100000,0.100000")
    (Transformation|SetRelativeLocation (Variables|Default|GetStaticMesh) (select (Variables|Default|GetRightStart) "230.000000,-2.000000,-20.000000" "-230.000000,-2.000000,-20.000000") false false)))