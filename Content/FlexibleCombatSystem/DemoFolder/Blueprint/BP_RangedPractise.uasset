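; Demo ranged-practice minigame that scores the player's shooting at a set of targets and awards a medal message.
; Interact passes through a DoOnce, re-armed by Reset, to activate the targets and create the score widget.
; AddScore totals points and hits, calling Deactivate once every target is hit to show tiered tutorial text.
; Authority switches with local-controller checks keep the UI on local players.
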(event Custom|Reset
  (for _array_element (Variables|Default|GetTargets)
    (Default|Reset _array_element))
  (Utilities|FlowControl|DoOnce false) ; enters at Reset
)

(event Custom|Deactivate
  (bind _character (Variables|Default|GetCharacter))
  (bind _targetscore (Variables|Default|GetTargetScore))
  (Class|IInteract|Interact(Message) (Variables|Default|GetActivate))
  (Variables|Default|SetActive false)
  (for _array_element (Variables|Default|GetTargets)
    (Default|Deactivate _array_element))
  (Networking|SwitchHasAuthority
    (:Authority
      (Utilities|IsValid _character
        (:Is%20Valid
          (if (Pawn|IsLocallyControlled _character)
            (Default|Deactivate _targetscore :!label _label)
            (bind _returnvalue (UserInterface|CreateWidget "/Game/FlexibleCombatSystem/Widgets/General/WB_TutorialText.WB_TutorialText_C" 0 (select (>= (Variables|/Game/FlexibleCombatSystem/DemoFolder/Widgets/WB_TargetScore.WB_TargetScore_C|GetTargetScore _targetscore) 1500) "Damn son nice shooting that's a Gold Medal right there. You are like Robin Hood if he was a Mannequin. You're one Sexy Beast of a Bow and Arrow User!!  If you want to play again hit the button on the right" (select (>= (Variables|/Game/FlexibleCombatSystem/DemoFolder/Widgets/WB_TargetScore.WB_TargetScore_C|GetTargetScore _targetscore) 1200) "Silver Medal! Pretty impressive but you're going to need a score of 1500 to get Gold. If you want to play again hit the button on the right" (select (>= (Variables|/Game/FlexibleCombatSystem/DemoFolder/Widgets/WB_TargetScore.WB_TargetScore_C|GetTargetScore _targetscore) 900) "Hey Bronze medal, not bad at all my friend. You've gotta up your game to 1200 points for silver or 1400 points for gold, I believe in you! If you want to play again hit the button on the right" "That is some seriously unimpressive shooting I must say, not even a Bronze Medal which is only 900 points! If you want to play again hit the button on the right")))))
            (UserInterface|Viewport|AddtoViewport _returnvalue 0)
            (Utilities|FlowControl|Delay 13.0)
            (Default|EventMoveDown _returnvalue)))))
    (:Remote
      (goto _label))))

(event Custom|AddScore
  (params (Score :type Integer))
  (Networking|SwitchHasAuthority
    (:Authority
      (if (Pawn|IsLocalController (Game|GetPlayerController 0))
        (Variables|/Game/FlexibleCombatSystem/DemoFolder/Widgets/WB_TargetScore.WB_TargetScore_C|SetTargetScore (Variables|Default|GetTargetScore) (+ (Variables|/Game/FlexibleCombatSystem/DemoFolder/Widgets/WB_TargetScore.WB_TargetScore_C|GetTargetScore (Variables|Default|GetTargetScore)) Score) :!label _label)
        (bind _result (Math|Integer|IncrementInt (Variables|Default|GetTargetsHit))
          (:%20%20
            (if (== _result (Variables|Default|GetTotalTargets))
              (CallFunction|Deactivate))))))
    (:Remote
      (goto _label))))

(event EventInteract
  (params (Character :type Character%20Object%20Reference))
  (Variables|Default|SetCharacter Character)
  (Utilities|FlowControl|DoOnce false
    (:Completed
      (Variables|Default|SetActive true)
      (Variables|Default|SetTotalTargets (Utilities|Array|Length (Variables|Default|GetTargets)))
      (Networking|SwitchHasAuthority
        (:Authority
          (if (Pawn|IsLocalController (Game|GetPlayerController 0))
            (bind _returnvalue (UserInterface|CreateWidget "/Game/FlexibleCombatSystem/DemoFolder/Widgets/WB_TargetScore.WB_TargetScore_C" 0 self :!label _label))
            (UserInterface|Viewport|AddtoViewport _returnvalue 0)
            (Variables|Default|SetTargetScore _returnvalue)))
        (:Remote
          (goto _label)))
      (for _array_element (Variables|Default|GetTargets)
        (Default|Activate _array_element self))
      (Networking|SwitchHasAuthority
        (:Authority
          (if (Pawn|IsLocalController (Game|GetPlayerController 0))
            (Default|Activate (Variables|Default|GetTargetScore) :!label _label_2)))
        (:Remote
          (goto _label_2))))))

(fn ConstructionScript)