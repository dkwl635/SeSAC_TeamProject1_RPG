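; Demo dummy that shows off one animation from a chosen combat style, looping on its skeletal mesh.
; On BeginPlay it switches on AICombatStyle, destroys the weapon and shield components that style does not use, then plays the animation picked by AnimationNumber.
; Fists has an optional shield variant with fewer animations, and the Mage branch only strips all weapons without playing anything.
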(event EventBeginPlay
  (Utilities|IsValid (Variables|Default|GetMesh)
    (:Is%20Valid
      (switch Utilities|FlowControl|Switch|SwitchonE_AICombatStyle (Variables|SetupinGame|GetAI%20Combat%20Style)
        (:NewEnumerator7
          ;[1 1 1] Fists
          (if (Variables|SetupInGame|GetAddShield)
            (Components|DestroyComponent (Variables|Default|Get2h))
            (switch int (Variables|SetupInGame|GetAnimationNumber)
              (:0
                (Components|Animation|PlayAnimation (Variables|Default|GetMesh) "/Game/FlexibleCombatSystem/Animation/UE4-Mannequin/OffhandShield/Locomotion/OHS_Idle.OHS_Idle" true))
              (:1
                (Components|Animation|PlayAnimation (Variables|Default|GetMesh) "/Game/FlexibleCombatSystem/Animation/UE4-Mannequin/Fists/Locomotion/Fists_Jog_Fwd.Fists_Jog_Fwd" true)))
            (else
              (Components|DestroyComponent (Variables|Default|Get2h))
              (switch int (Variables|SetupInGame|GetAnimationNumber)
                (:0
                  (Components|Animation|PlayAnimation (Variables|Default|GetMesh) "/Game/FlexibleCombatSystem/Animation/UE4-Mannequin/Fists/Locomotion/Fists_Idle.Fists_Idle" true))
                (:1
                  (Components|Animation|PlayAnimation (Variables|Default|GetMesh) "/Game/FlexibleCombatSystem/Animation/UE4-Mannequin/Fists/Locomotion/Fists_Jog_Fwd.Fists_Jog_Fwd" true))
                (:2
                  (Components|Animation|PlayAnimation (Variables|Default|GetMesh) "/Game/FlexibleCombatSystem/Animation/UE4-Mannequin/Fists/Combat/Fists_Attack_A.Fists_Attack_A" true))
                (:3
                  (Components|Animation|PlayAnimation (Variables|Default|GetMesh) "/Game/FlexibleCombatSystem/Animation/UE4-Mannequin/Fists/Combat/Fists_Attack_B.Fists_Attack_B" true))
                (:4
                  (Components|Animation|PlayAnimation (Variables|Default|GetMesh) "/Game/FlexibleCombatSystem/Animation/UE4-Mannequin/Fists/Combat/Fists_Attack_C.Fists_Attack_C" true))
                (:5
                  (Components|Animation|PlayAnimation (Variables|Default|GetMesh) "/Game/FlexibleCombatSystem/Animation/UE4-Mannequin/Fists/Combat/Fists_Attack_D.Fists_Attack_D" true))
                (:6
                  (Components|Animation|PlayAnimation (Variables|Default|GetMesh) "/Game/FlexibleCombatSystem/Animation/UE4-Mannequin/Fists/Combat/Fists_Block.Fists_Block" true))))))
        (:NewEnumerator0
          (Components|DestroyComponent (Variables|Default|Get1HOffhand))
          ;[1 1 1] MHS
          (switch int (Variables|SetupInGame|GetAnimationNumber)
            (:0
              (Components|Animation|PlayAnimation (Variables|Default|GetMesh) "/Game/FlexibleCombatSystem/Animation/UE4-Mannequin/MainAndShield/Locomotion/MHS_Idle.MHS_Idle" true))
            (:1
              (Components|Animation|PlayAnimation (Variables|Default|GetMesh) "/Game/FlexibleCombatSystem/Animation/UE4-Mannequin/MainAndShield/Locomotion/Forwards/MHS_JogFwds.MHS_JogFwds" true))
            (:2
              (Components|Animation|PlayAnimation (Variables|Default|GetMesh) "/Game/FlexibleCombatSystem/Animation/UE4-Mannequin/MainAndShield/Brake/MHS_BrakeFwds.MHS_BrakeFwds" true))
            (:3
              (Components|Animation|PlayAnimation (Variables|Default|GetMesh) "/Game/FlexibleCombatSystem/Animation/UE4-Mannequin/MainAndShield/M_MHS_LightAttack_01.M_MHS_LightAttack_01" true))
            (:4
              (Components|Animation|PlayAnimation (Variables|Default|GetMesh) "/Game/FlexibleCombatSystem/Animation/UE4-Mannequin/MainAndShield/M_MHS_LightAttack_02.M_MHS_LightAttack_02" true))
            (:5
              (Components|Animation|PlayAnimation (Variables|Default|GetMesh) "/Game/FlexibleCombatSystem/Animation/UE4-Mannequin/MainAndShield/M_MHS_LightAttack_03.M_MHS_LightAttack_03" true))
            (:6
              (Components|Animation|PlayAnimation (Variables|Default|GetMesh) "/Game/FlexibleCombatSystem/Animation/UE4-Mannequin/MainAndShield/Combat/MHS_LightAttack_04.MHS_LightAttack_04" true))
            (:7
              (Components|Animation|PlayAnimation (Variables|Default|GetMesh) "/Game/FlexibleCombatSystem/Animation/UE4-Mannequin/MainAndShield/M_MHS_HeavyAttack_01.M_MHS_HeavyAttack_01" true))
            (:8
              (Components|Animation|PlayAnimation (Variables|Default|GetMesh) "/Game/FlexibleCombatSystem/Animation/UE4-Mannequin/MainAndShield/M_MHS_HeavyAttack_02.M_MHS_HeavyAttack_02" true))
            (:9
              (Components|Animation|PlayAnimation (Variables|Default|GetMesh) "/Game/FlexibleCombatSystem/Animation/UE4-Mannequin/Common/LungeAttack.LungeAttack" true))
            (:10
              (Components|Animation|PlayAnimation (Variables|Default|GetMesh) "/Game/FlexibleCombatSystem/Animation/UE4-Mannequin/MainAndShield/Combat/MHS_Block.MHS_Block" true))
            (:11
              (Components|Animation|PlayAnimation (Variables|Default|GetMesh) "/Game/FlexibleCombatSystem/Animation/UE4-Mannequin/MainAndShield/M_MHS_BreakBlockAttack.M_MHS_BreakBlockAttack" true))
            (:12
              (Components|Animation|PlayAnimation (Variables|Default|GetMesh) "/Game/FlexibleCombatSystem/Animation/UE4-Mannequin/MainAndShield/M_MHS_BlockBroken.M_MHS_BlockBroken" true))
            (:13
              (Components|Animation|PlayAnimation (Variables|Default|GetMesh) "/Game/FlexibleCombatSystem/Animation/UE4-Mannequin/MainAndShield/M_MHS_BlockImpact.M_MHS_BlockImpact" true))))
        (:NewEnumerator1
          (Components|DestroyComponent (Variables|Default|Get1HOffhand))
          ;[1 1 1] 2h
          (switch int (Variables|SetupInGame|GetAnimationNumber)
            (:0
              (Components|Animation|PlayAnimation (Variables|Default|GetMesh) "/Game/FlexibleCombatSystem/Animation/UE4-Mannequin/TwoHanded/Locomotion/2H_IdleLoco.2H_IdleLoco" true))
            (:1
              (Components|Animation|PlayAnimation (Variables|Default|GetMesh) "/Game/FlexibleCombatSystem/Animation/UE4-Mannequin/TwoHanded/Locomotion/Forwards/2H_JogFwds.2H_JogFwds" true))
            (:2
              (Components|Animation|PlayAnimation (Variables|Default|GetMesh) "/Game/FlexibleCombatSystem/Animation/UE4-Mannequin/TwoHanded/Brake/2H_BrakeFwds.2H_BrakeFwds" true))
            (:3
              (Components|Animation|PlayAnimation (Variables|Default|GetMesh) "/Game/FlexibleCombatSystem/Animation/UE4-Mannequin/TwoHanded/M_2H_LightAttack_01.M_2H_LightAttack_01" true))
            (:4
              (Components|Animation|PlayAnimation (Variables|Default|GetMesh) "/Game/FlexibleCombatSystem/Animation/UE4-Mannequin/TwoHanded/M_2H_LightAttack_02.M_2H_LightAttack_02" true))
            (:5
              (Components|Animation|PlayAnimation (Variables|Default|GetMesh) "/Game/FlexibleCombatSystem/Animation/UE4-Mannequin/TwoHanded/M_2H_LightAttack_03.M_2H_LightAttack_03" true))
            (:6
              (Components|Animation|PlayAnimation (Variables|Default|GetMesh) "/Game/FlexibleCombatSystem/Animation/UE4-Mannequin/TwoHanded/M_2H_LightAttack_04.M_2H_LightAttack_04" true))
            (:7
              (Components|Animation|PlayAnimation (Variables|Default|GetMesh) "/Game/FlexibleCombatSystem/Animation/UE4-Mannequin/TwoHanded/M_2H_HeavyAttack_01.M_2H_HeavyAttack_01" true))
            (:8
              (Components|Animation|PlayAnimation (Variables|Default|GetMesh) "/Game/FlexibleCombatSystem/Animation/UE4-Mannequin/TwoHanded/M_2H_HeavyAttack_02.M_2H_HeavyAttack_02" true))
            (:9
              (Components|Animation|PlayAnimation (Variables|Default|GetMesh) "/Game/FlexibleCombatSystem/Animation/UE4-Mannequin/Common/LungeAttack.LungeAttack" true))
            (:10
              (Components|Animation|PlayAnimation (Variables|Default|GetMesh) "/Game/FlexibleCombatSystem/Animation/UE4-Mannequin/TwoHanded/Combat/2H_Block.2H_Block" true))
            (:11
              (Components|Animation|PlayAnimation (Variables|Default|GetMesh) "/Game/FlexibleCombatSystem/Animation/UE4-Mannequin/TwoHanded/M_2H_BreakBlockAttack.M_2H_BreakBlockAttack" true))
            (:12
              (Components|Animation|PlayAnimation (Variables|Default|GetMesh) "/Game/FlexibleCombatSystem/Animation/UE4-Mannequin/TwoHanded/M_2H_BlockBreak.M_2H_BlockBreak" true))
            (:13
              (Components|Animation|PlayAnimation (Variables|Default|GetMesh) "/Game/FlexibleCombatSystem/Animation/UE4-Mannequin/TwoHanded/M_2H_BlockImpact.M_2H_BlockImpact" true))))
        (:NewEnumerator2
          (Components|DestroyComponent (Variables|Default|Get2h))
          ;[1 1 1] Dual Wield
          (switch int (Variables|SetupInGame|GetAnimationNumber)
            (:0
              (Components|Animation|PlayAnimation (Variables|Default|GetMesh) "/Game/FlexibleCombatSystem/Animation/UE4-Mannequin/Dual-Wield/Locomotion/DW_Idle.DW_Idle" true))
            (:1
              (Components|Animation|PlayAnimation (Variables|Default|GetMesh) "/Game/FlexibleCombatSystem/Animation/UE4-Mannequin/Dual-Wield/Locomotion/Forwards/DW_JogFwds.DW_JogFwds" true))
            (:2
              (Components|Animation|PlayAnimation (Variables|Default|GetMesh) "/Game/FlexibleCombatSystem/Animation/UE4-Mannequin/Dual-Wield/Brake/DW_BrakeFwds.DW_BrakeFwds" true))
            (:3
              (Components|Animation|PlayAnimation (Variables|Default|GetMesh) "/Game/FlexibleCombatSystem/Animation/UE4-Mannequin/Dual-Wield/Combat/DW_Attack_01.DW_Attack_01" true))
            (:4
              (Components|Animation|PlayAnimation (Variables|Default|GetMesh) "/Game/FlexibleCombatSystem/Animation/UE4-Mannequin/Dual-Wield/Combat/DW_Attack_02.DW_Attack_02" true))
            (:5
              (Components|Animation|PlayAnimation (Variables|Default|GetMesh) "/Game/FlexibleCombatSystem/Animation/UE4-Mannequin/Dual-Wield/Combat/DW_Attack_03.DW_Attack_03" true))
            (:6
              (Components|Animation|PlayAnimation (Variables|Default|GetMesh) "/Game/FlexibleCombatSystem/Animation/UE4-Mannequin/Dual-Wield/Combat/DW_Attack_04.DW_Attack_04" true))
            (:7
              (Components|Animation|PlayAnimation (Variables|Default|GetMesh) "/Game/FlexibleCombatSystem/Animation/UE4-Mannequin/Dual-Wield/M_DW_HeavyAttack_01.M_DW_HeavyAttack_01" true))
            (:8
              (Components|Animation|PlayAnimation (Variables|Default|GetMesh) "/Game/FlexibleCombatSystem/Animation/UE4-Mannequin/Dual-Wield/M_DW_HeavyAttack_02.M_DW_HeavyAttack_02" true))
            (:9
              (Components|Animation|PlayAnimation (Variables|Default|GetMesh) "/Game/FlexibleCombatSystem/Animation/UE4-Mannequin/Common/LungeAttack.LungeAttack" true))
            (:10
              (Components|Animation|PlayAnimation (Variables|Default|GetMesh) "/Game/FlexibleCombatSystem/Animation/UE4-Mannequin/Dual-Wield/Combat/DW_Block.DW_Block" true))
            (:11
              (Components|Animation|PlayAnimation (Variables|Default|GetMesh) "/Game/FlexibleCombatSystem/Animation/UE4-Mannequin/Dual-Wield/M_DW_BlockBreakAttack.M_DW_BlockBreakAttack" true))
            (:12
              (Components|Animation|PlayAnimation (Variables|Default|GetMesh) "/Game/FlexibleCombatSystem/Animation/UE4-Mannequin/Dual-Wield/Combat/DW_BlockBreak.DW_BlockBreak" true))
            (:13
              (Components|Animation|PlayAnimation (Variables|Default|GetMesh) "/Game/FlexibleCombatSystem/Animation/UE4-Mannequin/Dual-Wield/Combat/DW_BlockImpact.DW_BlockImpact" true))))
        (:NewEnumerator3
          (Components|DestroyComponent (Variables|Default|Get2h))
          ;[1 1 1] Duelist
          (switch int (Variables|SetupInGame|GetAnimationNumber)
            (:0
              (Components|Animation|PlayAnimation (Variables|Default|GetMesh) "/Game/FlexibleCombatSystem/Animation/UE4-Mannequin/Duelist-Left/Locomotion/1HL_Idle.1HL_Idle" true))
            (:1
              (Components|Animation|PlayAnimation (Variables|Default|GetMesh) "/Game/FlexibleCombatSystem/Animation/UE4-Mannequin/Duelist-Left/Locomotion/Forwards/1HL_JogFwds.1HL_JogFwds" true))
            (:2
              (Components|Animation|PlayAnimation (Variables|Default|GetMesh) "/Game/FlexibleCombatSystem/Animation/UE4-Mannequin/Duelist-Left/Brake/1HL_BrakeFwds.1HL_BrakeFwds" true))
            (:3
              (Components|Animation|PlayAnimation (Variables|Default|GetMesh) "/Game/FlexibleCombatSystem/Animation/UE4-Mannequin/Duelist-Left/Combat/1HL_LightAttack_01.1HL_LightAttack_01" true))
            (:4
              (Components|Animation|PlayAnimation (Variables|Default|GetMesh) "/Game/FlexibleCombatSystem/Animation/UE4-Mannequin/Duelist-Left/Combat/1HL_LightAttack_02.1HL_LightAttack_02" true))
            (:5
              (Components|Animation|PlayAnimation (Variables|Default|GetMesh) "/Game/FlexibleCombatSystem/Animation/UE4-Mannequin/Duelist-Left/M_1HL_LightAttack_03.M_1HL_LightAttack_03" true))
            (:6
              (Components|Animation|PlayAnimation (Variables|Default|GetMesh) "/Game/FlexibleCombatSystem/Animation/UE4-Mannequin/Duelist-Left/Combat/1HL_LightAttack_04.1HL_LightAttack_04" true))
            (:7
              (Components|Animation|PlayAnimation (Variables|Default|GetMesh) "/Game/FlexibleCombatSystem/Animation/UE4-Mannequin/Duelist-Left/Combat/1HL_HeavyAttack_01.1HL_HeavyAttack_01" true))
            (:8
              (Components|Animation|PlayAnimation (Variables|Default|GetMesh) "/Game/FlexibleCombatSystem/Animation/UE4-Mannequin/Duelist-Left/Combat/1HL_HeavyAttack_02.1HL_HeavyAttack_02" true))
            (:9
              (Components|Animation|PlayAnimation (Variables|Default|GetMesh) "/Game/FlexibleCombatSystem/Animation/UE4-Mannequin/Common/LungeAttack.LungeAttack" true))
            (:10
              (Components|Animation|PlayAnimation (Variables|Default|GetMesh) "/Game/FlexibleCombatSystem/Animation/UE4-Mannequin/TwoHanded/Combat/2H_Block.2H_Block" true))
            (:11
              (Components|Animation|PlayAnimation (Variables|Default|GetMesh) "/Game/FlexibleCombatSystem/Animation/UE4-Mannequin/Duelist-Left/Combat/1HL_BlockBreakAttack.1HL_BlockBreakAttack" true))
            (:12
              (Components|Animation|PlayAnimation (Variables|Default|GetMesh) "/Game/FlexibleCombatSystem/Animation/UE4-Mannequin/Duelist-Left/M_1HL_BlockBreak.M_1HL_BlockBreak" true))
            (:13
              (Components|Animation|PlayAnimation (Variables|Default|GetMesh) "/Game/FlexibleCombatSystem/Animation/UE4-Mannequin/Duelist-Left/M_1HL_BlockImpact.M_1HL_BlockImpact" true))))
        (:NewEnumerator5
          (Components|DestroyComponent (Variables|Default|Get2h))
          (switch int (Variables|SetupInGame|GetAnimationNumber)))))))

(fn ConstructionScript)