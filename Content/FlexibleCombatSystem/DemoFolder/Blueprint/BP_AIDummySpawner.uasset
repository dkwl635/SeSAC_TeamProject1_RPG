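; BP_AIDummySpawner is a demo actor that spawns a wave of four BP_AI_Dummy enemies and replaces it once all are dead.
; BeginPlay spawns the wave on authority at four component transforms, passing the shared AISetupData and itself in each dummy's ActorsToActivate.
; Interact checks on authority that every tracked dummy is dead, then after a short delay destroys them, clears the array and reuses the spawn logic.
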(event EventBeginPlay
  (Networking|SwitchHasAuthority
    (:Authority
      (for _array_element (Utilities|Array|MakeArray (Variables|Default|GetSpawn_24) (Variables|Default|GetSpawn_27) (Variables|Default|GetSpawn_28) (Variables|Default|GetSpawn_29))
        (bind _returnvalue (Game|SpawnActorfromClass "/Game/FlexibleCombatSystem/Blueprints/AI/Dummy/BP_AI_Dummy.BP_AI_Dummy_C" (Math|Transform|MakeTransform (Transformation|GetWorldLocation _array_element) (Transformation|GetWorldRotation _array_element) "1,1,1") "Undefined" 0 "NewEnumerator1" (Variables|Default|GetAI%20Setup%20Data) false (Utilities|Array|MakeArray self) 0 0 0 false 0))
        (Utilities|Array|Add (Variables|Default|GetAI) _returnvalue)))))

(event EventInteract
  (params (Character :type Character%20Object%20Reference))
  (bind _ai (Variables|Default|GetAI))
  (Networking|SwitchHasAuthority
    (:Authority
      (Variables|Default|SetAllDead true)
      (bind _array_element (Utilities|Array|ForEachLoopwithBreak (Variables|Default|GetAI) :!label _label)
        (:LoopBody
          (if (not (Variables|/Game/FlexibleCombatSystem/Blueprints/AI/BP_AI_Parent.BP_AI_Parent_C|GetDead _array_element))
            (Variables|Default|SetAllDead false)
            (goto _label Break)))
        (:Completed
          (if (Variables|Default|GetAllDead)
            (Utilities|FlowControl|Delay 2.0)
            (for _array_element_2 _ai
              (Actor|DestroyActor _array_element_2))
            (Utilities|Array|Clear _ai)
            (Networking|SwitchHasAuthority
              (:Authority
                (for _array_element_3 (Utilities|Array|MakeArray (Variables|Default|GetSpawn_24) (Variables|Default|GetSpawn_27) (Variables|Default|GetSpawn_28) (Variables|Default|GetSpawn_29))
                  (bind _returnvalue (Game|SpawnActorfromClass "/Game/FlexibleCombatSystem/Blueprints/AI/Dummy/BP_AI_Dummy.BP_AI_Dummy_C" (Math|Transform|MakeTransform (Transformation|GetWorldLocation _array_element_3) (Transformation|GetWorldRotation _array_element_3) "1,1,1") "Undefined" 0 "NewEnumerator1" (Variables|Default|GetAI%20Setup%20Data) false (Utilities|Array|MakeArray self) 0 0 0 false 0))
                  (Utilities|Array|Add (Variables|Default|GetAI) _returnvalue))))))))))

(fn ConstructionScript)