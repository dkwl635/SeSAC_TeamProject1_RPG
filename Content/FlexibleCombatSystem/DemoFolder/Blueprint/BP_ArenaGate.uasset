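; BP_ArenaGate is an interactable arena gate that raises to open, resets its linked ArenaSpawner and autosaves a checkpoint.
; A timeline slides the gate while Blocker collision toggles, with closing played in reverse at higher speed.
; The first opening saves through the GameMode and shows a checkpoint widget.
; InstantActivate snaps the gate open and shuts the save Gate node, preventing a repeat save after loading.
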(event Custom|OpenGates
  ;[1 1 1] Open/Close Gates
  (Utilities|FlowControl|Sequence
    (:then_0
      ;[1 1 1] Save Game Before First Arena
      (Utilities|FlowControl|DoOnce false
        (:Completed
          (Utilities|FlowControl|Gate false
            (:Exit
              (Utilities|FlowControl|Delay 0.2)
              (bind _returnvalue (Game|GetCurrentLevelName true))
              (Class|IGameMode|UpdateSaveSlot(Message) (Game|GetGameMode) "Autosave" _returnvalue)
              (Class|IGameMode|SaveCheckpoint(Message) (Game|GetGameMode) (Utilities|GetObjectName self))
              (bind _returnvalue_2 (UserInterface|CreateWidget "/Game/FlexibleCombatSystem/Widgets/General/WB_CheckpointReached.WB_CheckpointReached_C"))
              (UserInterface|Viewport|AddtoViewport _returnvalue_2 0))))))
    (:then_1
      (Collision|SetCollisionEnabled (Variables|Default|GetBlocker) "NoCollision")
      (Components|Timeline|SetPlayRate (Variables|Default|GetOpenLeGate) 1.0)
      (bind _newtrack_0 (Timeline|OpenLeGate PlayFromStart)
        (:Update
          (Transformation|SetRelativeLocation (Variables|Default|GetScene) (Math|Vector|Lerp(Vector) "0, 0, 0" "0, 0,250.000000" _newtrack_0) false false))))))

(event Custom|CloseGates
  ;[1 1 1] Open/Close Gates
  (Collision|SetCollisionEnabled (Variables|Default|GetBlocker) "QueryAndPhysics")
  (Components|Timeline|SetPlayRate (Variables|Default|GetOpenLeGate) 5.0)
  (bind _newtrack_0 (Timeline|OpenLeGate ReverseFromEnd)
    (:Update
      (Transformation|SetRelativeLocation (Variables|Default|GetScene) (Math|Vector|Lerp(Vector) "0, 0, 0" "0, 0,250.000000" _newtrack_0) false false))))

(event EventMCInteract
  ;[1 1 1] Open Gates & Save
  (CallFunction|OpenGates)
  (Default|ResetArena (Variables|Default|GetArenaSpawner)))

(event EventInstantActivate
  ;[1 1 1] Activate Instant (After Save)
  (Transformation|SetRelativeLocation (Variables|Default|GetScene) "0, 0,250.000000" false false)
  (Collision|SetCollisionEnabled (Variables|Default|GetBlocker) "NoCollision")
  ;[1 1 1] Save Game Before First Arena
  (Utilities|FlowControl|Gate false) ; enters at Close
)

(fn ConstructionScript)