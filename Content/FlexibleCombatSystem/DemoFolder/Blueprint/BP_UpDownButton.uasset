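; BP_UpDownButton is a demo pressure button that triggers a target actor when a Character overlaps its box.
; A timeline moves the mesh toward the LowerCube marker, then calls Activate when finished, with a Playing flag blocking re-triggers.
; Activate resets FloorButton and RangedPractise if that practice is valid and inactive; without one, it sends InteractMessage to ActorToActivate.
; The construction script positions LowerCube and picks a training material by button type.
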(event OnComponentBeginOverlap(Box)
  (params (OverlappedComponent :type Primitive%20Component%20Object%20Reference) (OtherActor :type Actor%20Object%20Reference) (OtherComp :type Primitive%20Component%20Object%20Reference) (OtherBodyIndex :type Integer) (bFromSweep :type Boolean) (SweepResult :type Hit%20Result%20Structure%20%28by%20ref%29))
  (bind _ascharacter (Utilities|Casting|CastToCharacter OtherActor))
  (Variables|Default|SetCHaracter _ascharacter)
  (if (not (Variables|Default|GetPlaying))
    (Variables|Default|SetPlaying true)
    (Variables|Default|SetRelative%20Location (Variables|/Script/Engine.SceneComponent|GetRelativeLocation (Variables|Default|GetStaticMesh)))
    (bind _newtrack_0 (Timeline|MoveButton PlayFromStart)
      (:Update
        (Transformation|SetRelativeLocation (Variables|Default|GetStaticMesh) (Math|Vector|Lerp(Vector) (Variables|Default|GetRelative%20Location) (Variables|/Script/Engine.SceneComponent|GetRelativeLocation (Variables|Default|GetLowerCube)) _newtrack_0) false false))
      (:Finished
        (CallFunction|Activate)
        (Variables|Default|SetPlaying false)))))

(event Custom|Activate
  (bind _ranged_practise (Variables|Default|GetRanged%20Practise))
  (Utilities|IsValid _ranged_practise
    (:Is%20Valid
      (if (not (Variables|/Game/FlexibleCombatSystem/DemoFolder/Blueprint/BP_RangedPractise.BP_RangedPractise_C|GetActive _ranged_practise))
        (Default|Reset (Variables|Default|GetFloorButton))
        (Default|Reset (Variables|Default|GetRanged%20Practise))))
    (:Is%20Not%20Valid
      (Class|IInteract|Interact(Message) (Variables|Default|GetActorToActivate) (Variables|Default|GetCHaracter)))))

(fn ConstructionScript
  (Transformation|SetRelativeLocation (Variables|Default|GetLowerCube) (Variables|Default|GetMoveLocation) false false)
  (if (Variables|Default|GetSystemsButton)
    (Rendering|Material|SetMaterial (Variables|Default|GetStaticMesh) 0 "/Game/FlexibleCombatSystem/DemoFolder/Materials/MI_SystemsTraining.MI_SystemsTraining")
    (else
      (Rendering|Material|SetMaterial (Variables|Default|GetStaticMesh) 0 (Utilities|Select :Index (Variables|Default|GetButtonType) :NewEnumerator0 "/Game/FlexibleCombatSystem/DemoFolder/Materials/MI_MeleeTraining.MI_MeleeTraining" :NewEnumerator1 "/Game/FlexibleCombatSystem/DemoFolder/Materials/MI_RangedTraining.MI_RangedTraining" :NewEnumerator2 "/Game/FlexibleCombatSystem/DemoFolder/Materials/MI_MagicTraining.MI_MagicTraining")))))