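; BP_TitleSpawner is a demo-folder actor in the Flexible Combat System that displays a title text in the level.
; Its construction script copies the Text variable into a TextRender component.
; Event graph events are empty, and the logic that would pass Text to a WB_TutorialTitleText widget and destroy the TextRender is disconnected, so it never runs.
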(event Collision|EventActorBeginOverlap
  (params (OtherActor :type Actor%20Object%20Reference)))

(event EventTick
  (params (DeltaSeconds :type Float%20%28single-precision%29)))

(event EventBeginPlay)

(fn ConstructionScript
  (Rendering|Components|TextRender|SetText (Variables|Default|GetTextRender) (Variables|Default|GetText)))