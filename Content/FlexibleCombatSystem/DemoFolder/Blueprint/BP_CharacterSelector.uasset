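; BP_CharacterSelector is a demo selector that rotates its Spinner component left or right one step at a time, tracking the position in SpinCount.
; Spin steps the yaw by 51.43 degrees, a seventh of a turn, using the SpinLeft timeline and shortest-path rotator lerp for both directions.
; A DoOnce blocks new spins until the timeline finishes.
; SpinCount wraps to 0 above 4, but to 6 below 0.
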(event Custom|Spin
  (params (Left/Right :type Boolean))
  (bind _spinner (Variables|Default|GetSpinner))
  (bind _returnvalue (Transformation|GetWorldRotation _spinner))
  (Utilities|FlowControl|DoOnce false :!label _label
    (:Completed
      (Variables|Default|SetSpinning true)
      (Variables|Default|SetWorldRotation (.yaw (Transformation|GetWorldRotation (Variables|Default|GetSpinner))))
      (if Left/Right
        (bind _result (Math|Integer|IncrementInt (Variables|Default|GetSpinCount))
          (:%20%20
            (if (> _result 4)
              (Variables|Default|SetSpinCount 0))
            (Variables|Default|SetWorldRotationDestination (- (.yaw _returnvalue) 51.43))
            (bind _newtrack_0 (Timeline|SpinLeft PlayFromStart)
              (:Update
                (Transformation|SetWorldRotation (Variables|Default|GetSpinner) (Math|Rotator|Lerp(Rotator) (Math|Rotator|MakeRotator 0.0 0.0 (Variables|Default|GetWorldRotation)) (Math|Rotator|MakeRotator 0.0 0.0 (Variables|Default|GetWorldRotationDestination)) _newtrack_0 true) false false))
              (:Finished
                (Variables|Default|SetSpinning false)
                (goto _label Reset)))))
        (else
          (bind _result_2 (Math|Integer|DecrementInt (Variables|Default|GetSpinCount))
            (:%20%20
              (if (< _result_2 0)
                (Variables|Default|SetSpinCount 6))
              (Variables|Default|SetWorldRotationDestination (+ (.yaw _returnvalue) 51.43))
              (Timeline|SpinLeft PlayFromStart))))))))

(fn ConstructionScript)