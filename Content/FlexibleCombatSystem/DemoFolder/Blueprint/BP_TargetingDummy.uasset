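; BP_TargetingDummy is a demo targeting dummy for the Flexible Combat System.
; On BeginPlay it sets the player/AI faction on its CombatStatusComponent, the only active logic in its graphs.
; Its character-style functions for death, wounding, companions, movement and data passing are stubs returning false, empty or default values.
; PassFactionType returns a fixed enum value and does not read the faction set on the component.
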(event EventBeginPlay
  (Variables|/Game/FlexibleCombatSystem/Blueprints/Components/CombatStatusComponent.CombatStatusComponent_C|SetPlayer/AI%20Faction (Variables|Default|GetCombatStatusComponent) "NewEnumerator1"))

(event Collision|EventActorBeginOverlap
  (params (OtherActor :type Actor%20Object%20Reference)))

(event EventTick
  (params (DeltaSeconds :type Float%20%28single-precision%29)))

(fn ConstructionScript)

(fn CharacterRevived
  (return false))

(fn CompanionDied
  (params (CompanionData :type Data%20Table%20Row%20Handle%20Structure))
  (return false))

(fn HasCompanion?
  (return false))

(fn IsDead
  (return false))

(fn IsFacingEnemy?
  (return false))

(fn IsMoving?
  (return false))

(fn IsWounded
  (return false))

(fn PassArmorMeshes
  (return 0 0 0 0 0 0 0 0 0 0 0))

(fn PassBody
  (return 0 0 0 0 0 0 0 0))

(fn PassCamera
  (return 0 0))

(fn PassCompanions
  (return 0))

(fn PassFactionType
  (return "NewEnumerator0"))

(fn PassMovementMode
  (return "MOVE_None"))

(fn PassPlayerController
  (return 0))

(fn PassRootMotion
  (return false))

(fn PassThumbstickAxis
  (return "0, 0, 0"))

(fn ProduceSaveTexture
  (params (SaveName :type Text))
  (return))

(fn SendDeath
  (params (KillerCharacterRef :type Actor%20Object%20Reference))
  (return false))

(fn UpdateCompanionWounded
  (params (Wounded :type Boolean) (Companion%20Data :type Data%20Table%20Row%20Handle%20Structure))
  (return false))

(fn UpdateMovementMode
  (params (MovementMode :type EMovementMode%20Enum :default "MOVE_None"))
  (return false))

(fn Wounded
  (params (KillerRef :type Actor%20Object%20Reference))
  (return false))