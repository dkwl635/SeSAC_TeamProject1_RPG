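; Pressure-plate floor button that triggers a linked actor when a character stands on it, styled for the Melee, Ranged, Magic or Systems training variants.
; Box overlaps play or reverse a timeline that moves the mesh toward or away from a lowered position.
; A completed press runs Activate on authority, locking the button and sending InteractMessage with the character to the linked actor until Reset.
; The construction script places the lowered marker and picks the material.
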(event OnComponentBeginOverlap(Box)
  (params (OverlappedComponent :type Primitive%20Component%20Object%20Reference) (OtherActor :type Actor%20Object%20Reference) (OtherComp :type Primitive%20Component%20Object%20Reference) (OtherBodyIndex :type Integer) (bFromSweep :type Boolean) (SweepResult :type Hit%20Result%20Structure%20%28by%20ref%29))
  (bind _ascharacter (Utilities|Casting|CastToCharacter OtherActor))
  (Variables|Default|SetAs%20Character _ascharacter)
  (Variables|Default|SetMoving true)
  (if (not (Variables|Default|GetLocked))
    (Variables|Default|SetRelative%20Location (Variables|/Script/Engine.SceneComponent|GetRelativeLocation (Variables|Default|GetStaticMesh)))
    (bind _newtrack_0 (Timeline|MoveButton Play)
      (:Update
        (Transformation|SetRelativeLocation (Variables|Default|GetStaticMesh) (Math|Vector|Lerp(Vector) (Variables|Default|GetRelative%20Location) (select (Variables|Default|GetMoving) (Variables|/Script/Engine.SceneComponent|GetRelativeLocation (Variables|Default|GetLowerCube)) "0, 0, 0") _newtrack_0) false false))
      (:Finished
        (if (Variables|Default|GetMoving)
          (Networking|SwitchHasAuthority
            (:Authority
              (CallFunction|Activate))))))))

(event OnComponentEndOverlap(Box)
  (params (OverlappedComponent :type Primitive%20Component%20Object%20Reference) (OtherActor :type Actor%20Object%20Reference) (OtherComp :type Primitive%20Component%20Object%20Reference) (OtherBodyIndex :type Integer))
  (Utilities|Casting|CastToCharacter OtherActor)
  (Variables|Default|SetMoving false)
  (if (not (Variables|Default|GetLocked))
    (Variables|Default|SetRelative%20Location (Variables|/Script/Engine.SceneComponent|GetRelativeLocation (Variables|Default|GetStaticMesh)))
    (bind _newtrack_0 (Timeline|MoveButton Reverse)
      (:Update
        (Transformation|SetRelativeLocation (Variables|Default|GetStaticMesh) (Math|Vector|Lerp(Vector) (Variables|Default|GetRelative%20Location) (select (Variables|Default|GetMoving) (Variables|/Script/Engine.SceneComponent|GetRelativeLocation (Variables|Default|GetLowerCube)) "0, 0, 0") _newtrack_0) false false))
      (:Finished
        (if (Variables|Default|GetMoving)
          (Networking|SwitchHasAuthority
            (:Authority
              (CallFunction|Activate))))))))

(event Custom|Activate
  (Variables|Default|SetLocked true)
  (Class|IInteract|Interact(Message) (Variables|Default|GetActor) (Variables|Default|GetAs%20Character)))

(event Custom|Reset
  (Transformation|SetRelativeLocation (Variables|Default|GetStaticMesh) "0, 0, 0" false false)
  (Variables|Default|SetLocked false)
  (bind _newtrack_0 (Timeline|MoveButton SetNewTime)
    (:Update
      (Transformation|SetRelativeLocation (Variables|Default|GetStaticMesh) (Math|Vector|Lerp(Vector) (Variables|Default|GetRelative%20Location) (select (Variables|Default|GetMoving) (Variables|/Script/Engine.SceneComponent|GetRelativeLocation (Variables|Default|GetLowerCube)) "0, 0, 0") _newtrack_0) false false))
    (:Finished
      (if (Variables|Default|GetMoving)
        (Networking|SwitchHasAuthority
          (:Authority
            (CallFunction|Activate)))))))

(fn ConstructionScript
  (Transformation|SetRelativeLocation (Variables|Default|GetLowerCube) (Variables|Default|GetMoveLocation) false false)
  (if (Variables|Default|GetSystemsRoom)
    (Rendering|Material|SetMaterial (Variables|Default|GetStaticMesh) 0 "/Game/FlexibleCombatSystem/DemoFolder/Materials/MI_SystemsTraining.MI_SystemsTraining")
    (else
      (Rendering|Material|SetMaterial (Variables|Default|GetStaticMesh) 0 (Utilities|Select :Index (Variables|Default|GetButtonType) :NewEnumerator0 "/Game/FlexibleCombatSystem/DemoFolder/Materials/MI_MeleeTraining.MI_MeleeTraining" :NewEnumerator1 "/Game/FlexibleCombatSystem/DemoFolder/Materials/MI_RangedButton.MI_RangedButton" :NewEnumerator2 "/Game/FlexibleCombatSystem/DemoFolder/Materials/MI_MagicButton.MI_MagicButton")))))