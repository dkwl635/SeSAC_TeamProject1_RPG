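; Blueprint interface for AI controllers in the Flexible Combat System, declaring the calls used to drive and query combat AI.
; Setters and events cover attack timers, strafing, blocks, arrow and spell readiness, attack style, crowd control and madness states.
; Pass and Has getters return behaviour, block cooldown, target, attack group, ranged capability and combat types.
; It declares signatures only, with default returns, leaving the logic to implementers.
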(fn PassBehaviour
  (return "NewEnumerator1"))

(fn BeginAttackTimer)

(fn EndAttackTimer)

(fn ToggleStrafe
  (params (ToggleOn :type Boolean)))

(fn BlockBreak)

(fn PassBlockCD
  (return false))

(fn HasTarget
  (return false))

(fn SetAttackGroupCheck
  (return))

(fn PassAttackGroup
  (return false))

(fn UpdateArrowLoaded
  (params (Loaded :type Boolean)))

(fn PassHasRangedAttacks
  (return false))

(fn UpdateAttackStyle
  (params (AttackStyle :type E_AttackStyle%20Enum :default "NewEnumerator0") (WeaponStyle :type E_WeaponType%20Enum :default "NewEnumerator2")))

(fn BlockedAttack)

(fn SpellCharged)

(fn UpdateSpellCharged
  (params (Charged :type Boolean)))

(fn MadnessOver)

(fn MadnessTargetDead
  (params (DeadTarget :type Actor%20Object%20Reference)))

(fn MadnessActive)

(fn UpdateCrowdControlled
  (params (Active :type Boolean)))

(fn PassCombatTypes
  (params (AttackStyle :type E_AttackStyle%20Enum :default "NewEnumerator0") (WeaponType :type E_WeaponType%20Enum :default "NewEnumerator2"))
  (return))