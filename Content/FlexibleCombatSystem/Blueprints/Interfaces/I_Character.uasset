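; Blueprint interface for characters in the Flexible Combat System, letting other objects query and drive players and enemies without casting.
; State queries cover death, player identity, facing, movement, weapon range, draw state and attack style.
; Commands handle player setup, ranged aim camera, inventory camera, control locking, XP, movement mode, death and enemy HUD removal.
; Further functions cover assassination eligibility, cameras and components, plus access to body and armor meshes.
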(fn GetWeaponRange
  (return 0.0))

(fn IsPlayer?
  (return false))

(fn IsDead
  (return false))

(fn IsFacingEnemy?
  (return false))

(fn SendDeath
  (return))

(fn IsWeaponDrawn?
  (return false))

(fn UpdateRangedAim
  (params (TargetArmCurrent :type Float%20%28single-precision%29) (TargetArmDestination :type Float%20%28single-precision%29) (CameraLocationCurrent :type Vector) (CameraLocationDestination :type Vector) (CameraRotationCurrent :type Rotator) (CameraRotationDestination :type Rotator)))

(fn InitializePlayer)

(fn PassArmorMeshes
  (return 0 0 0 0 0 0 0 0 0 0 0))

(fn RetrievePlayerStatus
  (return false "NewEnumerator2" "NewEnumerator0"))

(fn ToggleInventoryCamera!
  (params (ToggleOn :type Boolean)))

(fn IncreaseXP
  (params (XP%20Amount :type Integer)))

(fn SetDisableControls
  (params (DisableMovement :type Boolean) (DisableCamera :type Boolean))
  (return))

(fn PassCamera
  (return 0 0))

(fn IsMoving?
  (return false))

(fn UpdateMovementMode
  (params (MovementMode :type EMovementMode%20Enum :default "MOVE_None"))
  (return false))

(fn PassMovementMode
  (return "MOVE_None"))

(fn FindAvailableAssassinationCam
  (return 0))

(fn RemoveEnemyHUD
  (return))

(fn PassAssassinationComps
  (return 0 0))

(fn CanbeAssassinated
  (return false))

(fn PassBody
  (return 0 0 0 0 0 0 0 0))