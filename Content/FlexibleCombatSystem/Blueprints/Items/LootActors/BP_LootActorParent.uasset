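; Parent Blueprint for lootable actors in the Flexible Combat System, exposing loot, outline and inventory info to other systems.
; On interact, if not yet looted, it opens the loot menu with its LootComponent, flags it for saving and triggers an animation hook, which is empty here.
; For dropped loot, DroppedItemToggle registers or clears the actor as the player inventory component's DropContainer.
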(event EventInteract
  (params (Character :type Character%20Object%20Reference))
  (bind _lootcomponent (Variables|Default|GetLootComponent))
  ;[1 1 1] Interact - Open Loot
  (if (not (Variables|/Game/FlexibleCombatSystem/Blueprints/Components/LootComponent.LootComponent_C|GetActorLooted (Variables|Default|GetLootComponent)))
    ;;[1 1 1] Open Loot Menu & Save Data
    (Class|IPlayerController|ToggleLootMenu(Message) (Game|GetPlayerController 0) _lootcomponent)
    (Default|LootWorthSaving _lootcomponent)
    (Class|ILootInterface|ToggleAnimation(Message) self)))

(event EventToggleAnimation
  ;[1 1 1] Interact - Open Loot
)

(fn ConstructionScript)

(fn DroppedItemToggle
  (params (ToggleOn :type Boolean))
  (if (Variables|/Game/FlexibleCombatSystem/Blueprints/Components/LootComponent.LootComponent_C|GetDroppedLoot (Variables|Default|GetLootComponent))
    (if ToggleOn
      (bind _inventorycomponent (Class|IPlayerController|PassInventoryComp(Message) (Game|GetPlayerController 0)))
      (Variables|/Game/FlexibleCombatSystem/Blueprints/Components/InventoryComponent.InventoryComponent_C|SetDropContainer _inventorycomponent self)
      (else
        (bind _inventorycomponent_2 (Class|IPlayerController|PassInventoryComp(Message) (Game|GetPlayerController 0)))
        (Variables|/Game/FlexibleCombatSystem/Blueprints/Components/InventoryComponent.InventoryComponent_C|SetDropContainer _inventorycomponent_2 0)))))

(fn RetrieveInventoryInfo
  (return "NewEnumerator0" "" 0 0 false 0 0))

(fn RetrieveLootInfo
  (return (Variables|SetupinGame|GetLootSetupInfo)))

(fn RetrieveOutlineInfo
  (bind _lootsetupinfo (Variables|SetupinGame|GetLootSetupInfo))
  (bind (_lootname _rarityoflootcolour) (Utilities|Struct|BreakS_LootSetupInfo _lootsetupinfo))
  (return _lootname _rarityoflootcolour "NewEnumerator1" 0 (Variables|Default|GetItem) (Variables|Default|GetItem2) 0))