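; Base actor for spells in the combat system, with mostly empty charge, release, load and send events as hooks for child spells.
; Initialize sets the Niagara effect, caches the caster's camera, components and mesh, then begins charging; triggering spends mana once.
; Helpers position a surface placement marker, solve projectile velocity from camera traces or an AI's target, and on interruption reset input then trigger or load the next spell.
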(event Custom|BeginMagicCharge
  ;[1 1 1] Begin Charge - Called When Spell Created
)

(event Custom|StopMagicCharge
  ;[1 1 1] Stop Magic Charge - Called When Spell Released
)

(event Custom|SendMagicSpell
  ;[1 1 1] Send Magic Spell - Called When Spell Tries To Fire
)

(event Custom|TriggerMagicSpell
  ;[1 1 1] Trigger Magic Spell - Called when Anim Notify Fires Spell
  (Utilities|FlowControl|DoOnce false
    (:Completed
      (Default|ReduceMana (Variables|Default|GetMagicComponent)))))

(event Custom|ReleaseSpellChannel
  ;[1 1 1] Release Spell Channel - Called When Left MB Released
)

(event Custom|DestroySpell
  ;[1 1 1] Destroy Self - Called When Spell Getting Destroyed
  (Utilities|FlowControl|DoOnce false
    (:Completed
      (Actor|DestroyActor))))

(event Custom|Initialize
  (params (SpellInfo :type S%20Spell%20Info%20Structure) (NiagaraSystem :type Niagara%20System%20Object%20Reference))
  ;[1 1 1] Setup & Initialize
  (Variables|SpellInfo|SetSpellInfo SpellInfo)
  (Variables|Default|SetNiagara%20System%20Ref NiagaraSystem)
  (Class|NiagaraComponent|SetAsset (Variables|Default|GetNiagaraSystem) NiagaraSystem true)
  (Components|Activation|Activate (Variables|Default|GetNiagaraSystem) false)
  (CallFunction|SetupVariables&References)
  (CallFunction|BeginMagicCharge))

(event Custom|LoadSpell
  (params (TimeRemaining :type Float%20%28single-precision%29))
  ;[1 1 1] Load Spell - Called When Spell Load Game Creates Spells Again
)

(fn ConstructionScript)

(fn UpdateSpellPlacement
  (bind _magiccomponent (Variables|Default|GetMagicComponent))
  (bind _followcamera (Variables|References|GetFollowCamera))
  (bind _returnvalue (Transformation|GetWorldLocation _followcamera))
  (bind _spellplacementps (Variables|/Game/FlexibleCombatSystem/Blueprints/Components/MagicComponent.MagicComponent_C|GetSpellPlacementPS _magiccomponent))
  (Utilities|IsValid (Variables|/Game/FlexibleCombatSystem/Blueprints/Components/MagicComponent.MagicComponent_C|GetSpellPlacementPS (Variables|Default|GetMagicComponent))
    (:Is%20Valid
      ;[1 1 1] Sets Marker For Spell Placement
      (Niagara|SetNiagaraVariable(Float) (Variables|/Game/FlexibleCombatSystem/Blueprints/Components/MagicComponent.MagicComponent_C|GetSpellPlacementPS (Variables|Default|GetMagicComponent)) "User.Size" (Utilities|Struct|BreakS_SpellPlacement (.SpellPlacement (Utilities|Struct|BreakS_SpellInfo (Variables|SpellInfo|GetSpellInfo)))))
      (if (Variables|Default|GetAI_Spell)
        (bind _ascharacter (Utilities|Casting|CastToCharacter (Variables|Default|GetEnemyTarget)))
        (Variables|Default|SetSpellPlacementLocation (Transformation|GetWorldLocation (Variables|/Script/Engine.Character|GetMesh _ascharacter)))
        (Transformation|SetWorldTransform (Variables|/Game/FlexibleCombatSystem/Blueprints/Components/MagicComponent.MagicComponent_C|GetSpellPlacementPS (Variables|Default|GetMagicComponent)) (Math|Transform|MakeTransform (Variables|Default|GetSpellPlacementLocation) "0, 0, 0" "1,1,1") false false)
        (else
          (bind (_outhit _returnvalue_2) (Collision|LineTraceByChannel _returnvalue (+ _returnvalue (* (Math|Vector|GetForwardVector _followcamera) (+ (Math|Conversions|ToFloat(Integer) (.Range (Utilities|Struct|BreakS_SpellInfo (Variables|SpellInfo|GetSpellInfo)))) (Math|Vector|Distance(Vector) (Transformation|GetWorldLocation (Variables|References|GetFollowCamera)) (Transformation|GetActorLocation (Variables|References|GetCharacterActorRef)))))) "TraceTypeQuery1" false (Utilities|Array|MakeArray (Variables|References|GetCharacterActorRef)) "None"))
          (if _returnvalue_2
            (if (Math|Vector|Equal(Vector) (.Y (Math|Rotator|BreakRotIntoAxes (Math|Rotator|MakeRotfromZ (.ImpactNormal (Collision|BreakHitResult _outhit))))) "1.000000, 0, 0" 0.0001)
              (Variables|Default|SetSpellPlacementLocation (.ImpactPoint (Collision|BreakHitResult _outhit)))
              (Development|SetHiddeninGame _spellplacementps false false)
              (Transformation|SetWorldTransform _spellplacementps (Math|Transform|MakeTransform (Variables|Default|GetSpellPlacementLocation) (Math|Rotator|MakeRotfromZ (.ImpactNormal (Collision|BreakHitResult _outhit))) "1,1,1") false false)
              (else
                (Development|SetHiddeninGame _spellplacementps true false :!label _label)))
            (else
              (goto _label))))))))

(fn CalculateSpellVelocity
  ;[1 1 1] Calculates Required Spell Velocity
  (if (Variables|Default|GetAI_Spell)
    ;[1 1 1] Calculate Projectile For Enemy AI
    (bind _tossvelocity (Class|GameplayStatics|BlueprintSuggestProjectileVelocity (Transformation|GetActorLocation) (Transformation|GetActorLocation (Variables|Default|GetEnemyTarget)) (Utilities|Struct|BreakS_SpellProjectile (.SpellProjectile (Utilities|Struct|BreakS_SpellInfo (Variables|SpellInfo|GetSpellInfo)))) 1.0 "DoNotTrace" 0.0 false false))
    (Variables|SpellInfo|SetSpellVelocity _tossvelocity)
    (else
      (bind (_outhit _returnvalue) (Collision|LineTraceByChannel (CallFunction|GetCameraLocation) (CallFunction|GetCameraForward) "TraceTypeQuery3" false (Utilities|Array|MakeArray (Variables|References|GetCharacterActorRef)) "None"))
      (bind _tossvelocity_2 (Class|GameplayStatics|BlueprintSuggestProjectileVelocity (Transformation|GetActorLocation) (Math|Vector|SelectVector (.ImpactPoint (Collision|BreakHitResult _outhit)) (.TraceEnd (Collision|BreakHitResult _outhit)) _returnvalue) (Utilities|Struct|BreakS_SpellProjectile (.SpellProjectile (Utilities|Struct|BreakS_SpellInfo (Variables|SpellInfo|GetSpellInfo)))) 1.0 "DoNotTrace" 0.0 false false))
      (Variables|SpellInfo|SetSpellVelocity _tossvelocity_2))))

(fn GetCameraRelative
  (return (- (Transformation|GetWorldLocation (Variables|References|GetFollowCamera)) (Transformation|GetActorLocation (Game|GetPlayerCharacter 0)))))

(fn GetCameraLocation
  ;[1 1 1] Gets Camera Location With Character Taken Into Account
  (return (+ (Math|Vector|GetForwardVector (Pawn|GetControlRotation (Game|GetPlayerCharacter 0) :!class /Script/Engine.Pawn)) (+ (CallFunction|GetCameraRelative) (Transformation|GetActorLocation (Game|GetPlayerCharacter 0))))))

(fn GetCameraForward
  ;[1 1 1] Gets Distance In Front Of Camera
  (return (+ (Transformation|GetWorldLocation (Variables|References|GetFollowCamera)) (* (Math|Vector|GetForwardVector (Pawn|GetControlRotation (Game|GetPlayerCharacter 0) :!class /Script/Engine.Pawn)) 3e+03))))

(fn GetCameraPlayerLevel
  (bind _camerarelative (CallFunction|GetCameraRelative))
  (bind _returnvalue (Game|GetPlayerCharacter 0))
  (bind _returnvalue_2 (Transformation|GetActorLocation _returnvalue))
  (bind _returnvalue_3 (+ _camerarelative _returnvalue_2))
  (return (+ (* (Math|Vector|GetForwardVector (Pawn|GetControlRotation (Game|GetPlayerCharacter 0) :!class /Script/Engine.Pawn)) (Math|Vector|VectorLength (- (Transformation|GetActorLocation _returnvalue) _returnvalue_3))) _returnvalue_3)))

(fn SetupVariables&References
  (bind _characteractorref (Variables|References|GetCharacterActorRef))
  (bind _camera (Class|ICharacter|PassCamera(Message) (Game|GetPlayerCharacter 0)))
  (Variables|References|SetFollowCamera _camera)
  (Variables|Default|SetMagicComponent (Actor|GetComponentbyClass _characteractorref "/Game/FlexibleCombatSystem/Blueprints/Components/MagicComponent.MagicComponent_C"))
  (Variables|Default|SetEquipmentComponent (Actor|GetComponentbyClass _characteractorref "/Game/FlexibleCombatSystem/Blueprints/Components/EquipmentComponent.EquipmentComponent_C"))
  (Variables|Default|SetInputBufferComponent (Actor|GetComponentbyClass _characteractorref "/Game/FlexibleCombatSystem/Blueprints/Components/InputBufferComponent.InputBufferComponent_C"))
  (bind _ascharacter (Utilities|Casting|CastToCharacter _characteractorref))
  (bind _output_get (Variables|References|SetCharacterRef _ascharacter))
  (Variables|References|SetCharacterMesh (Variables|/Script/Engine.Character|GetMesh _output_get)))

(fn RemovePlacementMarker
  (bind _magiccomponent (Variables|Default|GetMagicComponent))
  (bind _spellplacementps (Variables|/Game/FlexibleCombatSystem/Blueprints/Components/MagicComponent.MagicComponent_C|GetSpellPlacementPS _magiccomponent))
  (Utilities|IsValid _spellplacementps
    (:Is%20Valid
      (Components|DestroyComponent _spellplacementps))))

(fn Spell-Interupted
  (bind _inputbuffercomponent (Variables|Default|GetInputBufferComponent))
  ;[1 1 1] Reset Variables To Allow Us To Charge Next Spell
  (Variables|/Game/FlexibleCombatSystem/Blueprints/Components/InputBufferComponent.InputBufferComponent_C|SetConsumeInputBuffer _inputbuffercomponent "NewEnumerator4")
  (Variables|/Game/FlexibleCombatSystem/Blueprints/Components/MeleeComponent.MeleeComponent_C|SetStunned (Variables|/Game/FlexibleCombatSystem/Blueprints/Components/InputBufferComponent.InputBufferComponent_C|GetMeleeComponent _inputbuffercomponent) false)
  ;[1 1 1] Trigger Spell IF Buff/Heal/Teleport
  (if (Utilities|Enum|Equal(Enum) (.SpellCategory (Utilities|Struct|BreakS_SpellInfo (Variables|SpellInfo|GetSpellInfo))) "NewEnumerator6")
    (Default|TriggerMagicSpell (Variables|Default|GetMagicComponent)) ; Trigger Buffs, Heals, Teleport Instantly
    (else
      ;[1 1 1] Load Next Spell
      (Default|NextSpell (Variables|Default|GetMagicComponent)))))