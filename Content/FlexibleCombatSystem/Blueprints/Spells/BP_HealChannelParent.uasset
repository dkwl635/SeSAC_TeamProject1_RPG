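; BP_HealChannelParent is a base Blueprint for channeled healing spells that restore the user's health over time.
; Each spell tick reduces mana through MagicComponent and adds the SpellInfo amount to EquipmentComponent's Health, capped at MaxHealth.
; The tick then broadcasts the health update and spawns a WB_CombatText widget showing the rounded amount at player 0's location.
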(event EventActivateSpellTick
  (bind _equipmentcomponent (Variables|Default|GetEquipmentComponent))
  (bind _spellinfo (Variables|Default|GetSpellInfo))
  (bind _spelldurations (Utilities|Struct|BreakS_SpellInfo _spellinfo))
  (bind _maxhealth (Variables|/Game/FlexibleCombatSystem/Blueprints/Components/EquipmentComponent.EquipmentComponent_C|GetMaxHealth _equipmentcomponent))
  (bind _spellamount (Utilities|Struct|BreakS_DurationSpells _spelldurations))
  ;[1 1 1] Heals the User Over Time
  (Default|ReduceMana (Variables|Default|GetMagicComponent))
  (bind _output_get (Variables|/Game/FlexibleCombatSystem/Blueprints/Components/EquipmentComponent.EquipmentComponent_C|SetHealth _equipmentcomponent (+ (Variables|/Game/FlexibleCombatSystem/Blueprints/Components/EquipmentComponent.EquipmentComponent_C|GetHealth (Variables|Default|GetEquipmentComponent)) _spellamount)))
  (if (> _output_get _maxhealth)
    (Variables|/Game/FlexibleCombatSystem/Blueprints/Components/EquipmentComponent.EquipmentComponent_C|SetHealth _equipmentcomponent _maxhealth))
  (Default|UpdateHealthDispatch _equipmentcomponent)
  (bind _returnvalue (UserInterface|CreateWidget "/Game/FlexibleCombatSystem/Widgets/Combat/WB_CombatText.WB_CombatText_C" 0 (Transformation|GetActorLocation (Game|GetPlayerCharacter 0)) (Math|Float|Round _spellamount) "NewEnumerator13"))
  (UserInterface|Viewport|AddtoViewport _returnvalue 0))

(fn ConstructionScript
  (|CallParentFunction))