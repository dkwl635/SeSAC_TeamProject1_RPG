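; BP_SelfCastSpell is a spell Blueprint for self-cast magic in the Flexible Combat System, handling charge, cast and trigger.
; Charge events toggle a Niagara effect, and sending clears the placement timer, plays the charge sound and casting montage, and calls SpellInterupted on interruption.
; An animation-driven trigger fires once, calling the empty SpellEffect event and playing the fire sound.
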(event Custom|SpellEffect
  ;[1 1 1] Trigger Spell Attack (Triggered From Animation)
)

(event EventBeginMagicCharge
  ;[1 1 1] Start Charge
  (Components|Activation|Activate (Variables|Default|GetNiagara_0) false))

(event EventStopMagicCharge
  ;[1 1 1] Release Charge
  (Components|Activation|Deactivate (Variables|Default|GetNiagara_0)))

(event EventSendMagicSpell
  ;[1 1 1] Send Animation Spell
  (Utilities|Time|ClearandInvalidateTimerbyHandle (Variables|Default|GetSpellPlacementTimer))
  (Audio|SpawnSoundatLocation (Utilities|Struct|BreakS_SpellSounds (Utilities|Struct|BreakS_SpellInfo (Variables|Default|GetSpellInfo))) (Transformation|GetActorLocation) "0, 0, 0" 1.0 1.0 0.0 0 0)
  (Animation|Montage|PlayMontage (Variables|Default|GetCharacterMesh) (Utilities|Struct|BreakS_SpellInfo (Variables|Default|GetSpellInfo))
    (:OnInterrupted
      (CallFunction|Spell-Interupted))))

(event EventTriggerMagicSpell
  ;[1 1 1] Trigger Spell Attack (Triggered From Animation)
  (Utilities|FlowControl|DoOnce false
    (:Completed
      (CallFunction|SpellEffect)
      (Audio|SpawnSoundatLocation (Utilities|Struct|BreakS_SpellSounds (.SpellSoundFX (Utilities|Struct|BreakS_SpellInfo (Variables|Default|GetSpellInfo)))) (Transformation|GetActorLocation) "0, 0, 0" 1.0 1.0 0.0 0 0))))

(fn ConstructionScript
  (|CallParentFunction))