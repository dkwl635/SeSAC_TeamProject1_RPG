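; BP_RuneParent is a rune spell in the Flexible Combat System that places a physical rune in the world.
; When its SpellEffect event fires, it gets damage and a critical-hit result from MagicComponent using SpellInfo.
; It then spawns BP_PhysicalRune at the spell placement location, handing it the damage results, owning character, AI-caster flag and spell info.
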(event EventSpellEffect
  ;[1 1 1] Spell Effect
  (bind (_spell_damage _critical_hit) (Default|CalculateMagicDamage (Variables|Default|GetMagicComponent) (Variables|Default|GetSpellInfo)))
  (Variables|Default|SetSpellDamage _spell_damage)
  (Variables|Default|SetCriticalHit _critical_hit)
  (Game|SpawnActorfromClass "/Game/FlexibleCombatSystem/Blueprints/Spells/BP_PhysicalRune.BP_PhysicalRune_C" (Math|Transform|MakeTransform (Variables|Default|GetSpellPlacementLocation) "0, 0, 0" "1,1,1") "Undefined" 0 (Utilities|GetObjectName (Variables|Default|GetCharacterActorRef)) (Variables|Default|GetSpellDamage) (Variables|Default|GetCriticalHit) (Variables|Default|GetAI_Spell) (Variables|Default|GetCharacterActorRef) (Variables|Default|GetSpellInfo) 0))

(fn ConstructionScript
  (|CallParentFunction))