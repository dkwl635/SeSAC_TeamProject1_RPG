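; Parent Blueprint for channelled beam spells, used by players and AI, driven by charge, channel and release events.
; An animation-triggered event spawns a Niagara beam and starts a looping timer that scales down spell damage and drains mana.
; Each tick sphere-traces along the camera aim, or actor forward for AI, applying point damage.
; Spells with "Drain" in their name also heal the caster, while helpers manage charge and loop audio.
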(event Custom|ActivateSpellTick
  ;[1 1 1] Trigger Spell Attack (Triggered From Animation)
  (bind (_spell_damage _critical_hit) (Default|CalculateMagicDamage (Variables|Default|GetMagicComponent) (Variables|Default|GetSpellInfo)))
  (CallFunction|SpellChannelDmgAdjust _spell_damage)
  (Variables|Default|SetCriticalHit _critical_hit)
  (if (Variables|Default|GetAI_Spell)
    (CallFunction|ApplyAITraceDamage)
    (else
      (CallFunction|ApplyTraceDamage))))

(event EventBeginMagicCharge
  ;[1 1 1] Start Charge
  (Class|NiagaraComponent|SetAsset (Variables|Default|GetNiagaraLeftHand) (Variables|Default|GetNiagara%20System%20Ref) true)
  (CallFunction|RemovePlacementMarker)
  (Transformation|AttachComponentToComponent (Variables|Default|GetNiagaraLeftHand) (Variables|/Script/Engine.Character|GetMesh (Variables|Default|GetCharacterRef)) "LeftHandSpell" "SnapToTarget" "SnapToTarget" "SnapToTarget" true) ; Right PS Already Attached Via Root Of Current BP
  (Components|Activation|Activate (Variables|Default|GetNiagaraLeftHand) false)
  (CallFunction|SFXChannelCharge))

(event EventStopMagicCharge
  (bind _charactermesh (Variables|Default|GetCharacterMesh))
  ;[1 1 1] Release Charge - Right Mouse Button Release
  (CallFunction|DeactivateChannel)
  (Components|Activation|Deactivate (Variables|Default|GetNiagaraLeftHand))
  (CallFunction|StopAudio)
  (Default|CallEventSpellChanneling (Variables|Default|GetMagicComponent) false)
  (if (Variables|Default|GetChanneling)
    (Default|ClearBuffer (Variables|Default|GetInputBufferComponent) false) ; Channel End Anim Clears Buffer, As we're not playing it we need to clear
    (elif (CallFunction|IsPlayingMontage _charactermesh (Variables|Default|GetSpellEnd))
      (Audio|Components|Audio|Stop _charactermesh) ; Prevents Channel End Anim Playing
    )))

(event EventSendMagicSpell
  ;[1 1 1] Send Animation Spell - Loop Through Animation Until Release
  (CallFunction|CalculateAnimationEnd)
  (Default|CallEventSpellChanneling (Variables|Default|GetMagicComponent) true))

(event EventTriggerMagicSpell
  ;[1 1 1] Trigger Spell Attack (Triggered From Animation)
  (Variables|Default|SetChanneling true)
  (Components|Activation|Deactivate (Variables|Default|GetNiagaraLeftHand))
  (CallFunction|SpawnNiagaraChannel)
  (bind _returnvalue (Utilities|Time|SetTimerbyEvent (EventDispatchers|CreateEvent :!event Custom|ActivateSpellTick) (Variables|Default|GetChannelTickTime) true))
  (Variables|Default|SetSpellTickTimer _returnvalue)
  (CallFunction|SFXChannelLoop)
  (Class|AISenseHearing|ReportNoiseEvent (Variables|Default|GetSpellPlacementLocation) 1.0 (Variables|Default|GetCharacterActorRef) 5e+02 "None"))

(event EventReleaseSpellChannel
  (bind _channelloopsound (Variables|Default|GetChannelLoopSound))
  ;[1 1 1] Release Spell Channel - Left Mouse Button Release
  (Variables|Default|SetChanneling false)
  (CallFunction|DeactivateChannel)
  (Components|Activation|Activate (Variables|Default|GetNiagaraLeftHand) true)
  (Utilities|IsValid _channelloopsound
    (:Is%20Valid
      (Audio|Components|Audio|Stop _channelloopsound))
    (:Is%20Not%20Valid
      _))
  (CallFunction|SFXChannelCharge)
  ;;[1 1 1] Channel End Montage - Clears Buffer
  (Animation|Montage|PlayMontage (Variables|Default|GetCharacterMesh) (Variables|Default|GetSpellEnd)
    (:OnBlendOut
      _)
    (:OnInterrupted
      _))
  (Default|CallEventSpellChanneling (Variables|Default|GetMagicComponent) false)
  (CallFunction|Spell-Interupted))

(fn ConstructionScript
  (|CallParentFunction))

(fn ApplyTraceDamage
  (bind _location (CallFunction|GetCameraPlayerLevel))
  (bind _spellinfo (Variables|Default|GetSpellInfo))
  (bind _spellinfo_2 (Variables|Default|GetSpellInfo))
  (bind _followcamera (Variables|Default|GetFollowCamera))
  (bind _niagarachannel (Variables|Default|GetNiagaraChannel))
  (bind _range (Utilities|Struct|BreakS_SpellInfo _spellinfo_2))
  (bind (_damagetype _specialdamageinfo) (Utilities|Struct|BreakS_SpellInfo _spellinfo))
  (bind _returnvalue (Math|Vector|GetForwardVector _followcamera))
  (bind _returnvalue_2 (Math|Conversions|ToFloat(Integer) _range))
  (bind _returnvalue_3 (* _returnvalue _returnvalue_2))
  (bind _returnvalue_4 (+ _location _returnvalue_3))
  (bind _returnvalue_5 (Math|Rotator|FindLookatRotation _location _returnvalue_4))
  ;[1 1 1] Sets The Location Of The Damage Trace + NS
  (Utilities|Array|Clear (Variables|Default|GetDamageActor))
  (Transformation|SetWorldRotation _niagarachannel (Math|Rotator|MakeRotator (.roll _returnvalue_5) (.pitch _returnvalue_5) (+ (.yaw _returnvalue_5) 1e+01)) false false)
  (Niagara|SetNiagaraVariable(Vector3) _niagarachannel "User.BeamEnd" _returnvalue_4)
  (bind _outhits (Collision|MultiSphereTraceForObjects (Transformation|GetActorLocation (Variables|Default|GetCharacterRef)) _returnvalue_4 5e+01 (Utilities|Array|MakeArray "ObjectTypeQuery4") false (Utilities|Array|MakeArray (Variables|Default|GetCharacterActorRef)) "None"))
  ;[1 1 1] Deals The Damage
  (for _array_element _outhits
    (bind _dead (Class|ICharacter|IsDead(Message) (.HitActor (Collision|BreakHitResult _array_element))))
    (if (not _dead)
      (Utilities|IsValid (Actor|GetComponentbyClass (.HitActor (Collision|BreakHitResult _array_element)) "/Game/FlexibleCombatSystem/Blueprints/Components/TakingDamage.TakingDamage_C")
        (:Is%20Valid
          (if (not (Utilities|Array|ContainsItem (Variables|Default|GetDamageActor) (.HitActor (Collision|BreakHitResult _array_element))))
            (Utilities|Array|Add (Variables|Default|GetDamageActor) (.HitActor (Collision|BreakHitResult _array_element)))
            (Default|PassDamageInfo (Actor|GetComponentbyClass (.HitActor (Collision|BreakHitResult _array_element)) "/Game/FlexibleCombatSystem/Blueprints/Components/TakingDamage.TakingDamage_C") 0 "NewEnumerator19" _damagetype (Variables|Default|GetCriticalHit) _specialdamageinfo)
            (Game|Damage|ApplyPointDamage (.HitActor (Collision|BreakHitResult _array_element)) (Variables|Default|GetSpellDamage) (.ImpactPoint (Collision|BreakHitResult _array_element)) _array_element 0 (Variables|Default|GetCharacterActorRef))
            (CallFunction|DrainLife (.ImpactPoint (Collision|BreakHitResult _array_element))))))))
  (Default|ReduceMana (Variables|Default|GetMagicComponent)))

(fn CalculateAnimationEnd
  (bind _spellinfo (Variables|Default|GetSpellInfo))
  (bind (_name _animation) (Utilities|Struct|BreakS_SpellInfo _spellinfo))
  (Development|PrintString (Utilities|String|ToString(Text) _name))
  (if (== _animation "/Game/FlexibleCombatSystem/Animation/Magic/Channel/SpellChannel_1/M_SpellChannel1.M_SpellChannel1")
    (Variables|Default|SetSpellEnd "/Game/FlexibleCombatSystem/Animation/Magic/Channel/SpellChannel_1/M_SpellChannel1_End.M_SpellChannel1_End")
    (Default|CallEventSpellChannelNumber (Variables|Default|GetMagicComponent))
    (elif (== (Utilities|Struct|BreakS_SpellInfo (Variables|Default|GetSpellInfo)) "/Game/FlexibleCombatSystem/Animation/Magic/Channel/SpellChannel_1/M_SpellChannel1.M_SpellChannel1")
      (Default|CallEventSpellChannelNumber (Variables|Default|GetMagicComponent) 1))))

(fn ApplyAITraceDamage
  (bind _returnvalue (Transformation|GetActorLocation))
  (bind _characterref (Variables|Default|GetCharacterRef))
  (bind _spellinfo (Variables|Default|GetSpellInfo))
  (bind _spellinfo_2 (Variables|Default|GetSpellInfo))
  (bind _niagarachannel (Variables|Default|GetNiagaraChannel))
  (bind _range (Utilities|Struct|BreakS_SpellInfo _spellinfo_2))
  (bind (_damagetype _specialdamageinfo) (Utilities|Struct|BreakS_SpellInfo _spellinfo))
  (bind _returnvalue_2 (Transformation|GetActorForwardVector _characterref))
  (bind _returnvalue_3 (Math|Conversions|ToFloat(Integer) _range))
  (bind _returnvalue_4 (* _returnvalue_2 _returnvalue_3))
  (bind _returnvalue_5 (+ _returnvalue _returnvalue_4))
  ;[1 1 1] AI Channel - Same as Player But Different Math
  (Transformation|SetWorldRotation _niagarachannel (Math|Rotator|FindLookatRotation _returnvalue _returnvalue_5) false false)
  (Niagara|SetNiagaraVariable(Vector3) _niagarachannel "User.BeamEnd" _returnvalue_5)
  (bind _outhits (Collision|MultiSphereTraceForObjects (Transformation|GetActorLocation (Variables|Default|GetCharacterRef)) _returnvalue_5 5e+01 (Utilities|Array|MakeArray "ObjectTypeQuery3") false (Utilities|Array|MakeArray (Variables|Default|GetCharacterActorRef)) "None"))
  (for _array_element _outhits
    (Utilities|IsValid (Actor|GetComponentbyClass (.HitActor (Collision|BreakHitResult _array_element)) "/Game/FlexibleCombatSystem/Blueprints/Components/TakingDamage.TakingDamage_C")
      (:Is%20Valid
        (Default|PassDamageInfo (Actor|GetComponentbyClass (.HitActor (Collision|BreakHitResult _array_element)) "/Game/FlexibleCombatSystem/Blueprints/Components/TakingDamage.TakingDamage_C") 0 "NewEnumerator19" _damagetype (Variables|Default|GetCriticalHit) _specialdamageinfo)
        (Game|Damage|ApplyPointDamage (.HitActor (Collision|BreakHitResult _array_element)) (Variables|Default|GetSpellDamage) (.ImpactPoint (Collision|BreakHitResult _array_element)) _array_element 0 (Variables|Default|GetCharacterActorRef))
        (CallFunction|DrainLife "0, 0, 0"))))
  (Default|ReduceMana (Variables|Default|GetMagicComponent)))

(fn DrainLife
  (params (Location :type Vector))
  (bind _equipmentcomponent (Variables|Default|GetEquipmentComponent))
  (bind _equipmentcomponent_2 (Variables|Default|GetEquipmentComponent))
  (bind _equipmentcomponent_3 (Variables|Default|GetEquipmentComponent))
  (bind _maxhealth (Variables|/Game/FlexibleCombatSystem/Blueprints/Components/EquipmentComponent.EquipmentComponent_C|GetMaxHealth _equipmentcomponent_2))
  ;[1 1 1] IF Drain Life (Damage Type Not Best Indicator Name Would Be Better Once Decided Upon)
  (if (Utilities|String|Contains (Utilities|String|ToString(Text) (.Name (Utilities|Struct|BreakS_SpellInfo (Variables|Default|GetSpellInfo)))) "Drain")
    (Niagara|SpawnSystematLocation "/Game/FlexibleCombatSystem/VFX/MagicVFX/Channel/NS_DrainLifeHit.NS_DrainLifeHit" Location)
    ;[1 1 1] Drain Life
    (if (>= (Variables|/Game/FlexibleCombatSystem/Blueprints/Components/EquipmentComponent.EquipmentComponent_C|GetHealth _equipmentcomponent_2) _maxhealth)
      (Variables|/Game/FlexibleCombatSystem/Blueprints/Components/EquipmentComponent.EquipmentComponent_C|SetHealth (Variables|Default|GetEquipmentComponent) _maxhealth)
      (else
        (Variables|/Game/FlexibleCombatSystem/Blueprints/Components/EquipmentComponent.EquipmentComponent_C|SetHealth _equipmentcomponent (+ (Variables|/Game/FlexibleCombatSystem/Blueprints/Components/EquipmentComponent.EquipmentComponent_C|GetHealth _equipmentcomponent) (Variables|Default|GetSpellDamage)))))
    (Default|CallUpdateHealth _equipmentcomponent_3 (Variables|/Game/FlexibleCombatSystem/Blueprints/Components/EquipmentComponent.EquipmentComponent_C|GetHealth _equipmentcomponent_3) (Variables|/Game/FlexibleCombatSystem/Blueprints/Components/EquipmentComponent.EquipmentComponent_C|GetMaxHealth _equipmentcomponent_3))
    (bind _returnvalue (UserInterface|CreateWidget "/Game/FlexibleCombatSystem/Widgets/Combat/WB_CombatText.WB_CombatText_C" 0 (Transformation|GetActorLocation (Game|GetPlayerCharacter 0)) (Math|Float|Round (Variables|Default|GetSpellDamage)) "NewEnumerator13"))
    (UserInterface|Viewport|AddtoViewport _returnvalue 0)))

(fn DeactivateChannel
  (bind _niagarachannel (Variables|Default|GetNiagaraChannel))
  (Utilities|IsValid _niagarachannel
    (:Is%20Valid
      (Components|DestroyComponent _niagarachannel))
    (:Is%20Not%20Valid
      _))
  (Utilities|Time|ClearandInvalidateTimerbyHandle (Variables|Default|GetSpellTickTimer)))

(fn SFXChannelCharge
  (Utilities|IsValid (Variables|Default|GetChargeLoopSound)
    (:Is%20Valid
      (if (not (Audio|Components|Audio|IsPlaying (Variables|Default|GetChargeLoopSound)))
        (Audio|Components|Audio|Play (Variables|Default|GetChargeLoopSound) 0.0)))
    (:Is%20Not%20Valid
      (bind _returnvalue (Audio|SpawnSoundAttached (Utilities|Struct|BreakS_SpellSounds (.SpellSoundFX (Utilities|Struct|BreakS_SpellInfo (Variables|Default|GetSpellInfo)))) (Variables|Default|GetAbilityCollision) "None" "0, 0, 0" "0, 0, 0" "SnapToTarget" false 0.5 1.0 0.0 0 0))
      (bind _output_get (Variables|Default|SetChargeLoopSound _returnvalue))
      (Variables|/Script/Engine.AudioComponent|SetAttenuationSettings _output_get "/Game/FlexibleCombatSystem/SoundFX/SA_AttenuationMidFade.SA_AttenuationMidFade"))))

(fn SFXChannelLoop
  (bind _chargeloopsound (Variables|Default|GetChargeLoopSound))
  (Utilities|IsValid _chargeloopsound
    (:Is%20Valid
      (Audio|Components|Audio|Stop _chargeloopsound))
    (:Is%20Not%20Valid
      _))
  (Utilities|IsValid (Variables|Default|GetChannelLoopSound)
    (:Is%20Valid
      (if (not (Audio|Components|Audio|IsPlaying (Variables|Default|GetChannelLoopSound)))
        (Audio|Components|Audio|Play (Variables|Default|GetChannelLoopSound) 0.0)))
    (:Is%20Not%20Valid
      (bind _returnvalue (Audio|SpawnSoundAttached (Utilities|Struct|BreakS_SpellSounds (.SpellSoundFX (Utilities|Struct|BreakS_SpellInfo (Variables|Default|GetSpellInfo)))) (Variables|Default|GetAbilityCollision) "None" "0, 0, 0" "0, 0, 0" "SnapToTarget" false 0.5 1.0 0.0 0 0))
      (bind _output_get (Variables|Default|SetChannelLoopSound _returnvalue))
      (Variables|/Script/Engine.AudioComponent|SetAttenuationSettings _output_get "/Game/FlexibleCombatSystem/SoundFX/SA_AttenuationMidFade.SA_AttenuationMidFade"))))

(fn StopAudio
  (bind _chargeloopsound (Variables|Default|GetChargeLoopSound))
  (bind _channelloopsound (Variables|Default|GetChannelLoopSound))
  (Utilities|IsValid _channelloopsound
    (:Is%20Valid
      (Audio|Components|Audio|Stop _channelloopsound))
    (:Is%20Not%20Valid
      _))
  (Utilities|IsValid _chargeloopsound
    (:Is%20Valid
      (Audio|Components|Audio|Stop _chargeloopsound))))

(fn SpawnNiagaraChannel
  (bind _returnvalue (Niagara|SpawnSystemAttached (Utilities|Struct|BreakS_SpellChannel (.SpellChannel (Utilities|Struct|BreakS_SpellInfo (Variables|Default|GetSpellInfo)))) (Variables|Default|GetAbilityCollision) "None" "0, 0, 0" "0, 0, 0" "KeepRelativeOffset" false false))
  (Variables|Default|SetNiagaraChannel _returnvalue)
  (Transformation|SetWorldRotation (Variables|Default|GetNiagaraChannel) (Transformation|GetWorldRotation (Variables|/Script/Engine.Character|GetCapsuleComponent (Variables|Default|GetCharacterRef))) false false)
  (Niagara|SetNiagaraVariable(Vector3) (Variables|Default|GetNiagaraChannel) "User.BeamEnd" (Transformation|GetActorLocation))
  (Components|Activation|Activate (Variables|Default|GetNiagaraChannel) true))

(fn SpellChannelDmgAdjust
  (params (SpellDamage :type Float%20%28single-precision%29))
  ;[1 1 1] Spell Channel Scales too much with Intellect, must be brought down :-)
  (Variables|Default|SetSpellDamage (+ (/ SpellDamage 3.0) 4.0)))