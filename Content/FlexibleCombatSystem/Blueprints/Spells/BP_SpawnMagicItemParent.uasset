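; Parent spell actor for conjured-weapon spells that give the caster temporary magic weapons, with charge VFX, fire sound and cast montage.
; The animation-triggered spell event starts a duration buff matched to the weapon type, then spawns the weapon plus a second dagger, shield or magic arrows as needed.
; Items come from data table rows, take damage, effects and VFX from SpellInfo, and enter the inventory weightless and instantly equipped.
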(event EventBeginPlay
  (|CallParentFunction) ; This node is disabled and will not be called.\nDrag off pins to build functionality.
)

(event Collision|EventActorBeginOverlap
  (params (OtherActor :type Actor%20Object%20Reference))
  (|CallParentFunction OtherActor) ; This node is disabled and will not be called.\nDrag off pins to build functionality.
)

(event EventTick
  (params (DeltaSeconds :type Float%20%28single-precision%29))
  (|CallParentFunction DeltaSeconds) ; This node is disabled and will not be called.\nDrag off pins to build functionality.
)

(event EventBeginMagicCharge
  ;[1 1 1] Start Charge
  (Components|Activation|Activate (Variables|Default|GetNiagara) false))

(event EventStopMagicCharge
  ;[1 1 1] Release Charge
  (Components|Activation|Deactivate (Variables|Default|GetNiagara)))

(event EventSendMagicSpell
  ;[1 1 1] Send Animation Spell
  (Audio|SpawnSoundatLocation (Utilities|Struct|BreakS_SpellSounds (Utilities|Struct|BreakS_SpellInfo (Variables|Default|GetSpellInfo))) (Transformation|GetActorLocation) "0, 0, 0" 1.0 1.0 0.0 0 0)
  (Animation|Montage|PlayMontage (Variables|Default|GetCharacterMesh) (.Animation (Utilities|Struct|BreakS_SpellInfo (Variables|Default|GetSpellInfo)))))

(event EventTriggerMagicSpell
  ;[1 1 1] Trigger Spell Attack (Triggered From Animation)
  (|CallParentFunction)
  (CallFunction|CreateSpellDurationBar)
  (CallFunction|SpawnMagicItem)
  ;;[1 1 1] Spawn Off-Hand or Extra
  (switch Utilities|FlowControl|Switch|SwitchonE_SpawnWeaponType (Utilities|Struct|BreakS_SpawnWeaponInfo (.SpellSpawnWeapon (Utilities|Struct|BreakS_SpellInfo (Variables|Default|GetSpellInfo))))
    (:NewEnumerator3
      (CallFunction|SpawnMagicItem))
    (:NewEnumerator1
      (CallFunction|SpawnSpecificItem "/Game/FlexibleCombatSystem/DataTables/DT_ItemDataInfo.DT_ItemDataInfo" "MagicWep-Shield" 1))
    (:NewEnumerator2
      (CallFunction|SpawnSpecificItem "/Game/FlexibleCombatSystem/DataTables/DT_ItemDataInfo.DT_ItemDataInfo" "Arrow-Magic" 10))))

(fn ConstructionScript
  (|CallParentFunction))

(fn SpawnMagicItem
  (bind _spellinfo (Variables|Default|GetSpellInfo))
  (bind (_basedamage _spelldescription _damagetype _specialdamageinfo _spellspawnweapon) (Utilities|Struct|BreakS_SpellInfo _spellinfo))
  (bind (_weapondatatableinfo _weaponvfxinfo) (Utilities|Struct|BreakS_SpawnWeaponInfo _spellspawnweapon))
  ;[1 1 1] Spawn Weapon and Set its Values
  (bind _returnvalue (Utilities|GetDataTableRow (.datatable _weapondatatableinfo) (.rowname _weapondatatableinfo))
    (:then
      (bind _structout (Utilities|Struct|SetmembersinS_ItemData _returnvalue (Utilities|Text|ToText(String) (.RightS (Utilities|String|Split (Utilities|String|ToString(Text) (.Description (Utilities|Struct|BreakS_ItemDescription _spelldescription))) "Spawns"))) _weaponvfxinfo))
      (bind _structout_2 (Utilities|Struct|SetmembersinS_EquipmentInfo (.EquipmentInfo (Utilities|Struct|BreakS_ItemData _structout)) (Math|Conversions|ToFloat(Integer) _basedamage) _damagetype _specialdamageinfo))
      (bind _structout_3 (Utilities|Struct|SetmembersinS_ItemData _returnvalue _structout_2))
      (Default|AddtoInventory (Actor|GetComponentbyClass (Variables|Default|GetCharacterActorRef) "/Game/FlexibleCombatSystem/Blueprints/Components/InventoryComponent.InventoryComponent_C") (Utilities|Struct|MakeS_SlotInfo _structout_3 (Utilities|Struct|MakeDataTableRowHandle (.datatable _weapondatatableinfo) (.rowname _weapondatatableinfo)) 1) true true))))

(fn CreateSpellDurationBar
  (bind _spellinfo (Variables|Default|GetSpellInfo))
  (bind _characterref (Variables|Default|GetCharacterRef))
  (bind (_spellsoundfx _spelldescription _specialdamageinfo _spelldurations _spellspawnweapon) (Utilities|Struct|BreakS_SpellInfo _spellinfo))
  (Default|ActivateBuff :self (Actor|GetComponentbyClass _characterref "/Game/FlexibleCombatSystem/Blueprints/Components/BuffComponent.BuffComponent_C") :CharacterActorRef _characterref :BuffType (Utilities|Select :Index (.SpawnWeaponType (Utilities|Struct|BreakS_SpawnWeaponInfo _spellspawnweapon)) :NewEnumerator0 "NewEnumerator11" :NewEnumerator3 "NewEnumerator14" :NewEnumerator1 "NewEnumerator15" :NewEnumerator2 "NewEnumerator12") :BuffDuration (Utilities|Struct|BreakS_DurationSpells _spelldurations) :BarrierHitDamage 5.0 :Spawned%20Weapon true))

(fn SpawnSpecificItem
  (params (DataTable :type Data%20Table%20Object%20Reference) (RowName :type Name) (Quantity :type Integer))
  (bind _spellinfo (Variables|Default|GetSpellInfo))
  (bind (_basedamage _spellsoundfx _spelldescription _damagetype _specialdamageinfo) (Utilities|Struct|BreakS_SpellInfo _spellinfo))
  ;[1 1 1] Spawn Weapon and Set its Values
  (bind _returnvalue (Utilities|GetDataTableRow DataTable RowName)
    (:then
      (if (Utilities|Name|Equal(Name) RowName "Arrow-Magic")
        _
        (else
          (Utilities|Struct|SetmembersinS_ItemData _returnvalue (Utilities|Select :Index _damagetype :NewEnumerator0 "" :NewEnumerator1 (Utilities|Struct|MakeS_WeaponVFXInfo "/Game/FlexibleCombatSystem/VFX/MagicVFX/MagicWeapon/NE_Fire_Mesh.NE_Fire_Mesh" 6e+01 2e+01 1.5) :NewEnumerator2 "" :NewEnumerator8 (Utilities|Struct|MakeS_WeaponVFXInfo "/Game/FlexibleCombatSystem/VFX/MagicVFX/MagicWeapon/NE_Frost_Mesh.NE_Frost_Mesh" 6e+01) :NewEnumerator3 (Utilities|Struct|MakeS_WeaponVFXInfo "/Game/FlexibleCombatSystem/VFX/MagicVFX/MagicWeapon/NE_Lightning_Mesh.NE_Lightning_Mesh" 6e+01 2e+01 3.0 4.0) :NewEnumerator4 (Utilities|Struct|MakeS_WeaponVFXInfo "/Game/FlexibleCombatSystem/VFX/MagicVFX/MagicWeapon/NE_Poison_Mesh.NE_Poison_Mesh" 6e+01 2e+01 1.5) :NewEnumerator5 "" :NewEnumerator6 "" :NewEnumerator7 "" :NewEnumerator9 "")) ; Ignore if Magic Arrow, We Don't Want Flaming Quiver
        ))
      (bind _structout (Utilities|Struct|SetmembersinS_EquipmentInfo (.EquipmentInfo (Utilities|Struct|BreakS_ItemData _returnvalue)) (Math|Conversions|ToFloat(Integer) _basedamage) _damagetype _specialdamageinfo))
      (bind _structout_2 (Utilities|Struct|SetmembersinS_ItemData _returnvalue _structout))
      (Default|AddtoInventory (Actor|GetComponentbyClass (Variables|Default|GetCharacterActorRef) "/Game/FlexibleCombatSystem/Blueprints/Components/InventoryComponent.InventoryComponent_C") (Utilities|Struct|MakeS_SlotInfo _structout_2 (Utilities|Struct|MakeDataTableRowHandle DataTable RowName) Quantity) true true))))