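; Moving area-damage spell actor that glides toward its parent spell's placement location while its Niagara effect plays.
; A looping timer at the spell's tick frequency reports noise, sphere-traces around the actor, and damages each unique target with a TakingDamage component using MagicComponent's damage calculation, then reduces mana.
; Deactivation freezes the destination, stops the timer and effect, and destroys the actor five seconds later.
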(event Custom|Deactivate
  ;[1 1 1] Activate & Deactivate Damaging Spell
  (Variables|Default|SetFinalDestination (Variables|/Game/FlexibleCombatSystem/Blueprints/Spells/BP_AbilityParent.BP_AbilityParent_C|GetSpellPlacementLocation (Variables|Default|GetSpellParent)))
  (Variables|Default|SetDeactivating true)
  (Utilities|Time|ClearandInvalidateTimerbyHandle (stale EventBeginPlay _returnvalue))
  (Components|Activation|Deactivate (Variables|Default|GetNiagara))
  (Utilities|FlowControl|Delay 5.0)
  (Actor|DestroyActor))

(event Custom|ActivateSpellTick
  (bind _returnvalue (Transformation|GetActorLocation))
  (bind _spellinfo (Variables|Default|GetSpellInfo))
  (bind (_damagetype _specialdamageinfo) (Utilities|Struct|BreakS_SpellInfo _spellinfo))
  ;[1 1 1] Activate Spell Tick Damage
  (Class|AISenseHearing|ReportNoiseEvent (Variables|/Game/FlexibleCombatSystem/Blueprints/Spells/BP_AbilityParent.BP_AbilityParent_C|GetSpellPlacementLocation (Variables|Default|GetSpellParent)) 1.0 (Variables|Default|GetCharacterActorRef) 5e+02 "None")
  (Utilities|Array|Clear (Variables|Default|GetDamageEnemy))
  (bind (_spell_damage _critical_hit) (Default|CalculateMagicDamage (Variables|Default|GetMagicComponent) (Variables|Default|GetSpellInfo)))
  (Variables|Default|SetSpellDamage _spell_damage)
  (Variables|Default|SetCriticalHit _critical_hit)
  (bind _outhits (Collision|MultiSphereTraceForObjects _returnvalue _returnvalue (/ (Utilities|Struct|BreakS_SpellPlacement (.SpellPlacement (Utilities|Struct|BreakS_SpellInfo (Variables|Default|GetSpellInfo)))) 2.4) (Utilities|Array|MakeArray "ObjectTypeQuery4") false (Utilities|Array|MakeArray (Variables|Default|GetCharacterActorRef)) "None"))
  (for _array_element _outhits
    (Utilities|IsValid (Actor|GetComponentbyClass (.HitActor (Collision|BreakHitResult _array_element)) "/Game/FlexibleCombatSystem/Blueprints/Components/TakingDamage.TakingDamage_C")
      (:Is%20Valid
        (if (not (Utilities|Array|ContainsItem (Variables|Default|GetDamageEnemy) (.HitActor (Collision|BreakHitResult _array_element))))
          (Utilities|Array|Add (Variables|Default|GetDamageEnemy) (.HitActor (Collision|BreakHitResult _array_element)))
          (Default|PassDamageInfo (Actor|GetComponentbyClass (.HitActor (Collision|BreakHitResult _array_element)) "/Game/FlexibleCombatSystem/Blueprints/Components/TakingDamage.TakingDamage_C") 0 "NewEnumerator18" _damagetype (Variables|Default|GetCriticalHit) _specialdamageinfo)
          (Game|Damage|ApplyPointDamage (.HitActor (Collision|BreakHitResult _array_element)) (Variables|Default|GetSpellDamage) (.ImpactPoint (Collision|BreakHitResult _array_element)) _array_element 0 (Variables|Default|GetCharacterActorRef))))))
  (Default|ReduceMana (Variables|Default|GetMagicComponent)))

(event EventBeginPlay
  ;[1 1 1] Activate & Deactivate Damaging Spell
  (Class|NiagaraComponent|SetAsset (Variables|Default|GetNiagara) (Variables|Default|GetNiagaraPS) true)
  (bind _returnvalue (Utilities|Time|SetTimerbyEvent (delegate Custom|ActivateSpellTick) (Utilities|Struct|BreakS_SpellPlacement (Utilities|Struct|BreakS_SpellInfo (Variables|Default|GetSpellInfo))) true)))

(event EventTick
  (params (DeltaSeconds :type Float%20%28single-precision%29))
  ;[1 1 1] Update Spell Location
  (Transformation|SetActorLocation (Math|Interpolation|VInterpTo (Transformation|GetActorLocation) (select (Variables|Default|GetDeactivating) (Variables|Default|GetFinalDestination) (Variables|/Game/FlexibleCombatSystem/Blueprints/Spells/BP_AbilityParent.BP_AbilityParent_C|GetSpellPlacementLocation (Variables|Default|GetSpellParent))) DeltaSeconds (Variables|Default|GetMoveSpeed)) false false))

(fn ConstructionScript)