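; Parent Blueprint for placed spell attacks whose Niagara effect triggers a single area hit on enemies.
; SpellEffect calculates damage and crit via MagicComponent, spawns the spell's Niagara system and passes itself as User.BP_Spell for the particle callback.
; ParticleData fires once, sphere-tracing physics bodies at the placement point with a scaled-down spell radius.
; Each unique actor with a TakingDamage component, excluding the caster, receives damage info and point damage.
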(event EventParticleData
  (params (Data :type Array%20of%20Basic%20Particle%20Data%20Structures) (NiagaraSystem :type Niagara%20System%20Object%20Reference))
  (bind _spellplacementlocation (Variables|Default|GetSpellPlacementLocation))
  (bind _spellinfo (Variables|Default|GetSpellInfo))
  (bind (_damagetype _specialdamageinfo) (Utilities|Struct|BreakS_SpellInfo _spellinfo))
  ;[1 1 1] Strike Enemies A Single Time
  (Utilities|FlowControl|DoOnce false
    (:Completed
      (bind _outhits (Collision|MultiSphereTraceForObjects _spellplacementlocation _spellplacementlocation (/ (Utilities|Struct|BreakS_SpellPlacement (.SpellPlacement (Utilities|Struct|BreakS_SpellInfo (Variables|Default|GetSpellInfo)))) 2.4) (Utilities|Array|MakeArray "ObjectTypeQuery4") false (Utilities|Array|MakeArray (Variables|Default|GetCharacterActorRef)) "None"))
      (for _array_element _outhits
        (if (not (Utilities|Array|ContainsItem (Variables|Default|GetHit%20Actor) (.HitActor (Collision|BreakHitResult _array_element))))
          (Utilities|Array|Add (Variables|Default|GetHit%20Actor) (.HitActor (Collision|BreakHitResult _array_element)))
          (Utilities|IsValid (Actor|GetComponentbyClass (.HitActor (Collision|BreakHitResult _array_element)) "/Game/FlexibleCombatSystem/Blueprints/Components/TakingDamage.TakingDamage_C")
            (:Is%20Valid
              (Default|PassDamageInfo (Actor|GetComponentbyClass (.HitActor (Collision|BreakHitResult _array_element)) "/Game/FlexibleCombatSystem/Blueprints/Components/TakingDamage.TakingDamage_C") 0 "NewEnumerator18" _damagetype (Variables|Default|GetCriticalHit) _specialdamageinfo)
              (Game|Damage|ApplyPointDamage (.HitActor (Collision|BreakHitResult _array_element)) (Variables|Default|GetSpellDamage) (.ImpactPoint (Collision|BreakHitResult _array_element)) _array_element 0 (Variables|Default|GetCharacterActorRef)))))))))

(event EventSpellEffect
  ;[1 1 1] Strike Enemies A Single Time
  (bind (_spell_damage _critical_hit) (Default|CalculateMagicDamage (Variables|Default|GetMagicComponent) (Variables|Default|GetSpellInfo)))
  (Variables|Default|SetSpellDamage _spell_damage)
  (Variables|Default|SetCriticalHit _critical_hit)
  (bind _returnvalue (Niagara|SpawnSystematLocation (Utilities|Struct|BreakS_SpellPlacement (Utilities|Struct|BreakS_SpellInfo (Variables|Default|GetSpellInfo))) (Variables|Default|GetSpellPlacementLocation)))
  (Components|Activation|Activate _returnvalue false)
  (Niagara|SetNiagaraVariable(Object) _returnvalue "User.BP_Spell" self))

(fn ConstructionScript
  (|CallParentFunction))