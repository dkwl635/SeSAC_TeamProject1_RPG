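; BP_PhysicalRune is a placed spell trap that shows a Niagara effect chosen by damage type and sized to the spell radius.
; A non-owner player or enemy overlapping it, unless rolling, triggers a one-time explosion that damages pawns found by sphere trace through TakingDamage and point damage.
; Non-enemy runes register save info with the game mode and unregister on detonation; decoration runes skip saving and damage.
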(event OnComponentBeginOverlap(Sphere)
  (params (OverlappedComponent :type Primitive%20Component%20Object%20Reference) (OtherActor :type Actor%20Object%20Reference) (OtherComp :type Primitive%20Component%20Object%20Reference) (OtherBodyIndex :type Integer) (bFromSweep :type Boolean) (SweepResult :type Hit%20Result%20Structure%20%28by%20ref%29))
  (bind _returnvalue (Transformation|GetActorLocation))
  (bind _spell_info (Variables|Default|GetSpell%20Info))
  (bind (_damagetype _specialdamageinfo) (Utilities|Struct|BreakS_SpellInfo _spell_info))
  ;[1 1 1] Rune Explosion Damage
  (if (not (Variables|Default|GetDecoration))
    (if (and (Utilities|Enum|NotEqual(Enum) (Variables|Default|GetRuneOwner) (Utilities|GetObjectName OtherActor)) (or (Actor|ActorHasTag OtherActor "Player") (Actor|ActorHasTag OtherActor "EnemyAI")))
      (if (not (CallFunction|IsPlayingMontage (Variables|/Game/FlexibleCombatSystem/Blueprints/Components/MovementStatusComponent.MovementStatusComponent_C|GetMesh (Actor|GetComponentbyClass OtherActor "/Game/FlexibleCombatSystem/Blueprints/Components/MovementStatusComponent.MovementStatusComponent_C")) "/Game/FlexibleCombatSystem/Animation/Common/M_Roll.M_Roll"))
        (Utilities|FlowControl|DoOnce false
          (:Completed
            (Audio|PlaySoundatLocation (Utilities|Struct|BreakS_SpellSounds (.SpellSoundFX (Utilities|Struct|BreakS_SpellInfo (Variables|Default|GetSpell%20Info)))) (Transformation|GetActorLocation) "0, 0, 0" 1.0 1.0 0.0 0 0 0)
            (Niagara|SpawnSystematLocation (Utilities|Struct|BreakS_SpellPlacement (.SpellPlacement (Utilities|Struct|BreakS_SpellInfo (Variables|Default|GetSpell%20Info)))) (Transformation|GetActorLocation))
            (bind _outhits (Collision|MultiSphereTraceForObjects _returnvalue _returnvalue (Variables|/Script/Engine.SphereComponent|GetSphereRadius (Variables|Default|GetSphere)) (Utilities|Array|MakeArray "ObjectTypeQuery3") false 0 "None"))
            (for _array_element _outhits
              (if (not (Utilities|Array|ContainsItem (Variables|Default|GetHit%20Actor) (.HitActor (Collision|BreakHitResult _array_element))))
                (Utilities|Array|Add (Variables|Default|GetHit%20Actor) (.HitActor (Collision|BreakHitResult _array_element)))
                (Utilities|IsValid (Actor|GetComponentbyClass (.HitActor (Collision|BreakHitResult _array_element)) "/Game/FlexibleCombatSystem/Blueprints/Components/TakingDamage.TakingDamage_C")
                  (:Is%20Valid
                    (Default|PassDamageInfo (Actor|GetComponentbyClass (.HitActor (Collision|BreakHitResult _array_element)) "/Game/FlexibleCombatSystem/Blueprints/Components/TakingDamage.TakingDamage_C") 0 "NewEnumerator18" _damagetype (Variables|Default|GetCriticalHit) _specialdamageinfo)
                    (Game|Damage|ApplyPointDamage (.HitActor (Collision|BreakHitResult _array_element)) (Variables|Default|GetSpellDamage) (.ImpactPoint (Collision|BreakHitResult _array_element)) _array_element 0 (Variables|Default|GetDamage%20Causer))))))
            (Utilities|FlowControl|Delay 0.1)
            (if (Variables|Default|GetEnemyAI)
              _
              (else
                (Class|IGameMode|RunePlaced(Message) (Game|GetGameMode) false (Variables|Default|GetRuneSaveInfo))))
            (Actor|DestroyActor)))))))

(event EventBeginPlay
  ;[1 1 1] Setup Rune
  (if (Variables|Default|GetDecoration)
    _
    (else
      (CallFunction|SaveInfo)))
  (Class|NiagaraComponent|SetAsset (Variables|Default|GetNiagara) (Utilities|Select :Index (Utilities|Struct|BreakS_SpellInfo (Variables|Default|GetSpell%20Info)) :NewEnumerator0 0 :NewEnumerator1 "/Game/FlexibleCombatSystem/VFX/MagicVFX/Runes/NS_Rune_Fire.NS_Rune_Fire" :NewEnumerator2 "/Game/FlexibleCombatSystem/VFX/MagicVFX/Runes/NS_Rune_Ice.NS_Rune_Ice" :NewEnumerator8 0 :NewEnumerator3 "/Game/FlexibleCombatSystem/VFX/MagicVFX/Runes/NS_Rune_Lightning.NS_Rune_Lightning" :NewEnumerator4 "/Game/FlexibleCombatSystem/VFX/MagicVFX/Runes/NS_Rune_Poison.NS_Rune_Poison" :NewEnumerator5 "/Game/FlexibleCombatSystem/VFX/MagicVFX/Runes/NS_Rune_Madness.NS_Rune_Madness" :NewEnumerator6 0 :NewEnumerator7 0 :NewEnumerator9 0) true)
  (Niagara|SetNiagaraVariable(Float) (Variables|Default|GetNiagara) "User.Size" (Utilities|Struct|BreakS_SpellPlacement (.SpellPlacement (Utilities|Struct|BreakS_SpellInfo (Variables|Default|GetSpell%20Info))))))

(fn ConstructionScript)

(fn SaveInfo
  (if (not (Variables|Default|GetEnemyAI))
    (Variables|Default|SetRuneSaveInfo (Utilities|Struct|MakeS_RuneSaveInfo (Transformation|GetActorTransform) (Variables|Default|GetRuneOwner) (Variables|Default|GetSpellDamage) (Variables|Default|GetCriticalHit) (Variables|Default|GetSpell%20Info)))
    (Class|IGameMode|RunePlaced(Message) (Game|GetGameMode) true (Variables|Default|GetRuneSaveInfo))))