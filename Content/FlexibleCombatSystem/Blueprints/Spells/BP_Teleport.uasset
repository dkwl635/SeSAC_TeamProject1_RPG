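; Teleport spell in the Flexible Combat System that relocates its player or AI caster with Niagara effects.
; Casting takes a player's destination from the visible placement marker, while AI runs an EQS query around its target.
; Sphere traces select the first queried point with a clear hit on a Player or EnemyAI actor.
; The animation-triggered SpellEffect moves the caster if a location exists, reports noise, then destroys the spell.
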(event Custom|OnQueryFinishedEvent
  (params (QueryInstance :type Env%20Query%20Instance%20Blueprint%20Wrapper%20Object%20Reference) (QueryStatus :type EEnvQueryStatus%20Enum :default "Processing"))
  (bind _enemytarget (Variables|Default|GetEnemyTarget))
  (bind _returnvalue (Transformation|GetActorLocation _enemytarget))
  ;[1 1 1] Trigger Niagara PS Begin
  ;;[1 1 1] Out of All Possible Locations Find One Where AI Can See Enemy
  (bind _resultlocations (AI|EQS|GetQueryResultsasLocations QueryInstance))
  (bind _array_element (Utilities|Array|ForEachLoopwithBreak _resultlocations :!label _label)
    (:LoopBody
      (bind _outhit (Collision|SphereTraceByChannel (Math|Vector|MakeVector (.X (Math|Vector|BreakVector _array_element)) (.Y (Math|Vector|BreakVector _array_element)) (.Z (Math|Vector|BreakVector _returnvalue))) _returnvalue 4.0 "TraceTypeQuery3" false 0 "None"))
      (Utilities|IsValid (.HitActor (Collision|BreakHitResult _outhit))
        (:Is%20Valid
          (if (or (Actor|ActorHasTag (.HitActor (Collision|BreakHitResult _outhit)) "Player") (Actor|ActorHasTag (.HitActor (Collision|BreakHitResult _outhit)) "EnemyAI"))
            (Variables|Default|SetTeleportLocation _array_element)
            (goto _label Break)))))))

(event EventBeginPlay
  (|CallParentFunction) ; This node is disabled and will not be called.\nDrag off pins to build functionality.
)

(event Collision|EventActorBeginOverlap
  (params (OtherActor :type Actor%20Object%20Reference))
  (|CallParentFunction OtherActor) ; This node is disabled and will not be called.\nDrag off pins to build functionality.
)

(event EventSpellEffect
  ;[1 1 1] Trigger Spell Attack (Triggered From Animation)
  ;;[1 1 1] Safety Check Incase No TP Locations Exist
  (if (Math|Vector|Equal(Vector) (Variables|Default|GetTeleportLocation) "0, 0, 0" 0.0001)
    _
    (else
      (CallFunction|Teleport)))
  (Variables|/Game/FlexibleCombatSystem/Blueprints/Components/MagicComponent.MagicComponent_C|SetSpellCharged (Variables|Default|GetMagicComponent) false)
  (Actor|DestroyActor))

(event EventSendMagicSpell
  ;[1 1 1] Trigger Niagara PS Begin
  (|CallParentFunction)
  (if (Variables|Default|GetAI_Spell)
    (CallFunction|RemovePlacementMarker)
    (Niagara|SpawnSystematLocation "/Game/FlexibleCombatSystem/VFX/MagicVFX/Teleport/NS_Skill_TeleportationIn.NS_Skill_TeleportationIn" (Transformation|GetWorldLocation (Variables|/Script/Engine.Character|GetMesh (Variables|Default|GetCharacterRef))) :!label _label)
    (if (Variables|Default|GetAI_Spell)
      (CallFunction|FindTeleportLocation)
      (else
        (Variables|Default|SetTeleportLocation (Transformation|GetWorldLocation (Variables|/Game/FlexibleCombatSystem/Blueprints/Components/MagicComponent.MagicComponent_C|GetSpellPlacementPS (Variables|Default|GetMagicComponent))))
        (CallFunction|RemovePlacementMarker)))
    (elif (not (Variables|/Script/Engine.SceneComponent|GetbHiddenInGame (Variables|/Game/FlexibleCombatSystem/Blueprints/Components/MagicComponent.MagicComponent_C|GetSpellPlacementPS (Variables|Default|GetMagicComponent))))
      (goto _label))))

(fn ConstructionScript
  (|CallParentFunction))

(fn FindTeleportLocation
  (bind _returnvalue (AI|EQS|RunEQSQuery "/Game/FlexibleCombatSystem/Blueprints/AI/EQS/EQS_AroundTarget.EQS_AroundTarget" (Variables|Default|GetEnemyTarget) "AllMatching"))
  (EventDispatchers|BindEventtoOnQueryFinishedEvent _returnvalue (EventDispatchers|CreateEvent :!event Custom|OnQueryFinishedEvent)))

(fn Teleport
  (bind _teleportlocation (Variables|Default|GetTeleportLocation))
  (bind _enemytarget (Variables|Default|GetEnemyTarget))
  (bind _teleportlocation_2 (Variables|Default|GetTeleportLocation))
  ;[1 1 1] Set Location, Rotation, Spawn Niagara VFX & Sound FX
  (Transformation|SetActorLocation (Variables|Default|GetCharacterActorRef) (Math|Vector|MakeVector (.x _teleportlocation_2) (.y _teleportlocation_2) (+ (.z _teleportlocation_2) 1e+02)) false false)
  (Niagara|SpawnSystematLocation "/Game/FlexibleCombatSystem/VFX/MagicVFX/Teleport/NS_Skill_TeleportationOut.NS_Skill_TeleportationOut" _teleportlocation)
  (Class|AISenseHearing|ReportNoiseEvent _teleportlocation 1.0 (Variables|Default|GetCharacterActorRef) 5e+02 "None")
  ;;[1 1 1] Enemy AI Face Player On Teleport
  (Utilities|IsValid _enemytarget
    (:Is%20Valid
      (Transformation|SetActorRotation (Math|Rotator|FindLookatRotation (Transformation|GetActorLocation (Variables|Default|GetCharacterActorRef)) (Transformation|GetActorLocation _enemytarget))))))