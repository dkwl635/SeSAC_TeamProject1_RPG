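; BP_BuffParent is the parent spell Blueprint for buff spells in the Flexible Combat System.
; On its SpellEffect event it calls ActivateBuff on the caster's BuffComponent, passing effect, type, duration, amount, barrier reflect and damage data from SpellInfo.
; It then reduces mana through the MagicComponent, leaving the buff logic itself to the BuffComponent.
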(event EventSpellEffect
  (bind _spellinfo (Variables|Default|GetSpellInfo))
  (bind (_damagetype _specialdamageinfo _spelldurations) (Utilities|Struct|BreakS_SpellInfo _spellinfo))
  (bind (_spellps _spellduration _spellamount _spelldurationtype _barrierreflectdamage) (Utilities|Struct|BreakS_DurationSpells _spelldurations))
  ;[1 1 1] Creates Buff, See Buff Component For Details
  (Default|ActivateBuff (Actor|GetComponentbyClass (Variables|Default|GetCharacterRef) "/Game/FlexibleCombatSystem/Blueprints/Components/BuffComponent.BuffComponent_C") _spellps (Variables|Default|GetCharacterRef) _spelldurationtype _spellduration _spellamount _barrierreflectdamage _damagetype _specialdamageinfo false)
  (Default|ReduceMana (Variables|Default|GetMagicComponent)))

(fn ConstructionScript
  (|CallParentFunction))