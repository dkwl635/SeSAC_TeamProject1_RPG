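; Parent Blueprint for single heal spells in the combat system, applying a one-time health boost when its SpellEffect event fires.
; It attaches the spell's Niagara effect to the character, spends mana, then adds the spell amount to EquipmentComponent health, clamped to max.
; It dispatches the health update and shows combat text if that component exists.
; After a short delay, it removes the effect and destroys itself.
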(event EventSpellEffect
  (bind _spellinfo (Variables|Default|GetSpellInfo))
  (bind _characteractorref (Variables|Default|GetCharacterActorRef))
  (bind _characterref (Variables|Default|GetCharacterRef))
  (bind _equipmentcomponent (Variables|Default|GetEquipmentComponent))
  (bind _spelldurations (Utilities|Struct|BreakS_SpellInfo _spellinfo))
  (bind _returnvalue (Actor|GetComponentbyClass _characterref "/Game/FlexibleCombatSystem/Blueprints/Components/CombatTextComponent.CombatTextComponent_C"))
  (bind _maxhealth (Variables|/Game/FlexibleCombatSystem/Blueprints/Components/EquipmentComponent.EquipmentComponent_C|GetMaxHealth _equipmentcomponent))
  (bind _spellamount (Utilities|Struct|BreakS_DurationSpells _spelldurations))
  ;[1 1 1] Increase Health
  (bind _returnvalue_2 (Niagara|SpawnSystemAttached (Utilities|Struct|BreakS_DurationSpells (.SpellDurations (Utilities|Struct|BreakS_SpellInfo (Variables|Default|GetSpellInfo)))) (Variables|/Script/Engine.Actor|GetRootComponent _characteractorref) "None" (Transformation|GetActorLocation _characteractorref) "0, 0, 0" "KeepWorldPosition" false))
  (Variables|Default|SetNiagaraPS _returnvalue_2)
  (Default|ReduceMana (Variables|Default|GetMagicComponent))
  (bind _output_get (Variables|/Game/FlexibleCombatSystem/Blueprints/Components/EquipmentComponent.EquipmentComponent_C|SetHealth _equipmentcomponent (+ (Variables|/Game/FlexibleCombatSystem/Blueprints/Components/EquipmentComponent.EquipmentComponent_C|GetHealth (Variables|Default|GetEquipmentComponent)) _spellamount)))
  (if (> _output_get _maxhealth)
    (Variables|/Game/FlexibleCombatSystem/Blueprints/Components/EquipmentComponent.EquipmentComponent_C|SetHealth _equipmentcomponent _maxhealth))
  (Default|UpdateHealthDispatch _equipmentcomponent)
  (Utilities|IsValid _returnvalue
    (:Is%20Valid
      (Default|CombatTextPopup _returnvalue (Transformation|GetActorLocation _characterref) (Math|Float|Round _spellamount) "NewEnumerator13" false false false))
    (:Is%20Not%20Valid
      _))
  (Utilities|FlowControl|Delay 2.0)
  (Components|Activation|Deactivate (Variables|Default|GetNiagaraPS))
  (Components|DestroyComponent (Variables|Default|GetNiagaraPS))
  (Actor|DestroyActor))

(fn ConstructionScript
  (|CallParentFunction))