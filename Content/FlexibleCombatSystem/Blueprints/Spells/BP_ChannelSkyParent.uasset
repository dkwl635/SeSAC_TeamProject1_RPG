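; Parent Blueprint for channeled area spells that strike a placed ground location for as long as the channel is held.
; Charging shows a Niagara marker updated by a fast looping timer, then casting locks controls and pauses it.
; An animation-triggered event spawns the effect and loop sound, then a repeating timer sphere-traces pawns, applies damage and drains mana.
; Releasing stops the damage, restores controls, respawns the marker and plays the end montage.
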(event Custom|ActivateSpellTick
  ;[1 1 1] Trigger Spell Attack (Triggered From Animation)
  (CallFunction|SphereTraceAttack))

(event EventBeginMagicCharge
  ;[1 1 1] Start Charge
  (CallFunction|RemovePlacementMarker)
  (bind _returnvalue (Niagara|SpawnSystematLocation (Utilities|Struct|BreakS_SpellPlacement (.SpellPlacement (Utilities|Struct|BreakS_SpellInfo (Variables|Default|GetSpellInfo)))) (Variables|Default|GetSpellPlacementLocation)))
  (bind _output_get (Variables|/Game/FlexibleCombatSystem/Blueprints/Components/MagicComponent.MagicComponent_C|SetSpellPlacementPS (Variables|Default|GetMagicComponent) _returnvalue))
  (Niagara|SetNiagaraVariable(Float) _output_get "User.Size" (Utilities|Struct|BreakS_SpellPlacement (.SpellPlacement (Utilities|Struct|BreakS_SpellInfo (Variables|Default|GetSpellInfo)))))
  (CallFunction|UpdateSpellPlacement)
  (bind _returnvalue_2 (Utilities|Time|SetTimerbyFunctionName 0 "UpdateSpellPlacement" 0.01 true))
  (Variables|Default|SetSpellPlacementTimer _returnvalue_2))

(event EventStopMagicCharge
  (bind _charactermesh (Variables|Default|GetCharacterMesh))
  ;[1 1 1] Release Charge - Right Mouse Button Release
  (CallFunction|DeactivateChannel)
  (CallFunction|RemovePlacementMarker)
  (Class|ICharacter|SetDisableControls(Message) (Variables|Default|GetCharacterRef) false false)
  (Default|CallEventSpellChanneling (Variables|Default|GetMagicComponent) false)
  (if (Variables|Default|GetChanneling)
    (Default|ClearBuffer (Variables|Default|GetInputBufferComponent) false) ; Channel End Anim Clears Buffer, As we're not playing it we need to clear
    (elif (CallFunction|IsPlayingMontage _charactermesh (Variables|Default|GetSpellEnd))
      (Audio|Components|Audio|Stop _charactermesh) ; Prevents Channel End Anim Playing
    )))

(event EventSendMagicSpell
  ;[1 1 1] Send Animation Spell - Loop Through Animation Until Release
  (Class|ICharacter|SetDisableControls(Message) (Variables|Default|GetCharacterRef) true true)
  (Utilities|Time|PauseTimerbyHandle (Variables|Default|GetSpellPlacementTimer))
  (CallFunction|CalculateAnimationEnd)
  (Default|CallEventSpellChanneling (Variables|Default|GetMagicComponent) true)
  (bind _returnvalue (Audio|SpawnSoundatLocation (Utilities|Struct|BreakS_SpellSounds (.SpellSoundFX (Utilities|Struct|BreakS_SpellInfo (Variables|Default|GetSpellInfo)))) (Transformation|GetActorLocation) "0, 0, 0" 1.0 1.0 0.0 0 0))
  (Variables|Default|SetSpellAnimSound _returnvalue))

(event EventTriggerMagicSpell
  (bind _spellanimsound (Variables|Default|GetSpellAnimSound))
  ;[1 1 1] Trigger Spell Attack (Triggered From Animation)
  (Utilities|Time|ClearandInvalidateTimerbyHandle (Variables|Default|GetSpellPlacementTimer))
  (CallFunction|RemovePlacementMarker)
  (Variables|Default|SetChanneling true)
  (bind _returnvalue (Niagara|SpawnSystematLocation (Utilities|Struct|BreakS_SpellPlacement (.SpellPlacement (Utilities|Struct|BreakS_SpellInfo (Variables|Default|GetSpellInfo)))) (Variables|Default|GetSpellPlacementLocation)))
  (Variables|Default|SetSpellPS _returnvalue)
  (Utilities|IsValid _spellanimsound
    (:Is%20Valid
      (Audio|Components|Audio|FadeOut _spellanimsound 1.0 0.0 "Linear" :!class /Script/Engine.AudioComponent))
    (:Is%20Not%20Valid
      _))
  (bind _returnvalue_2 (Audio|SpawnSoundatLocation (Utilities|Struct|BreakS_SpellSounds (.SpellSoundFX (Utilities|Struct|BreakS_SpellInfo (Variables|Default|GetSpellInfo)))) (Transformation|GetActorLocation) "0, 0, 0" 1.0 1.0 0.0 0 0))
  (Variables|Default|SetSpellChannelSound _returnvalue_2)
  (bind _returnvalue_3 (Utilities|Time|SetTimerbyEvent (delegate Custom|ActivateSpellTick) (.TickFrequency (Utilities|Struct|BreakS_SpellPlacement (.SpellPlacement (Utilities|Struct|BreakS_SpellInfo (Variables|Default|GetSpellInfo))))) true))
  (Variables|Default|SetDamageChannel _returnvalue_3))

(event EventReleaseSpellChannel
  (bind _spellchannelsound (Variables|Default|GetSpellChannelSound))
  ;[1 1 1] Release Spell Channel - Left Mouse Button Release
  (Variables|Default|SetChanneling false)
  (CallFunction|DeactivateChannel)
  (Utilities|IsValid _spellchannelsound
    (:Is%20Valid
      (Audio|Components|Audio|FadeOut _spellchannelsound 1.0 0.0 "Linear" :!class /Script/Engine.AudioComponent))
    (:Is%20Not%20Valid
      _))
  (CallFunction|SetupMarker)
  (Class|ICharacter|SetDisableControls(Message) (Variables|Default|GetCharacterRef) false false)
  ;;[1 1 1] Channel End Montage - Clears Buffer
  (Animation|Montage|PlayMontage (Variables|Default|GetCharacterMesh) (Variables|Default|GetSpellEnd)
    (:OnBlendOut
      _)
    (:OnInterrupted
      _))
  (Default|CallEventSpellChanneling (Variables|Default|GetMagicComponent) false)
  (CallFunction|Spell-Interupted))

(fn ConstructionScript
  (|CallParentFunction))

(fn SetupAnimationMontages
  (if (== (.Animation (Utilities|Struct|BreakS_SpellInfo (Variables|Default|GetSpellInfo))) "/Game/FlexibleCombatSystem/Animation/Magic/Channel/SpellChannel_2/M_SpellChannel2.M_SpellChannel2")
    (Variables|Default|SetSpellStart "/Game/FlexibleCombatSystem/Animation/Magic/Channel/SpellChannel_2/M_SpellChannel2Start.M_SpellChannel2Start")
    (Variables|Default|SetSpellLoop "/Game/FlexibleCombatSystem/Animation/Magic/Channel/SpellChannel_2/M_SpellChannel2Mid.M_SpellChannel2Mid")
    (Variables|Default|SetSpellEnd "/Game/FlexibleCombatSystem/Animation/Magic/Channel/SpellChannel_2/M_SpellChannel2End.M_SpellChannel2End")))

(fn SphereTraceAttack
  (bind _spellinfo (Variables|Default|GetSpellInfo))
  (bind _spellplacementlocation (Variables|Default|GetSpellPlacementLocation))
  (bind (_damagetype _specialdamageinfo) (Utilities|Struct|BreakS_SpellInfo _spellinfo))
  ;[1 1 1] Deal Damage To All in Area
  (bind (_spell_damage _critical_hit) (Default|CalculateMagicDamage (Variables|Default|GetMagicComponent) (Variables|Default|GetSpellInfo)))
  (LocalVariables|SetSpellDamage _spell_damage)
  (LocalVariables|SetCriticalHit _critical_hit)
  (bind _outhits (Collision|MultiSphereTraceForObjects _spellplacementlocation _spellplacementlocation (/ (Utilities|Struct|BreakS_SpellPlacement (.SpellPlacement (Utilities|Struct|BreakS_SpellInfo (Variables|Default|GetSpellInfo)))) 2.4) (Utilities|Array|MakeArray "ObjectTypeQuery3") false (Utilities|Array|MakeArray (Variables|Default|GetCharacterActorRef)) "None"))
  (for _array_element _outhits
    (Utilities|IsValid (Actor|GetComponentbyClass (.HitActor (Collision|BreakHitResult _array_element)) "/Game/FlexibleCombatSystem/Blueprints/Components/TakingDamage.TakingDamage_C")
      (:Is%20Valid
        (Default|PassDamageInfo (Actor|GetComponentbyClass (.HitActor (Collision|BreakHitResult _array_element)) "/Game/FlexibleCombatSystem/Blueprints/Components/TakingDamage.TakingDamage_C") 0 "NewEnumerator18" _damagetype (LocalVariables|GetCriticalHit) _specialdamageinfo)
        (Game|Damage|ApplyPointDamage (.HitActor (Collision|BreakHitResult _array_element)) (LocalVariables|GetSpellDamage) (.ImpactPoint (Collision|BreakHitResult _array_element)) _array_element 0 (Variables|Default|GetCharacterActorRef)))))
  (Default|ReduceMana (Variables|Default|GetMagicComponent)))

(fn CalculateAnimationEnd
  (if (== (.Animation (Utilities|Struct|BreakS_SpellInfo (Variables|Default|GetSpellInfo))) "/Game/FlexibleCombatSystem/Animation/Magic/Channel/SpellChannel_1/M_SpellChannel1.M_SpellChannel1")
    (Variables|Default|SetSpellEnd "/Game/FlexibleCombatSystem/Animation/Magic/Channel/SpellChannel_1/M_SpellChannel1_End.M_SpellChannel1_End")
    (Default|CallEventSpellChannelNumber (Variables|Default|GetMagicComponent))
    (elif (== (.Animation (Utilities|Struct|BreakS_SpellInfo (Variables|Default|GetSpellInfo))) "/Game/FlexibleCombatSystem/Animation/Magic/Channel/SpellChannel_2/M_SpellChannel2.M_SpellChannel2")
      (Variables|Default|SetSpellEnd "/Game/FlexibleCombatSystem/Animation/Magic/Channel/SpellChannel_2/M_SpellChannel2End.M_SpellChannel2End")
      (Default|CallEventSpellChannelNumber (Variables|Default|GetMagicComponent) 1))))

(fn DeactivateChannel
  (bind _spellps (Variables|Default|GetSpellPS))
  (Utilities|Time|ClearandInvalidateTimerbyHandle (Variables|Default|GetDamageChannel))
  (Utilities|IsValid _spellps
    (:Is%20Valid
      (Components|Activation|Deactivate _spellps))))

(fn SetupMarker
  ;[1 1 1] Respawn Marker OR Activate
  (Utilities|IsValid (Variables|/Game/FlexibleCombatSystem/Blueprints/Components/MagicComponent.MagicComponent_C|GetSpellPlacementPS (Variables|Default|GetMagicComponent))
    (:Is%20Valid
      (Components|Activation|Activate (Variables|/Game/FlexibleCombatSystem/Blueprints/Components/MagicComponent.MagicComponent_C|GetSpellPlacementPS (Variables|Default|GetMagicComponent)) false))
    (:Is%20Not%20Valid
      (bind _returnvalue (Niagara|SpawnSystematLocation (Utilities|Struct|BreakS_SpellPlacement (.SpellPlacement (Utilities|Struct|BreakS_SpellInfo (Variables|Default|GetSpellInfo)))) (Variables|Default|GetSpellPlacementLocation)))
      (bind _output_get (Variables|/Game/FlexibleCombatSystem/Blueprints/Components/MagicComponent.MagicComponent_C|SetSpellPlacementPS (Variables|Default|GetMagicComponent) _returnvalue))
      (Niagara|SetNiagaraVariable(Float) _output_get "User.Size" (Utilities|Struct|BreakS_SpellPlacement (.SpellPlacement (Utilities|Struct|BreakS_SpellInfo (Variables|Default|GetSpellInfo)))))))
  (bind _returnvalue_2 (Utilities|Time|SetTimerbyFunctionName 0 "UpdateSpellPlacement" 0.01 true))
  (Variables|Default|SetSpellPlacementTimer _returnvalue_2))