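; Parent Blueprint for channeled moving spells in the combat system, handling charge, trigger, channel and release.
; Charging spawns a Niagara placement marker refreshed by a looping timer calling UpdateSpellPlacement.
; An animation-driven trigger spawns BP_MovingDamagingSpell at that location with an attached loop sound.
; Releasing or stopping deactivates it, while montage handling, MagicComponent channeling events and input-buffer clearing coordinate the animation state.
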(event EventBeginMagicCharge
  ;[1 1 1] Start Charge
  (CallFunction|RemovePlacementMarker)
  (bind _returnvalue (Niagara|SpawnSystematLocation (Utilities|Struct|BreakS_SpellPlacement (.SpellPlacement (Utilities|Struct|BreakS_SpellInfo (Variables|Default|GetSpellInfo)))) (Variables|Default|GetSpellPlacementLocation)))
  (bind _output_get (Variables|/Game/FlexibleCombatSystem/Blueprints/Components/MagicComponent.MagicComponent_C|SetSpellPlacementPS (Variables|Default|GetMagicComponent) _returnvalue))
  (Niagara|SetNiagaraVariable(Float) _output_get "User.Size" (Utilities|Struct|BreakS_SpellPlacement (.SpellPlacement (Utilities|Struct|BreakS_SpellInfo (Variables|Default|GetSpellInfo)))))
  (bind _returnvalue_2 (Utilities|Time|SetTimerbyFunctionName 0 "UpdateSpellPlacement" 0.01 true))
  (Variables|Default|SetSpellPlacementTimer _returnvalue_2))

(event EventStopMagicCharge
  (bind _charactermesh (Variables|Default|GetCharacterMesh))
  ;[1 1 1] Release Charge - Right Mouse Button Release
  (CallFunction|DeactivateSpell)
  (CallFunction|RemovePlacementMarker)
  (Default|CallEventSpellChanneling (Variables|Default|GetMagicComponent) false)
  (if (Variables|Default|GetChanneling)
    (Default|ClearBuffer (Variables|Default|GetInputBufferComponent) false) ; Channel End Anim Clears Buffer, As we're not playing it we need to clear
    (elif (CallFunction|IsPlayingMontage _charactermesh (Variables|Default|GetSpellEnd))
      (Audio|Components|Audio|Stop _charactermesh) ; Prevents Channel End Anim Playing
    )))

(event EventSendMagicSpell
  ;[1 1 1] Send Animation Spell - Loop Through Animation Until Release
  (CallFunction|CalculateAnimationEnd)
  (Default|CallEventSpellChanneling (Variables|Default|GetMagicComponent) true)
  (bind _returnvalue (Audio|SpawnSoundatLocation (Utilities|Struct|BreakS_SpellSounds (.SpellSoundFX (Utilities|Struct|BreakS_SpellInfo (Variables|Default|GetSpellInfo)))) (Transformation|GetActorLocation) "0, 0, 0" 1.0 1.0 0.0 0 0))
  (Variables|Default|SetSpellAnimSound _returnvalue))

(event EventTriggerMagicSpell
  ;[1 1 1] Trigger Spell Attack (Triggered From Animation)
  (|CallParentFunction)
  (Audio|Components|Audio|FadeOut (Variables|Default|GetSpellAnimSound) 1.0 0.0 "Linear" :!class /Script/Engine.AudioComponent)
  (Variables|Default|SetChanneling true)
  (bind _returnvalue (Game|SpawnActorfromClass "/Game/FlexibleCombatSystem/Blueprints/Spells/BP_MovingDamagingSpell.BP_MovingDamagingSpell_C" (Math|Transform|MakeTransform (Variables|Default|GetSpellPlacementLocation) "0, 0, 0" "1,1,1") "Undefined" 0 (.SpellPS (Utilities|Struct|BreakS_SpellPlacement (.SpellPlacement (Utilities|Struct|BreakS_SpellInfo (Variables|Default|GetSpellInfo))))) self 1.5 (Variables|Default|GetMagicComponent) (Variables|Default|GetCharacterActorRef) 0))
  (Variables|Default|SetDamagingSpell _returnvalue)
  (Variables|/Game/FlexibleCombatSystem/Blueprints/Spells/BP_MovingDamagingSpell.BP_MovingDamagingSpell_C|SetSpellInfo _returnvalue (Variables|Default|GetSpellInfo))
  (bind _returnvalue_2 (Audio|SpawnSoundAttached (Utilities|Struct|BreakS_SpellSounds (Utilities|Struct|BreakS_SpellInfo (Variables|Default|GetSpellInfo))) (Variables|/Script/Engine.Actor|GetRootComponent _returnvalue) "None" "0, 0, 0" "0, 0, 0" "KeepRelativeOffset" false 1.0 1.0 0.0 0 0))
  (bind _output_get (Variables|Default|SetLoopSound _returnvalue_2))
  (Variables|/Script/Engine.AudioComponent|SetAttenuationSettings _output_get "/Game/FlexibleCombatSystem/SoundFX/SA_AttenuationMidFade.SA_AttenuationMidFade"))

(event EventReleaseSpellChannel
  ;[1 1 1] Release Spell Channel - Left Mouse Button Release
  (Variables|Default|SetChanneling false)
  (CallFunction|DeactivateSpell)
  (Audio|Components|Audio|FadeOut (Variables|Default|GetLoopSound) 1.0 0.0 "Linear" :!class /Script/Engine.AudioComponent)
  ;;[1 1 1] Channel End Montage - Clears Buffer
  (Animation|Montage|PlayMontage (Variables|Default|GetCharacterMesh) (Variables|Default|GetSpellEnd)
    (:OnBlendOut
      _)
    (:OnInterrupted
      _))
  (Default|CallEventSpellChanneling (Variables|Default|GetMagicComponent) false)
  (CallFunction|Spell-Interupted))

(fn ConstructionScript
  (|CallParentFunction))

(fn SetupAnimationMontages
  (if (== (.Animation (Utilities|Struct|BreakS_SpellInfo (Variables|Default|GetSpellInfo))) "/Game/FlexibleCombatSystem/Animation/Magic/Channel/SpellChannel_1/M_SpellChannel1.M_SpellChannel1")
    (Variables|Default|SetSpellStart "/Game/FlexibleCombatSystem/Animation/Magic/Channel/SpellChannel_1/M_SpellChannel1_Start.M_SpellChannel1_Start")
    (Variables|Default|SetSpellLoop "/Game/FlexibleCombatSystem/Animation/Magic/Channel/SpellChannel_1/M_SpellChannel1_Mid.M_SpellChannel1_Mid")
    (Variables|Default|SetSpellEnd "/Game/FlexibleCombatSystem/Animation/Magic/Channel/SpellChannel_1/M_SpellChannel1_End.M_SpellChannel1_End")))

(fn CalculateAnimationEnd
  ;[1 1 1] Set the End Animation Based Upon Animation Set
  (if (== (.Animation (Utilities|Struct|BreakS_SpellInfo (Variables|Default|GetSpellInfo))) "/Game/FlexibleCombatSystem/Animation/Magic/Channel/SpellChannel_1/M_SpellChannel1.M_SpellChannel1")
    (Variables|Default|SetSpellEnd "/Game/FlexibleCombatSystem/Animation/Magic/Channel/SpellChannel_1/M_SpellChannel1_End.M_SpellChannel1_End")
    (Default|CallEventSpellChannelNumber (Variables|Default|GetMagicComponent))
    (elif (== (.Animation (Utilities|Struct|BreakS_SpellInfo (Variables|Default|GetSpellInfo))) "/Game/FlexibleCombatSystem/Animation/Magic/Channel/SpellChannel_2/M_SpellChannel2.M_SpellChannel2")
      (Variables|Default|SetSpellEnd "/Game/FlexibleCombatSystem/Animation/Magic/Channel/SpellChannel_2/M_SpellChannel2End.M_SpellChannel2End")
      (Default|CallEventSpellChannelNumber (Variables|Default|GetMagicComponent) 1))))

(fn DeactivateSpell
  (bind _damagingspell (Variables|Default|GetDamagingSpell))
  (Utilities|IsValid _damagingspell
    (:Is%20Valid
      (Default|Deactivate _damagingspell))))