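; Base spell Blueprint for spells aimed with a ground placement marker, leaving SpellEffect empty for children to fill.
; Charging spawns a radius-sized particle marker on the magic component and runs a fast looping timer to update placement.
; Sending clears the input buffer if the marker is hidden, otherwise pauses updates and plays the cast montage.
; The animation-driven trigger removes the marker, runs the effect, plays fire sound and reports AI noise.
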(event Custom|SpellEffect
  ;[1 1 1] Trigger Spell Attack (Triggered From Animation)
)

(event EventBeginPlay
  (|CallParentFunction) ; This node is disabled and will not be called.\nDrag off pins to build functionality.
)

(event Collision|EventActorBeginOverlap
  (params (OtherActor :type Actor%20Object%20Reference))
  (|CallParentFunction OtherActor) ; This node is disabled and will not be called.\nDrag off pins to build functionality.
)

(event EventTick
  (params (DeltaSeconds :type Float%20%28single-precision%29))
  (|CallParentFunction DeltaSeconds) ; This node is disabled and will not be called.\nDrag off pins to build functionality.
)

(event EventBeginMagicCharge
  ;[1 1 1] Start Charge
  (CallFunction|RemovePlacementMarker)
  (bind _returnvalue (Niagara|SpawnSystematLocation (Utilities|Struct|BreakS_SpellPlacement (.SpellPlacement (Utilities|Struct|BreakS_SpellInfo (Variables|Default|GetSpellInfo)))) (Variables|Default|GetSpellPlacementLocation)))
  (bind _output_get (Variables|/Game/FlexibleCombatSystem/Blueprints/Components/MagicComponent.MagicComponent_C|SetSpellPlacementPS (Variables|Default|GetMagicComponent) _returnvalue))
  (Niagara|SetNiagaraVariable(Float) _output_get "User.Size" (Utilities|Struct|BreakS_SpellPlacement (.SpellPlacement (Utilities|Struct|BreakS_SpellInfo (Variables|Default|GetSpellInfo)))))
  (bind _returnvalue_2 (Utilities|Time|SetTimerbyFunctionName 0 "UpdateSpellPlacement" 0.01 true))
  (Variables|Default|SetSpellPlacementTimer _returnvalue_2))

(event EventStopMagicCharge
  ;[1 1 1] Release Charge
  (CallFunction|RemovePlacementMarker)
  (Utilities|Time|ClearandInvalidateTimerbyHandle (Variables|Default|GetSpellPlacementTimer)))

(event EventSendMagicSpell
  ;[1 1 1] Send Animation Spell
  (Utilities|IsValid (Variables|/Game/FlexibleCombatSystem/Blueprints/Components/MagicComponent.MagicComponent_C|GetSpellPlacementPS (Variables|Default|GetMagicComponent))
    (:Is%20Valid
      ;;[1 1 1] Reset Input Buffer IF Spell Fail
      (if (Variables|/Script/Engine.SceneComponent|GetbHiddenInGame (Variables|/Game/FlexibleCombatSystem/Blueprints/Components/MagicComponent.MagicComponent_C|GetSpellPlacementPS (Variables|Default|GetMagicComponent)))
        (Default|ClearBuffer (Variables|Default|GetInputBufferComponent) false)
        (else
          (Utilities|Time|PauseTimerbyHandle (Variables|Default|GetSpellPlacementTimer))
          (bind _returnvalue (Audio|SpawnSoundatLocation (Utilities|Struct|BreakS_SpellSounds (.SpellSoundFX (Utilities|Struct|BreakS_SpellInfo (Variables|Default|GetSpellInfo)))) (Transformation|GetActorLocation) "0, 0, 0" 1.0 1.0 0.0 0 0))
          (Variables|Default|SetAnimationSound _returnvalue)
          (Animation|Montage|PlayMontage (Variables|Default|GetCharacterMesh) (Utilities|Struct|BreakS_SpellInfo (Variables|Default|GetSpellInfo))
            (:OnInterrupted
              ;;[1 1 1] Load Next Spell & Unpause Timer For Placement Marker
              (CallFunction|Spell-Interupted)
              (if (not (Utilities|Enum|Equal(Enum) (Utilities|Struct|BreakS_SpellInfo (Variables|Default|GetSpellInfo)) "NewEnumerator6"))
                (Utilities|Time|UnpauseTimerbyHandle (Variables|Default|GetSpellPlacementTimer))))))))))

(event EventTriggerMagicSpell
  (bind _animationsound (Variables|Default|GetAnimationSound))
  ;[1 1 1] Trigger Spell Attack (Triggered From Animation)
  (|CallParentFunction)
  (Utilities|FlowControl|DoOnce false
    (:Completed
      (Utilities|Time|ClearandInvalidateTimerbyHandle (Variables|Default|GetSpellPlacementTimer))
      (CallFunction|RemovePlacementMarker)
      (CallFunction|SpellEffect)
      (Utilities|IsValid _animationsound
        (:Is%20Valid
          (Audio|Components|Audio|FadeOut _animationsound 1.0 0.0 "Linear" :!class /Script/Engine.AudioComponent))
        (:Is%20Not%20Valid
          _))
      (Audio|SpawnSoundatLocation (Utilities|Struct|BreakS_SpellSounds (.SpellSoundFX (Utilities|Struct|BreakS_SpellInfo (Variables|Default|GetSpellInfo)))) (Variables|Default|GetSpellPlacementLocation) "0, 0, 0" 1.0 1.0 0.0 0 0)
      (Class|AISenseHearing|ReportNoiseEvent (Variables|Default|GetSpellPlacementLocation) 1.0 (Variables|Default|GetCharacterActorRef) 5e+02 "None"))))

(fn ConstructionScript
  (|CallParentFunction))