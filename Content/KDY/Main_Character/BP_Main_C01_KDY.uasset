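; Main player character for a dungeon game: a modular-mesh hero that turns toward the cursor, moves by input, and fights with a combo attack and three skills.
; A timed Tick handles cursor facing and the Skill02 flicker, which teleports between nearby living Enemy or Boss pawns, spawning short-lived damage actors.
; Montages drive the seven-step combo and other skills.
; StatsActor holds HP, feeds the inventory, and triggers death and GameOver.
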(event Custom|Btn_Click
  (bind _returnvalue (Transformation|GetActorLocation))
  (bind _mesh (Variables|Character|GetMesh))
  (if (Variables|Default|GetBtn%20Attack)
    (Variables|Default|SetBtn%20Attack false)
    (switch int (Variables|Default|GetCombo)
      (:0
        (Animation|Montage|PlayMontage _mesh "/Game/KDY/Main_Character/Animation/Attack/Main_Attack.Main_Attack" 1.0 0.0 "Main_Attack0"
          (:then
            (Effects|SpawnEmitteratLocation "/Game/FXVarietyPack/Particles/P_ky_waterBallHit.P_ky_waterBallHit" _returnvalue)
            (Audio|PlaySound2D "/Game/FlexibleCombatSystem/SoundFX/Spells/SW_FireballHit.SW_FireballHit" 1.0 1.0 0.0 0 0)
            (Variables|Default|SetCombo 1))))
      (:1
        (Animation|Montage|PlayMontage _mesh "/Game/KDY/Main_Character/Animation/Attack/Main_Attack.Main_Attack" 1.0 0.0 "Main_Attack1"
          (:then
            (Effects|SpawnEmitteratLocation "/Game/FXVarietyPack/Particles/P_ky_ThunderBallHit.P_ky_ThunderBallHit" _returnvalue)
            (Audio|PlaySound2D "/Game/FlexibleCombatSystem/SoundFX/Spells/SW_FireballHit.SW_FireballHit" 1.0 1.0 0.0 0 0)
            (Variables|Default|SetCombo 2))))
      (:2
        (Animation|Montage|PlayMontage _mesh "/Game/KDY/Main_Character/Animation/Attack/Main_Attack.Main_Attack" 1.0 0.0 "Main_Attack2"
          (:then
            (Effects|SpawnEmitteratLocation "/Game/FXVarietyPack/Particles/P_ky_hit2.P_ky_hit2" _returnvalue)
            (Audio|PlaySound2D "/Game/FlexibleCombatSystem/SoundFX/Spells/SW_FireballHit.SW_FireballHit" 1.0 1.0 0.0 0 0)
            (Variables|Default|SetCombo 3))))
      (:3
        (Animation|Montage|PlayMontage _mesh "/Game/KDY/Main_Character/Animation/Attack/Main_Attack.Main_Attack" 1.0 0.0 "Main_Attack3"
          (:then
            (Effects|SpawnEmitteratLocation "/Game/FXVarietyPack/Particles/P_ky_hit1.P_ky_hit1" _returnvalue)
            (Audio|PlaySound2D "/Game/FlexibleCombatSystem/SoundFX/Spells/SW_FireballHit.SW_FireballHit" 1.0 1.0 0.0 0 0)
            (Variables|Default|SetCombo 4))))
      (:4
        (Animation|Montage|PlayMontage _mesh "/Game/KDY/Main_Character/Animation/Attack/Main_Attack.Main_Attack" 1.0 0.0 "Main_Attack4"
          (:then
            (Effects|SpawnEmitteratLocation "/Game/FXVarietyPack/Particles/P_ky_waterBallHit.P_ky_waterBallHit" _returnvalue)
            (Audio|PlaySound2D "/Game/FlexibleCombatSystem/SoundFX/Spells/SW_FireballHit.SW_FireballHit" 1.0 1.0 0.0 0 0)
            (Variables|Default|SetCombo 5))))
      (:5
        (Animation|Montage|PlayMontage _mesh "/Game/KDY/Main_Character/Animation/Attack/Main_Attack.Main_Attack" 1.0 0.0 "Main_Attack5"
          (:then
            (Effects|SpawnEmitteratLocation "/Game/FXVarietyPack/Particles/P_ky_ThunderBallHit.P_ky_ThunderBallHit" _returnvalue)
            (Audio|PlaySound2D "/Game/FlexibleCombatSystem/SoundFX/Spells/SW_FireballHit.SW_FireballHit" 1.0 1.0 0.0 0 0)
            (Variables|Default|SetCombo 6))))
      (:6
        (Animation|Montage|PlayMontage _mesh "/Game/KDY/Main_Character/Animation/Attack/Main_Attack.Main_Attack" 1.0 0.0 "Main_Attack6"
          (:then
            (Effects|SpawnEmitteratLocation "/Game/FXVarietyPack/Particles/P_ky_hit2.P_ky_hit2" _returnvalue)
            (Audio|PlaySound2D "/Game/FlexibleCombatSystem/SoundFX/Spells/SW_FireballHit.SW_FireballHit" 1.0 1.0 0.0 0 0)
            (Variables|Default|SetCombo 0)))))))

(event Custom|ResetCombo
  (Variables|Default|SetIs%20Attacking false)
  (Variables|Default|SetBtn%20Attack false)
  (Variables|Default|SetCombo 0))

(event Custom|Dead
  (if (not (Variables|Default|GetIs%20Die))
    (Variables|Default|SetIs%20Die true)
    (Animation|PlayAnimMontage "/Game/KDY/Main_Character/Animation/Dead/Main_Die_Mot_02.Main_Die_Mot_02" 1.0 "None")
    (Utilities|FlowControl|Delay 2.5)
    (Development|PrintString "Dead!!")
    (Actor|DestroyActor)
    ;[0.15 0.15 0.15 0.5] 게임 상태 변화 시키기
    (bind _asbp_dungeon_game_state (Utilities|Casting|CastToBP_DungeonGameState (Game|GetGameState)))
    (Class|DungeonGameStateBase|ChangeGameState _asbp_dungeon_game_state "GameOver")))

(event Input|EnhancedActionEvents|EnhancedInputActionIA_Main_Move
  (params (ActionValue :type Vector%202D%20Structure) (ElapsedSeconds :type Float%20%28double-precision%29) (TriggeredSeconds :type Float%20%28double-precision%29) (InputAction :type Input%20Action%20Object%20Reference :default "/Game/KDY/Main_Character/InPut/IA_Main_Move.IA_Main_Move"))
  (bind _returnvalue (Pawn|GetControlRotation :!class /Script/Engine.Pawn))
  ;[0.15 0.15 0.15 0.5] WASD 로 걸어다니기
  (if (> (Class|StatsActorComponent|GetHp (Variables|Default|GetStatsActor)) 1.0)
    (Pawn|Input|AddMovementInput (Math|Vector|Normalize (Math|Vector|GetRightVector (Math|Rotator|MakeRotator (.roll _returnvalue) 0.0 (.yaw _returnvalue)))) (.x ActionValue) false)
    (Pawn|Input|AddMovementInput (Math|Vector|Normalize (Math|Vector|GetForwardVector (Math|Rotator|MakeRotator 0.0 0.0 (.yaw (Pawn|GetControlRotation :!class /Script/Engine.Pawn))))) (.y ActionValue) false)
    (else
      (Pawn|Components|CharacterMovement|DisableMovement (Variables|Character|GetCharacterMovement)))))

(event Input|EnhancedActionEvents|EnhancedInputActionIA_Main_Attack
  (params (ActionValue :type Boolean) (ElapsedSeconds :type Float%20%28double-precision%29) (TriggeredSeconds :type Float%20%28double-precision%29) (InputAction :type Input%20Action%20Object%20Reference :default "/Game/KDY/Main_Character/InPut/IA_Main_Attack.IA_Main_Attack"))
  (bind _returnvalue (Transformation|GetActorLocation))
  (bind _mesh (Variables|Character|GetMesh))
  (:Started
    (Development|PrintString (Utilities|String|ToString(Integer) (Variables|Default|GetCombo)))
    (if (Variables|Default|GetIs%20Attacking)
      (Variables|Default|SetBtn%20Attack true)
      (Variables|Default|SetIs%20Attacking false)
      (else
        (Variables|Default|SetIs%20Attacking true)
        (switch int (Variables|Default|GetCombo)
          (:0
            (Animation|Montage|PlayMontage _mesh "/Game/KDY/Main_Character/Animation/Attack/Main_Attack.Main_Attack" 1.0 0.0 "Main_Attack0"
              (:then
                (Effects|SpawnEmitteratLocation "/Game/FXVarietyPack/Particles/P_ky_waterBallHit.P_ky_waterBallHit" _returnvalue)
                (Audio|PlaySound2D "/Game/FlexibleCombatSystem/SoundFX/Spells/SW_FireballHit.SW_FireballHit" 1.0 1.0 0.0 0 0)
                (Variables|Default|SetCombo 1))))
          (:1
            (Animation|Montage|PlayMontage _mesh "/Game/KDY/Main_Character/Animation/Attack/Main_Attack.Main_Attack" 1.0 0.0 "Main_Attack1"
              (:then
                (Effects|SpawnEmitteratLocation "/Game/FXVarietyPack/Particles/P_ky_ThunderBallHit.P_ky_ThunderBallHit" _returnvalue)
                (Audio|PlaySound2D "/Game/FlexibleCombatSystem/SoundFX/Spells/SW_FireballHit.SW_FireballHit" 1.0 1.0 0.0 0 0)
                (Variables|Default|SetCombo 2))))
          (:2
            (Animation|Montage|PlayMontage _mesh "/Game/KDY/Main_Character/Animation/Attack/Main_Attack.Main_Attack" 1.0 0.0 "Main_Attack2"
              (:then
                (Effects|SpawnEmitteratLocation "/Game/FXVarietyPack/Particles/P_ky_hit2.P_ky_hit2" _returnvalue)
                (Audio|PlaySound2D "/Game/FlexibleCombatSystem/SoundFX/Spells/SW_FireballHit.SW_FireballHit" 1.0 1.0 0.0 0 0)
                (Variables|Default|SetCombo 3))))
          (:3
            (Animation|Montage|PlayMontage _mesh "/Game/KDY/Main_Character/Animation/Attack/Main_Attack.Main_Attack" 1.0 0.0 "Main_Attack3"
              (:then
                (Effects|SpawnEmitteratLocation "/Game/FXVarietyPack/Particles/P_ky_hit1.P_ky_hit1" _returnvalue)
                (Audio|PlaySound2D "/Game/FlexibleCombatSystem/SoundFX/Spells/SW_FireballHit.SW_FireballHit" 1.0 1.0 0.0 0 0)
                (Variables|Default|SetCombo 4))))
          (:4
            (Animation|Montage|PlayMontage _mesh "/Game/KDY/Main_Character/Animation/Attack/Main_Attack.Main_Attack" 1.0 0.0 "Main_Attack4"
              (:then
                (Effects|SpawnEmitteratLocation "/Game/FXVarietyPack/Particles/P_ky_waterBallHit.P_ky_waterBallHit" _returnvalue)
                (Audio|PlaySound2D "/Game/FlexibleCombatSystem/SoundFX/Spells/SW_FireballHit.SW_FireballHit" 1.0 1.0 0.0 0 0)
                (Variables|Default|SetCombo 5))))
          (:5
            (Animation|Montage|PlayMontage _mesh "/Game/KDY/Main_Character/Animation/Attack/Main_Attack.Main_Attack" 1.0 0.0 "Main_Attack5"
              (:then
                (Effects|SpawnEmitteratLocation "/Game/FXVarietyPack/Particles/P_ky_ThunderBallHit.P_ky_ThunderBallHit" _returnvalue)
                (Audio|PlaySound2D "/Game/FlexibleCombatSystem/SoundFX/Spells/SW_FireballHit.SW_FireballHit" 1.0 1.0 0.0 0 0)
                (Variables|Default|SetCombo 6))))
          (:6
            (Animation|Montage|PlayMontage _mesh "/Game/KDY/Main_Character/Animation/Attack/Main_Attack.Main_Attack" 1.0 0.0 "Main_Attack6"
              (:then
                (Effects|SpawnEmitteratLocation "/Game/FXVarietyPack/Particles/P_ky_hit2.P_ky_hit2" _returnvalue)
                (Audio|PlaySound2D "/Game/FlexibleCombatSystem/SoundFX/Spells/SW_FireballHit.SW_FireballHit" 1.0 1.0 0.0 0 0)
                (Variables|Default|SetCombo 0)))))))))

(event Input|EnhancedActionEvents|EnhancedInputActionIA_Main_Skill01
  (params (ActionValue :type Boolean) (ElapsedSeconds :type Float%20%28double-precision%29) (TriggeredSeconds :type Float%20%28double-precision%29) (InputAction :type Input%20Action%20Object%20Reference :default "/Game/KDY/Main_Character/InPut/IA_Main_Skill01.IA_Main_Skill01"))
  (:Started
    (if (> (Class|StatsActorComponent|GetHp (Variables|Default|GetStatsActor)) 1.0)
      (Animation|PlayAnimMontage "/Game/KDY/Main_Character/Animation/BP_Main_Skill01.BP_Main_Skill01" 1.0 "None")
      (Utilities|FlowControl|Delay 1.0)
      (bind _returnvalue (Game|SpawnActorfromClass "/Game/KDY/Main_Character/Skill01_Damage.Skill01_Damage_C" (Math|Conversions|ToTransform(Vector) (Transformation|GetActorLocation)) "Undefined" "MultiplyWithRoot" 0 0))
      (AddComponent|AddNiagaraComponent false)
      (Audio|PlaySound2D "/Game/FlexibleCombatSystem/SoundFX/Spells/SW_FireballHit.SW_FireballHit" 1.0 1.0 0.0 0 0)
      (Utilities|FlowControl|Delay 0.2)
      (Actor|DestroyActor _returnvalue)
      (else
        (Pawn|Components|CharacterMovement|DisableMovement (Variables|Character|GetCharacterMovement))))))

(event Input|EnhancedActionEvents|EnhancedInputActionIA_Main_Skill02
  (params (ActionValue :type Boolean) (ElapsedSeconds :type Float%20%28double-precision%29) (TriggeredSeconds :type Float%20%28double-precision%29) (InputAction :type Input%20Action%20Object%20Reference :default "/Game/KDY/Main_Character/InPut/IA_Main_Skill02.IA_Main_Skill02"))
  (:Started
    (bind _outactors (Collision|SphereOverlapActors (Transformation|GetActorLocation) 5e+03 (Utilities|Array|MakeArray "ObjectTypeQuery3") 0))
    (Variables|Default|SetFlicker%20Target%20Array _outactors)))

(event Input|EnhancedActionEvents|EnhancedInputActionIA_Main_Skill03
  (params (ActionValue :type Boolean) (ElapsedSeconds :type Float%20%28double-precision%29) (TriggeredSeconds :type Float%20%28double-precision%29) (InputAction :type Input%20Action%20Object%20Reference :default "/Game/KDY/Main_Character/InPut/IA_Main_Skill03.IA_Main_Skill03"))
  (Animation|PlayAnimMontage "/Game/KDY/Main_Character/Animation/BP_Main_Skill03.BP_Main_Skill03" 1.0 "None")
  (Transformation|AddLocalRotation (Variables|Character|GetMesh) (* (Variables|Default|GetSkill03Rotation) (Variables|Default|GetSkill03%20Speed)) false false)
  (bind _returnvalue (Game|SpawnActorfromClass "/Game/KDY/Main_Character/Skill01_Damage.Skill01_Damage_C" (Math|Conversions|ToTransform(Vector) (Transformation|GetActorLocation)) "Undefined" "MultiplyWithRoot" 0 0))
  (Actor|DestroyActor _returnvalue))

(event EventBeginPlay
  (bind _inventory (Variables|Default|GetInventory))
  ;[0.15 0.15 0.15 0.5] 김재완 - 인벤 및 플레이어 UI 붙이기 꼭 있어야 함 수정 필요하면 뒤에 이어서 붙여 사용하세요
  (Class|InventoryComponent|InitInventory _inventory)
  (Class|InventoryComponent|SetStatsComponent _inventory (Variables|Default|GetStatsActor))
  (bind _returnvalue (UserInterface|CreateWidget "/Game/KJW/Blueprint/UI/Player/WBP_PlayerMain.WBP_PlayerMain_C"))
  (UserInterface|Viewport|AddtoViewport _returnvalue 0))

(event Game|Damage|EventAnyDamage
  (params (Damage :type Float%20%28single-precision%29) (DamageType :type Damage%20Type%20Object%20Reference) (InstigatedBy :type Controller%20Object%20Reference) (DamageCauser :type Actor%20Object%20Reference))
  (bind _returnvalue (Class|StatsActorComponent|AddHp (Variables|Default|GetStatsActor) (* Damage -1.0)))
  (Development|PrintString (Utilities|String|Append "Player HP : " (Utilities|String|ToString(Float) _returnvalue)) true true "(R=1.000000,G=0.000000,B=0.000000,A=1.000000)")
  (if (<= (Class|StatsActorComponent|GetHp (Variables|Default|GetStatsActor)) 0.0)
    (CallFunction|Dead)
    (else
      (Animation|PlayAnimMontage "/Game/KDY/Main_Character/Animation/Hit/Main_Hit_Mot_01.Main_Hit_Mot_01" 1.0 "None"))))

(event EventControllerChanged
  (params (OldController :type Controller%20Object%20Reference) (NewController :type Controller%20Object%20Reference))
  (bind _asplayer_controller (Utilities|Casting|CastToPlayerController NewController))
  (Input|AddMappingContext (PlayerController|LocalPlayerSubsystems|GetEnhancedInputLocalPlayerSubsystem _asplayer_controller) "/Game/KDY/Main_Character/InPut/IA_Main_TPS.IA_Main_TPS" 0 "(bIgnoreAllPressedKeysUntilRelease=True,bForceImmediately=False,bNotifyUserSettings=False)"))

(event EventTick
  (params (DeltaSeconds :type Float%20%28single-precision%29))
  (bind _returnvalue (Transformation|GetActorRotation))
  ;[0.15 0.15 0.15 0.5] 플레이어 캐릭터가 커서방향으로 바라보게 만들기
  (bind _output_get (Variables|Default|SetCurrent%20Time (+ DeltaSeconds (Variables|Default|GetCurrent%20Time))))
  (if (> _output_get (Variables|Default|GetDelay%20Time))
    (Variables|Default|SetCurrent%20Time 0.0)
    (if (> (Class|StatsActorComponent|GetHp (Variables|Default|GetStatsActor)) 1.0)
      (Transformation|SetWorldRotation (Variables|Collision|GetCapsuleComponent) (Math|Rotator|MakeRotator (.roll _returnvalue) (.pitch _returnvalue) (.yaw (Math|Rotator|FindLookatRotation (Transformation|GetActorLocation) (.Location (Collision|BreakHitResult (.HitResult (Game|Player|GetHitResultUnderCursorbyChannel (Game|GetPlayerController 0) "TraceTypeQuery1" true))))))) false false)
      (if (Utilities|Array|IsValidIndex (Variables|Default|GetFlicker%20Target%20Array))
        (Utilities|IsValid (Variables|Default|GetFlicker%20Target)
          (:Is%20Valid
            _)
          (:Is%20Not%20Valid
            (Variables|Default|SetFlicker%20Target (.ReturnValue (Actor|FindNearestActor (Transformation|GetActorLocation) (Variables|Default|GetFlicker%20Target%20Array))))))
        (bind _asenemy (Utilities|Casting|CastToEnemy (Variables|Default|GetFlicker%20Target))
          (:then
            (if (> (Variables|/Script/TeamProject_POEKor.Enemy|GetHp _asenemy) 1.0)
              (Transformation|SetActorLocation (Transformation|GetActorLocation (Variables|Default|GetFlicker%20Target)) false false :!label _label)
              (Effects|SpawnEmitteratLocation "/Game/FXVarietyPack/Particles/P_ky_lightning3.P_ky_lightning3" (Transformation|GetActorLocation) "0, 0, 0" "0.500000,0.500000,0.500000")
              (Audio|PlaySound2D "/Game/FlexibleCombatSystem/SoundFX/Melee/SC_DrawWep_01_Cue.SC_DrawWep_01_Cue" 1.0 1.0 0.0 0 0)
              (bind _returnvalue_2 (Game|SpawnActorfromClass "/Game/KDY/Main_Character/Flicker_Damage.Flicker_Damage_C" (Math|Conversions|ToTransform(Vector) (Transformation|GetActorLocation)) "Undefined" "MultiplyWithRoot" 0 0))
              (Actor|DestroyActor _returnvalue_2)
              (Utilities|Array|RemoveItem (Variables|Default|GetFlicker%20Target%20Array) (Variables|Default|GetFlicker%20Target))
              (Variables|Default|SetFlicker%20Target 0)
              (if (<= (Utilities|Array|Length (Variables|Default|GetFlicker%20Target%20Array)) 0)
                (bind _outactors (Collision|SphereOverlapActors (Transformation|GetActorLocation) 5e+03 (Utilities|Array|MakeArray "ObjectTypeQuery3") 0))
                (Variables|Default|SetFlicker%20Target%20Array _outactors))
              (else
                (Utilities|Array|RemoveItem (Variables|Default|GetFlicker%20Target%20Array) (Variables|Default|GetFlicker%20Target) :!label _label_2)
                (Variables|Default|SetFlicker%20Target 0))))
          (:CastFailed
            (bind _asboss (Utilities|Casting|CastToBoss (Variables|Default|GetFlicker%20Target)))
            (if (> (Variables|/Script/TeamProject_POEKor.Boss|GetHp _asboss) 1.0)
              (goto _label)
              (else
                (goto _label_2)))))))))

(fn ConstructionScript
  (Components|SkinnedMesh|SetLeaderPoseComponent (Variables|Default|GetHelmet) (Variables|Character|GetMesh) false false))

(fn FlickerLocation
  (params (Direction :type Vector) (Speed :type Float%20%28double-precision%29) (Delta%20Second :type Float%20%28double-precision%29))
  (bind _returnvalue (Transformation|GetActorLocation))
  (Utilities|IsValid (Variables|Default|GetFlicker%20Target)
    (:Is%20Valid
      (if (Utilities|Array|ContainsItem (Variables|Default|GetFlicker%20Target%20Array) (Variables|Default|GetFlicker%20Target))
        (Utilities|Array|RemoveItem (Variables|Default|GetFlicker%20Target%20Array) (Variables|Default|GetFlicker%20Target))
        (bind _output_get (Variables|Default|SetFlicker%20Target (.ReturnValue (Actor|FindNearestActor (Transformation|GetActorLocation) (Variables|Default|GetFlicker%20Target%20Array)))))
        (Development|PrintString (Utilities|GetDisplayName _output_get))
        (Transformation|SetActorLocation (+ (* (.x _returnvalue) (.y _returnvalue)) (* Direction Speed Delta%20Second)) false false)))
    (:Is%20Not%20Valid
      (bind _output_get_2 (Variables|Default|SetFlicker%20Target (.ReturnValue (Actor|FindNearestActor (Transformation|GetActorLocation) (Variables|Default|GetFlicker%20Target%20Array)))))
      (Development|PrintString (Utilities|GetDisplayName _output_get_2)))))

(fn DieEvent
  (params (Die :type Boolean)))

(fn FlickrSearch
  (bind _outactors (Collision|SphereOverlapActors (Transformation|GetActorLocation) 1e+03 (Utilities|Array|MakeArray "ObjectTypeQuery3") 0))
  (Variables|Default|SetFlicker%20Target%20Array _outactors)
  (Utilities|IsValid (Variables|Default|GetFlicker%20Target)
    (:Is%20Valid
      (if (Utilities|Array|ContainsItem (Variables|Default|GetFlicker%20Target%20Array) (Variables|Default|GetFlicker%20Target))
        (Utilities|Array|RemoveItem (Variables|Default|GetFlicker%20Target%20Array) (Variables|Default|GetFlicker%20Target))
        (bind _output_get (Variables|Default|SetFlicker%20Target (.ReturnValue (Actor|FindNearestActor (Transformation|GetActorLocation) (Variables|Default|GetFlicker%20Target%20Array)))))
        (Development|PrintString (Utilities|GetDisplayName _output_get))))
    (:Is%20Not%20Valid
      (bind _output_get_2 (Variables|Default|SetFlicker%20Target (.ReturnValue (Actor|FindNearestActor (Transformation|GetActorLocation) (Variables|Default|GetFlicker%20Target%20Array)))))
      (Development|PrintString (Utilities|GetDisplayName _output_get_2)))))

(fn CanbeAssassinated
  (return false))

(fn FindAvailableAssassinationCam
  (return 0))

(fn GetWeaponRange
  (return 0.0))

(fn IsDead
  (return false))

(fn IsFacingEnemy?
  (bind _followcamera (Variables|Components|GetFollowCamera))
  (bind _returnvalue (Transformation|GetWorldLocation _followcamera))
  (bind _outhit (Collision|LineTraceByChannel _returnvalue (+ _returnvalue (* (Math|Vector|GetForwardVector _followcamera) 3e+03)) "TraceTypeQuery3" false 0 "None"))
  (Utilities|IsValid (.HitActor (Collision|BreakHitResult _outhit))
    (:Is%20Valid
      (return (Actor|ActorHasTag (.HitActor (Collision|BreakHitResult _outhit)) "EnemyAI")))
    (:Is%20Not%20Valid
      (return false))))

(fn IsMoving?
  (return (Math|Vector|NotEqual(Vector) (Transformation|GetVelocity) "0, 0, 0" 0.0001)))

(fn IsPlayer?
  (return true))

(fn IsWeaponDrawn?
  (return false))

(fn PassArmorMeshes
  (return (Variables|Default|GetHelmet) (Variables|Default|GetChest) 0 (Variables|Default|GetShoulder) (Variables|Default|GetBack) (Variables|Default|GetLegs) (Variables|Default|GetHands) (Variables|Default|GetBoots) 0 0 0))

(fn PassAssassinationComps
  (return 0 0))

(fn PassBody
  (return (Variables|Default|GetMannequinFillerMesh) (Variables|Default|GetHelmet) (Variables|Default|GetBack) (Variables|Default|GetHands) (Variables|Default|GetLegs) (Variables|Default|GetBoots) (Variables|Default|GetChest) (Variables|Default|GetShoulder)))

(fn PassCamera
  (return (Variables|Components|GetFollowCamera) (Variables|Components|GetCameraBoom)))

(fn PassMovementMode
  (return (Variables|/Script/Engine.CharacterMovementComponent|GetMovementMode (Variables|Character|GetCharacterMovement))))

(fn RetrievePlayerStatus
  (return false 0 0))

(fn SendDeath)

(fn SetDisableControls
  (params (DisableMovement :type Boolean) (DisableCamera :type Boolean)))

(fn UpdateMovementMode
  (params (MovementMode :type EMovementMode%20Enum :default "MOVE_None"))
  (Pawn|Components|CharacterMovement|SetMovementMode (Variables|Default|GetCharacterMovement) MovementMode 0)
  (return false))