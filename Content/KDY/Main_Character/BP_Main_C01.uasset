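; Player character for a dungeon game that moves by Enhanced Input, faces the cursor and sets up inventory and HUD.
; Attack and Skill01 play montages, then spawn a short-lived Damage actor at the character's location; Skill02 and Skill03 are empty.
; AnyDamage lowers HP, playing a hit reaction or Dead, which destroys the actor and requests GameOver.
; Modular armor follows the main mesh's pose; assassination and weapon queries are mostly stubs.
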(event Custom|Dead
  (if (not (Variables|Default|GetIs%20Die))
    (Variables|Default|SetIs%20Die true)
    (Animation|PlayAnimMontage "/Game/KDY/Main_Character/Animation/Dead/Main_Die_Mot_02.Main_Die_Mot_02" 1.0 "None")
    (Utilities|FlowControl|Delay 2.5)
    (Development|PrintString "Dead!!")
    (Actor|DestroyActor)
    ;[0.15 0.15 0.15 0.5] 게임 상태 변화 시키기
    (bind _asbp_dungeon_game_state (Utilities|Casting|CastToBP_DungeonGameState (Game|GetGameState)))
    (Class|DungeonGameStateBase|ChangeGameState _asbp_dungeon_game_state "GameOver")))

(event Input|EnhancedActionEvents|EnhancedInputActionIA_Main_Move
  (params (ActionValue :type Vector%202D%20Structure) (ElapsedSeconds :type Float%20%28double-precision%29) (TriggeredSeconds :type Float%20%28double-precision%29) (InputAction :type Input%20Action%20Object%20Reference :default "/Game/KDY/Main_Character/InPut/IA_Main_Move.IA_Main_Move"))
  (bind _returnvalue (Pawn|GetControlRotation :!class /Script/Engine.Pawn))
  ;[0.15 0.15 0.15 0.5] WASD 로 걸어다니기
  (if (> (Variables|Default|GetHP) 1.0)
    (Pawn|Input|AddMovementInput (Math|Vector|Normalize (Math|Vector|GetRightVector (Math|Rotator|MakeRotator (.roll _returnvalue) 0.0 (.yaw _returnvalue)))) (.x ActionValue) false)
    (Pawn|Input|AddMovementInput (Math|Vector|Normalize (Math|Vector|GetForwardVector (Math|Rotator|MakeRotator 0.0 0.0 (.yaw (Pawn|GetControlRotation :!class /Script/Engine.Pawn))))) (.y ActionValue) false)
    (else
      (Pawn|Components|CharacterMovement|DisableMovement (Variables|Character|GetCharacterMovement)))))

(event Input|EnhancedActionEvents|EnhancedInputActionIA_Main_Attack
  (params (ActionValue :type Boolean) (ElapsedSeconds :type Float%20%28double-precision%29) (TriggeredSeconds :type Float%20%28double-precision%29) (InputAction :type Input%20Action%20Object%20Reference :default "/Game/KDY/Main_Character/InPut/IA_Main_Attack.IA_Main_Attack"))
  (:Started
    (Animation|PlayAnimMontage "/Game/KDY/Main_Character/Animation/Attack/Main_Attack.Main_Attack" 1.0 "None")
    (Utilities|FlowControl|Delay 0.5)
    (bind _returnvalue (Game|SpawnActorfromClass "/Game/KDY/Main_Character/Damage.Damage_C" (Math|Conversions|ToTransform(Vector) (Transformation|GetActorLocation)) "Undefined" "MultiplyWithRoot" 0 0))
    (Utilities|FlowControl|Delay 0.2)
    (Actor|DestroyActor _returnvalue)))

(event Input|EnhancedActionEvents|EnhancedInputActionIA_Main_Skill01
  (params (ActionValue :type Boolean) (ElapsedSeconds :type Float%20%28double-precision%29) (TriggeredSeconds :type Float%20%28double-precision%29) (InputAction :type Input%20Action%20Object%20Reference :default "/Game/KDY/Main_Character/InPut/IA_Main_Skill01.IA_Main_Skill01"))
  (:Started
    (if (> (Variables|Default|GetHP) 1.0)
      (Animation|PlayAnimMontage "/Game/KDY/Main_Character/Animation/BP_Main_Skill01.BP_Main_Skill01" 1.0 "None")
      (Utilities|FlowControl|Delay 1.0)
      (bind _returnvalue (Game|SpawnActorfromClass "/Game/KDY/Main_Character/Damage.Damage_C" (Math|Conversions|ToTransform(Vector) (Transformation|GetActorLocation)) "Undefined" "MultiplyWithRoot" 0 0))
      (Utilities|FlowControl|Delay 0.2)
      (Actor|DestroyActor _returnvalue)
      (else
        (Pawn|Components|CharacterMovement|DisableMovement (Variables|Character|GetCharacterMovement))))))

(event Input|EnhancedActionEvents|EnhancedInputActionIA_Main_Skill02
  (params (ActionValue :type Boolean) (ElapsedSeconds :type Float%20%28double-precision%29) (TriggeredSeconds :type Float%20%28double-precision%29) (InputAction :type Input%20Action%20Object%20Reference :default "/Game/KDY/Main_Character/InPut/IA_Main_Skill02.IA_Main_Skill02")))

(event Input|EnhancedActionEvents|EnhancedInputActionIA_Main_Skill03
  (params (ActionValue :type Boolean) (ElapsedSeconds :type Float%20%28double-precision%29) (TriggeredSeconds :type Float%20%28double-precision%29) (InputAction :type Input%20Action%20Object%20Reference :default "/Game/KDY/Main_Character/InPut/IA_Main_Skill03.IA_Main_Skill03")))

(event EventBeginPlay
  ;[0.15 0.15 0.15 0.5] 김재완 - 인벤 및 플레이어 UI 붙이기 꼭 있어야 함 수정 필요하면 뒤에 이어서 붙여 사용하세요
  (Class|InventoryComponent|InitInventory (Variables|Default|GetInventory))
  (bind _returnvalue (UserInterface|CreateWidget "/Game/KJW/Blueprint/UI/Player/WBP_PlayerUI.WBP_PlayerUI_C"))
  (UserInterface|Viewport|AddtoViewport _returnvalue 0))

(event Game|Damage|EventAnyDamage
  (params (Damage :type Float%20%28single-precision%29) (DamageType :type Damage%20Type%20Object%20Reference) (InstigatedBy :type Controller%20Object%20Reference) (DamageCauser :type Actor%20Object%20Reference))
  (bind _output_get (Variables|Default|SetHP (- (Variables|Default|GetHP) Damage)))
  (Development|PrintString (Utilities|String|Append "Player HP : " (Utilities|String|ToString(Float) _output_get)) true true "(R=1.000000,G=0.000000,B=0.000000,A=1.000000)")
  (if (<= (Variables|Default|GetHP) 0.0)
    (CallFunction|Dead)
    (else
      (Animation|PlayAnimMontage "/Game/KDY/Main_Character/Animation/Hit/Main_Hit_Mot_01.Main_Hit_Mot_01" 1.0 "None"))))

(event EventControllerChanged
  (params (OldController :type Controller%20Object%20Reference) (NewController :type Controller%20Object%20Reference))
  (bind _asplayer_controller (Utilities|Casting|CastToPlayerController NewController))
  (Input|AddMappingContext (PlayerController|LocalPlayerSubsystems|GetEnhancedInputLocalPlayerSubsystem _asplayer_controller) "/Game/KDY/Main_Character/InPut/IA_Main_TPS.IA_Main_TPS" 0 "(bIgnoreAllPressedKeysUntilRelease=True,bForceImmediately=False,bNotifyUserSettings=False)"))

(event EventTick
  (params (DeltaSeconds :type Float%20%28single-precision%29))
  (bind _returnvalue (Transformation|GetActorRotation))
  ;[0.15 0.15 0.15 0.5] 플레이어 캐릭터가 커서방향으로 바라보게 만들기
  (if (> (Variables|Default|GetHP) 1.0)
    (Transformation|SetWorldRotation (Variables|Collision|GetCapsuleComponent) (Math|Rotator|MakeRotator (.roll _returnvalue) (.pitch _returnvalue) (.yaw (Math|Rotator|FindLookatRotation (Transformation|GetActorLocation) (.Location (Collision|BreakHitResult (.HitResult (Game|Player|GetHitResultUnderCursorbyChannel (Game|GetPlayerController 0) "TraceTypeQuery1" true))))))) false false)))

(fn ConstructionScript
  (Components|SkinnedMesh|SetLeaderPoseComponent (Variables|Default|GetHelmet) (Variables|Character|GetMesh) false false))

(fn CanbeAssassinated
  (return false))

(fn FindAvailableAssassinationCam
  (return 0))

(fn GetWeaponRange
  (return 0.0))

(fn IsDead
  (return false))

(fn IsFacingEnemy?
  (bind _followcamera (Variables|Components|GetFollowCamera))
  (bind _returnvalue (Transformation|GetWorldLocation _followcamera))
  (bind _outhit (Collision|LineTraceByChannel _returnvalue (+ _returnvalue (* (Math|Vector|GetForwardVector _followcamera) 3e+03)) "TraceTypeQuery3" false 0 "None"))
  (Utilities|IsValid (.HitActor (Collision|BreakHitResult _outhit))
    (:Is%20Valid
      (return (Actor|ActorHasTag (.HitActor (Collision|BreakHitResult _outhit)) "EnemyAI")))
    (:Is%20Not%20Valid
      (return false))))

(fn IsMoving?
  (return (Math|Vector|NotEqual(Vector) (Transformation|GetVelocity) "0, 0, 0" 0.0001)))

(fn IsPlayer?
  (return true))

(fn IsWeaponDrawn?
  (return false))

(fn PassArmorMeshes
  (return (Variables|Default|GetHelmet) (Variables|Default|GetChest) 0 (Variables|Default|GetShoulder) (Variables|Default|GetBack) (Variables|Default|GetLegs) (Variables|Default|GetHands) (Variables|Default|GetBoots) 0 0 0))

(fn PassAssassinationComps
  (return 0 0))

(fn PassBody
  (return (Variables|Default|GetMannequinFillerMesh) (Variables|Default|GetHelmet) (Variables|Default|GetBack) (Variables|Default|GetHands) (Variables|Default|GetLegs) (Variables|Default|GetBoots) (Variables|Default|GetChest) (Variables|Default|GetShoulder)))

(fn PassCamera
  (return (Variables|Components|GetFollowCamera) (Variables|Components|GetCameraBoom)))

(fn PassMovementMode
  (return (Variables|/Script/Engine.CharacterMovementComponent|GetMovementMode (Variables|Character|GetCharacterMovement))))

(fn RetrievePlayerStatus
  (return false 0 0))

(fn SendDeath)

(fn SetDisableControls
  (params (DisableMovement :type Boolean) (DisableCamera :type Boolean)))

(fn UpdateMovementMode
  (params (MovementMode :type EMovementMode%20Enum :default "MOVE_None"))
  (Pawn|Components|CharacterMovement|SetMovementMode (Variables|Default|GetCharacterMovement) MovementMode 0)
  (return false))